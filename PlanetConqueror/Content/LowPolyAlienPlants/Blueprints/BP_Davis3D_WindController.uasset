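; Wind controller for the low-poly alien plants that writes wind settings to the MPC_LowPolyAlienPlants material parameter collection.
; BeginPlay sets wind speed and scale.
; Three timelines, with no play inputs wired in the graph, have update logic for intensity, rotation and UV offsets.
; The rotation value splits the speed curve between X and Y offsets, which accumulate each update to scroll the wind.
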(event `self.ReceiveBeginPlay`
  (`KismetMaterialLibrary.SetScalarParameterValue` "/Game/LowPolyAlienPlants/Materials/MaterialFunctions/MPC_LowPolyAlienPlants.MPC_LowPolyAlienPlants" "WindSpeed" (`self.WindSpeed`))
  (`KismetMaterialLibrary.SetScalarParameterValue` "/Game/LowPolyAlienPlants/Materials/MaterialFunctions/MPC_LowPolyAlienPlants.MPC_LowPolyAlienPlants" "WindScale" (`self.WindScale`)))

(fn `UserConstructionScript`)