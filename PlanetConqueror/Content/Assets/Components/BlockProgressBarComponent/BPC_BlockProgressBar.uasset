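; Widget component that shows a block-segmented progress bar in screen space, rebuilt from ProgressBarData on BeginPlay and initially hidden.
; Value changes update the widget's lerped or immediate fill, with multicast events and authority checks keeping visual work off dedicated servers.
; Show and hide support recursive, delay-driven opacity fades, with a gate blocking fade-out during fade-in.
; Each tick rotates it toward the local player and resizes it by camera distance, hiding it when tiny.
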(event `self.ReceiveBeginPlay`
  ;[0.7274 0.9968 1] Widget Setting
  (`self.Reinit BPBar` (`self.ProgressBarData`))
  (`self.HideBPBar` false))

(event `self.ReceiveTick`
  (params (DeltaSeconds :type "Float (single-precision)"))
  (`self.UpdateBPBar` DeltaSeconds))

(event `Fade BPBar In`
  (params (`Fade Time` :type "Float (double-precision)") (`Fade Interval` :type "Float (double-precision)"))
  (bind _returnvalue (`GameplayStatics.GetWorldDeltaSeconds`))
  ;[0.7274 0.9968 1] Fade In Protocol
  ;;[1 1 0.467] Fade Timer가 끝나거나 Fade In이 완료되었을 때
  (if (or (<= `Fade Time` 0.0) (>= (`self.GetBPBarOpacity`) 1.0))
    ;;[1 1 0.467] Fade In Protocol이 끝난 후 확실하게 보이게 하기
    (`self.SetBPBarOpactiy` 1.0)
    (`self.Open Fade BPBar Out`)
    (else
      ;;[1 1 0.467] 불투명도 증가
      (`self.SetBPBarOpactiy` (+ (`self.GetBPBarOpacity`) (* `Fade Interval` (`GameplayStatics.GetWorldDeltaSeconds`))))
      ;;[1 1 0.467] Delay 후 반복
      (`KismetSystemLibrary.Delay` _returnvalue)
      (`self.Fade BPBar In` (- `Fade Time` _returnvalue) `Fade Interval`))))

(event `Fade BPBar Out`
  (params (`Fade Time` :type "Float (double-precision)") (`Fade Interval` :type "Float (double-precision)"))
  (bind _returnvalue (`GameplayStatics.GetWorldDeltaSeconds`))
  ;[0.7274 0.9968 1] Comment
  (`/Engine/EditorBlueprintResources/StandardMacros.Gate` false :!label _label
    (:`Exit`
      ;;[1 1 0.467] Fade Timer가 끝나거나 Fade out이 완료되었을 때
      (if (or (<= `Fade Time` 0.0) (<= (`self.GetBPBarOpacity`) 0.0))
        ;;[1 1 0.467] Fade Out Protocol이 끝난 후 확실하게 보이게 하기
        (`self.SetBPBarOpactiy` 0.0)
        (else
          ;;[1 1 0.467] 불투명도 감소
          (`self.SetBPBarOpactiy` (- (`self.GetBPBarOpacity`) (* `Fade Interval` (`GameplayStatics.GetWorldDeltaSeconds`))))
          ;;[1 1 0.467] Delay 후 반복
          (`KismetSystemLibrary.Delay` _returnvalue)
          (`self.Fade BPBar Out` (- `Fade Time` _returnvalue) `Fade Interval`))))))

(event `Open Fade BPBar Out`
  ;[0.7274 0.9968 1] Comment
  (goto _label :!via `Open`))

(event `Close Fade BPBar Out`
  ;[0.7274 0.9968 1] Comment
  (goto _label :!via `Close`))

(event `SetValue MC`
  (params (NewValue :type "Float (double-precision)") (Immediately :type Boolean))
  (`self.SetValue` NewValue Immediately))

(event `ShowBPBar MC`
  (params (`Fade In` :type Boolean) (`Fade Time` :type "Float (double-precision)"))
  (`self.Has Athority in Dedi`
    (:`Authority`
      _)
    (:`Remote`
      _))
  (`self.ShowBPBar` `Fade In` `Fade Time`))

(event `HideBPBar MC`
  (params (FadeOut :type Boolean) (ForcedFadeOut :type Boolean) (`Fade Time` :type "Float (double-precision)"))
  (`self.Has Athority in Dedi`
    (:`Authority`
      _)
    (:`Remote`
      _))
  (`self.HideBPBar` FadeOut ForcedFadeOut `Fade Time`))

(fn `GetCastedWidget`
  (returns (BlockProgressBarWidget :type "/Game/Widget/BlockProgressBar/Blueprints/WBP_BlockProgressBar Object Reference"))
  (return (`self.BlockProgressBarWidget`)))

(fn `HideBPBar`
  (params (`Fade Out` :type Boolean) (`Forced Fade Out` :type Boolean) (`Fade Time` :type "Float (double-precision)"))
  (`self.Has Athority in Dedi`
    (:`Authority In Dedi`
      (`self.HideBPBar MC` `Fade Out` `Forced Fade Out` `Fade Time`))
    (:`Authority`
      (if `Forced Fade Out` :!label _label
        (`self.Open Fade BPBar Out`))
      (if `Fade Out`
        ;[1 1 0.467] Fade Out Protocol 시작
        (`self.SetVisibility` true)
        (`self.Fade BPBar Out` `Fade Time` (/ 1.0 `Fade Time`))
        (else
          ;[1 1 0.467] 바로 숨기기
          (`Widget.SetRenderOpacity` (`self.BlockProgressBarWidget`) `Fade Time`)
          (`self.SetVisibility` false))))
    (:`Remote`
      (goto _label))))

(fn `IncreaseValue`
  (params (Value :type "Float (double-precision)") (Immediately :type Boolean :default true))
  (returns (Empty :type Boolean))
  (`self.SetValue MC` (`KismetMathLibrary.FMin` (+ Value (`self.CurValue`)) (`self.MaxValue`)) Immediately)
  (return (`self.IsEmpty`)))

(fn `IsEmpty`
  (returns (Empty :type Boolean))
  (return (<= (`self.CurValue`) 0.0)))

(fn `IsFull`
  (returns (FullHP :type Boolean))
  (return (== (`self.CurValue`) (`self.MaxValue`))))

(fn `Reinit BPBar`
  (params (`New Data` :type "/Game/Structs/S_BlockProgressBarData Structure"))
  (bind (_progressbardata_fillblock _progressbardata_blankblock _progressbardata_cntblock _progressbardata_blockinterval _progressbardata_filltype) (break `/Game/Structs/S_BlockProgressBarData` (`self.ProgressBarData`)))
  (bind (_x _y) (`KismetMathLibrary.BreakVector2D` (`self.OriginalDrawSize`)))
  (bind _aswbp_block_progress_bar (cast `/Game/Widget/BlockProgressBar/Blueprints/WBP_BlockProgressBar` (`self.GetWidget`)))
  (set `self.ProgressBarData` `New Data`)
  (bind _returnvalue (`|CreateWidget` (`GameplayStatics.GetObjectClass` _aswbp_block_progress_bar) null _progressbardata_fillblock _progressbardata_blankblock _progressbardata_cntblock _progressbardata_blockinterval _progressbardata_filltype))
  (bind _output_get (set `self.BlockProgressBarWidget` _returnvalue))
  (`self.SetWidget` _output_get)
  (`self.SetWidgetSpace` "Screen")
  (`self.SetDrawSize` (`self.OriginalDrawSize`))
  (`self.SetCollisionEnabled` "NoCollision")
  (set `self.DrawSizeRatio` (/ _x _y)))

(fn `SetValue`
  (params (NewValue :type "Float (double-precision)") (Immediately :type Boolean :default true))
  (returns (Value :type "Float (double-precision)"))
  (bind _output_get (set `self.CurValue` (`KismetMathLibrary.FMin` (`self.MaxValue`) NewValue)))
  (`self.Has Athority in Dedi`
    (:`Authority In Dedi`
      _)
    (:`Authority`
      (`/Game/Widget/BlockProgressBar/Blueprints/WBP_BlockProgressBar.Set Percentage` (`self.GetCastedWidget`) (/ _output_get (`self.MaxValue`)) Immediately (`self.BPBarLerpSpeed`) :!label _label))
    (:`Remote`
      (goto _label)))
  (return _output_get))

(fn `ShowBPBar`
  (params (`Fade In` :type Boolean) (`Fade Time` :type "Float (double-precision)"))
  (`self.Has Athority in Dedi`
    (:`Authority In Dedi`
      (`self.ShowBPBar MC` `Fade In` `Fade Time`))
    (:`Authority`
      (if `Fade In` :!label _label
        ;[1 1 0.467] Fade In Protocol 시작
        (`self.SetVisibility` true)
        (`self.Close Fade BPBar Out`)
        (`self.Fade BPBar In` `Fade Time` (/ 1.0 `Fade Time`))
        (else
          ;[1 1 0.467] 바로 보이기
          (`Widget.SetRenderOpacity` (`self.BlockProgressBarWidget`) 1.0)
          (`self.SetVisibility` true))))
    (:`Remote`
      (goto _label))))

(fn `TimerHideBPBar`
  (`self.HideBPBar` true false (`self.TimerFadeOutTime`)))

(fn `UpdateBPBar`
  (params (`Delta Seconds` :type "Float (double-precision)"))
  (locals (DistToPlayer :type "Float (double-precision)" :default 0.0))
  (bind _returnvalue (`GameplayStatics.GetPlayerPawn` 0))
  (bind (_originaldrawsize_x _originaldrawsize_y) (`KismetMathLibrary.BreakVector2D` (`self.OriginalDrawSize`)))
  (bind (_originaldrawsize_x_2 _originaldrawsize_y_2) (`KismetMathLibrary.BreakVector2D` (`self.OriginalDrawSize`)))
  (bind _disttoplayer (`local.DistToPlayer`))
  (bind _returnvalue_2 (+ _originaldrawsize_y (* (- (`self.ViewRangeMin`) _disttoplayer) (`self.SizeBiggerOffsetValue`))))
  (bind _returnvalue_3 (- _originaldrawsize_y_2 (* (- _disttoplayer (`self.ViewRangeMax`)) (`self.SizeSmallerOffsetValue`))))
  (`self.Has Athority in Dedi`
    (:`Authority`
      _)
    (:`Remote`
      _))
  ;[1 1 0.467] Calc Dist to Player(Client)
  (set `local.DistToPlayer` (`KismetMathLibrary.Vector_Distance` (`Actor.K2_GetActorLocation` (`GameplayStatics.GetPlayerCameraManager` 0)) (`self.K2_GetComponentLocation`)))
  ;[0.7274 0.9968 1] HP Bar Looking Player
  (`/Engine/EditorBlueprintResources/StandardMacros.IsValid` _returnvalue
    (:`Is Valid`
      (`self.K2_SetWorldRotation` (`KismetMathLibrary.FindLookAtRotation` (`self.K2_GetComponentLocation`) (`Actor.K2_GetActorLocation` _returnvalue)) false true)
      (`|ExecutionSequence`
        (:`then_1`
          ;[0.7274 0.9968 1] 위치에 따른 크기 조정 및 매우 멀 때 숨기기
          (`/Game/Macros/GlobalMacros.Compare In Range (float)` _disttoplayer (`self.ViewRangeMin`) (`self.ViewRangeMax`)
            (:`Value < Min`
              (`self.SetDrawSize` (`KismetMathLibrary.MakeVector2D` (* _returnvalue_2 (`self.DrawSizeRatio`)) _returnvalue_2)))
            (:`Value == Min`
              (`self.SetDrawSize` (`self.OriginalDrawSize`) :!label _label))
            (:`Value In Range`
              (goto _label))
            (:`Value == Max`
              (goto _label))
            (:`Value > Max`
              (if (<= _returnvalue_3 5.0)
                (`self.SetVisibility` false)
                (else
                  (`self.SetVisibility` true)
                  (`self.SetDrawSize` (`KismetMathLibrary.MakeVector2D` (* _returnvalue_3 (`self.DrawSizeRatio`)) _returnvalue_3)))))))))))