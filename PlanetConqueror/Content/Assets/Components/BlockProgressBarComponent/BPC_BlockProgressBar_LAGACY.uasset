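; Legacy component that shows a block-style progress bar, used as an HP bar, in a screen-space widget over its owner.
; Initialize creates WBP_BlockProgressBar from the supplied data and starts it hidden.
; Tick turns it toward player 0 and scales draw size by distance, hiding it when too small.
; Show/hide fades use self-calling Delay events with a gate on fade-out, and visual logic skips dedicated-server authority.
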(event `Initialize`
  (params (Owner :type "Actor Object Reference") (ComponentRelativeTransform :type "Transform Structure") (BlockProgressBarData :type "/Game/Structs/S_BlockProgressBarData Structure"))
  (bind (_fillblock _blankblock _cntblock _blockinterval _filltype) (break `/Game/Structs/S_BlockProgressBarData` BlockProgressBarData))
  (bind (_x _y) (`KismetMathLibrary.BreakVector2D` (`self.OriginalDrawSize`)))
  ;[0.7274 0.9968 1] Widget Setting
  (bind _returnvalue (`|AddComponentByClass` Owner "/Script/UMG.WidgetComponent" false ComponentRelativeTransform))
  (set `self.BlockProgressBarWidgetComponent` _returnvalue)
  (bind _returnvalue_2 (`|CreateWidget` "/Game/Widget/BlockProgressBar/Blueprints/WBP_BlockProgressBar.WBP_BlockProgressBar_C" null _fillblock _blankblock _cntblock _blockinterval _filltype))
  (set `self.BlockProgressBarWidget` _returnvalue_2)
  (`WidgetComponent.SetWidgetSpace` (`self.BlockProgressBarWidgetComponent`) "Screen")
  (`WidgetComponent.SetWidget` (`self.BlockProgressBarWidgetComponent`) (`self.BlockProgressBarWidget`))
  (`WidgetComponent.SetDrawSize` (`self.BlockProgressBarWidgetComponent`) (`self.OriginalDrawSize`))
  (`PrimitiveComponent.SetCollisionEnabled` (`self.BlockProgressBarWidgetComponent`) "NoCollision")
  (set `self.DrawSizeRatio` (/ _x _y))
  (`self.HideHPBar` false))

(event `self.ReceiveTick`
  (params (DeltaSeconds :type "Float (single-precision)"))
  (`self.UpdateHPBar` DeltaSeconds))

(event `Fade HPBar In`
  (params (`Fade Time` :type "Float (double-precision)") (`Fade Interval` :type "Float (double-precision)"))
  (bind _returnvalue (`GameplayStatics.GetWorldDeltaSeconds`))
  ;[0.7274 0.9968 1] Fade In Protocol
  ;;[1 1 0.467] Fade Timer가 끝나거나 Fade In이 완료되었을 때
  (if (or (<= `Fade Time` 0.0) (>= (`self.GetHPBarOpacity`) 1.0))
    ;;[1 1 0.467] Fade In Protocol이 끝난 후 확실하게 보이게 하기
    (`self.SetHPBarOpactiy` 1.0)
    (`self.Open Fade HPBar Out`)
    (else
      ;;[1 1 0.467] 불투명도 증가
      (`self.SetHPBarOpactiy` (+ (`self.GetHPBarOpacity`) (* `Fade Interval` (`GameplayStatics.GetWorldDeltaSeconds`))))
      ;;[1 1 0.467] Delay 후 반복
      (`KismetSystemLibrary.Delay` _returnvalue)
      (`self.Fade HPBar In` (- `Fade Time` _returnvalue) `Fade Interval`))))

(event `Fade HPBar Out`
  (params (`Fade Time` :type "Float (double-precision)") (`Fade Interval` :type "Float (double-precision)"))
  (bind _returnvalue (`GameplayStatics.GetWorldDeltaSeconds`))
  ;[0.7274 0.9968 1] Comment
  (`/Engine/EditorBlueprintResources/StandardMacros.Gate` false :!label _label
    (:`Exit`
      ;;[1 1 0.467] Fade Timer가 끝나거나 Fade out이 완료되었을 때
      (if (or (<= `Fade Time` 0.0) (<= (`self.GetHPBarOpacity`) 0.0))
        ;;[1 1 0.467] Fade Out Protocol이 끝난 후 확실하게 보이게 하기
        (`self.SetHPBarOpactiy` 0.0)
        (else
          ;;[1 1 0.467] 불투명도 감소
          (`self.SetHPBarOpactiy` (- (`self.GetHPBarOpacity`) (* `Fade Interval` (`GameplayStatics.GetWorldDeltaSeconds`))))
          ;;[1 1 0.467] Delay 후 반복
          (`KismetSystemLibrary.Delay` _returnvalue)
          (`self.Fade HPBar Out` (- `Fade Time` _returnvalue) `Fade Interval`))))))

(event `Open Fade HPBar Out`
  ;[0.7274 0.9968 1] Comment
  (goto _label :!via `Open`))

(event `Close Fade HPBar Out`
  ;[0.7274 0.9968 1] Comment
  (goto _label :!via `Close`))

(fn `HideHPBar`
  (params (`Fade Out` :type Boolean) (`Fade Time` :type "Float (double-precision)"))
  (`self.Has Athority in Dedi`
    (:`Remote`
      _)
    (:`No Dedi`
      _))
  (if `Fade Out`
    ;[1 1 0.467] Fade Out Protocol 시작
    (`self.SetVisibility` (`self.BlockProgressBarWidgetComponent`) true false)
    (`self.Fade HPBar Out` `Fade Time` (/ 1.0 `Fade Time`))
    (else
      ;[1 1 0.467] 바로 숨기기
      (`Widget.SetRenderOpacity` (`self.BlockProgressBarWidget`) `Fade Time`)
      (`self.SetVisibility` (`self.BlockProgressBarWidgetComponent`) false false))))

(fn `ShowHPBar`
  (params (`Fade In` :type Boolean) (`Fade Time` :type "Float (double-precision)"))
  (`self.Has Athority in Dedi`
    (:`Remote`
      _)
    (:`No Dedi`
      _))
  (if `Fade In`
    ;[1 1 0.467] Fade In Protocol 시작
    (`self.SetVisibility` (`self.BlockProgressBarWidgetComponent`) true false)
    (`self.Close Fade HPBar Out`)
    (`self.Fade HPBar In` `Fade Time` (/ 1.0 `Fade Time`))
    (else
      ;[1 1 0.467] 바로 보이기
      (`Widget.SetRenderOpacity` (`self.BlockProgressBarWidget`) 1.0)
      (`self.SetVisibility` (`self.BlockProgressBarWidgetComponent`) true false))))

(fn `TimerHideHPBar`
  (`self.HideHPBar` true (`self.TimerFadeOutTime`)))

(fn `UpdateHPBar`
  (params (`Delta Seconds` :type "Float (double-precision)"))
  (locals (DistToPlayer :type "Float (double-precision)" :default 0.0))
  (bind _returnvalue (`GameplayStatics.GetPlayerPawn` 0))
  (bind (_originaldrawsize_x _originaldrawsize_y) (`KismetMathLibrary.BreakVector2D` (`self.OriginalDrawSize`)))
  (bind _blockprogressbarwidgetcomponent (`self.BlockProgressBarWidgetComponent`))
  (bind (_originaldrawsize_x_2 _originaldrawsize_y_2) (`KismetMathLibrary.BreakVector2D` (`self.OriginalDrawSize`)))
  (bind _blockprogressbarwidgetcomponent_2 (`self.BlockProgressBarWidgetComponent`))
  (bind _disttoplayer (`local.DistToPlayer`))
  (bind _returnvalue_2 (+ _originaldrawsize_y (* (- 500.0 _disttoplayer) (`self.SizeBiggerOffsetValue`))))
  (bind _returnvalue_3 (- _originaldrawsize_y_2 (* (- _disttoplayer 1200.0) (`self.SizeSmallerOffsetValue`))))
  (`self.Has Athority in Dedi`
    (:`Remote`
      _)
    (:`No Dedi`
      _))
  ;[1 1 0.467] Calc Dist to Player(Client)
  (set `local.DistToPlayer` (`KismetMathLibrary.Vector_Distance` (`Actor.K2_GetActorLocation` (`GameplayStatics.GetPlayerPawn` 0)) (`self.K2_GetComponentLocation`)))
  ;[0.7274 0.9968 1] HP Bar Looking Player
  (`/Engine/EditorBlueprintResources/StandardMacros.IsValid` _returnvalue
    (:`Is Valid`
      (`self.K2_SetWorldRotation` _blockprogressbarwidgetcomponent_2 (`KismetMathLibrary.FindLookAtRotation` (`self.K2_GetComponentLocation` _blockprogressbarwidgetcomponent_2) (`Actor.K2_GetActorLocation` _returnvalue)) false true)
      (`|ExecutionSequence`
        (:`then_1`
          ;[0.7274 0.9968 1] 위치에 따른 크기 조정 및 매우 멀 때 숨기기
          (`/Game/Macros/GlobalMacros.Compare In Range (float)` _disttoplayer (`self.ViewRangeMin`) (`self.ViewRangeMax`)
            (:`Value < Min`
              (`WidgetComponent.SetDrawSize` (`self.BlockProgressBarWidgetComponent`) (`KismetMathLibrary.MakeVector2D` (* _returnvalue_2 (`self.DrawSizeRatio`)) _returnvalue_2)))
            (:`Value == Min`
              (`WidgetComponent.SetDrawSize` (`self.BlockProgressBarWidgetComponent`) (`self.OriginalDrawSize`) :!label _label))
            (:`Value In Range`
              (goto _label))
            (:`Value == Max`
              (goto _label))
            (:`Value > Max`
              (if (<= _returnvalue_3 5.0)
                (`self.SetVisibility` _blockprogressbarwidgetcomponent false false)
                (else
                  (`self.SetVisibility` _blockprogressbarwidgetcomponent true false)
                  (`WidgetComponent.SetDrawSize` (`self.BlockProgressBarWidgetComponent`) (`KismetMathLibrary.MakeVector2D` (* _returnvalue_3 (`self.DrawSizeRatio`)) _returnvalue_3)))))))))))