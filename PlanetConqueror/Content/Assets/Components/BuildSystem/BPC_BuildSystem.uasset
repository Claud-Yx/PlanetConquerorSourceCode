(event `self.ReceiveBeginPlay`
  (`|ExecutionSequence`
    (:`then_0`
      (bind _outrownames (`DataTableFunctionLibrary.GetDataTableRowNames` "/Game/DataTables/DT_Ghost.DT_Ghost"))
      (for _array_element _outrownames
        (bind _returnvalue (`|GetDataTableRow` "/Game/DataTables/DT_Ghost.DT_Ghost" _array_element)
          (:`then`
            (`KismetArrayLibrary.Array_Add` (`self.GhostDatas`) _returnvalue)))))
    (:`then_1`
      (bind _asbp_gs_in_game (cast `/Game/GameMode/BP_GS_InGame` (`GameplayStatics.GetGameState`)))
      (set `self.GameState` _asbp_gs_in_game))))

(event `BuildDelay`
  (`self.Has Athority in Dedi`
    (:`Authority`
      _)
    (:`Remote`
      _))
  (if (`self.IsBuildMode`)
    (`KismetSystemLibrary.Delay` 0.0)
    (`self.BuildCycle`)
    (else
      (`self.DestroyActor OS` (`self.BuildingGhost`) :!label _label)
      (set `self.CanBuild` false)
      (set `self.IsBuildMode` false))))

(event `StopBuildMode`
  (`self.Has Athority in Dedi`
    (:`Authority`
      (goto _label))
    (:`Remote`
      (goto _label))))

(event `LaunchBuildMode`
  (`self.Has Athority in Dedi`
    (:`Authority`
      _)
    (:`Remote`
      _))
  (`self.StopDeleteMode`)
  (set `self.IsBuildMode` true)
  (`self.BuildCycle`))

(event `DeleteDelay`
  (`self.Has Athority in Dedi`
    (:`Authority`
      _)
    (:`Remote`
      _))
  (if (`self.IsDeleteMode`)
    (`KismetSystemLibrary.Delay` 0.0)
    (`self.DeleteCycle`)
    (else
      (set `self.IsDeleteMode` false :!label _label)
      (cast `/Game/Assets/Building/BaseBlueprints/BP_BuildingBase` (`self.Deleting Actor`))
      (`self.DespawnDeletingBuildingOutline`))))

(event `StopDeleteMode`
  (`self.Has Athority in Dedi`
    (:`Authority`
      (goto _label))
    (:`Remote`
      (goto _label))))

(event `LaunchDeleteMode`
  (`self.Has Athority in Dedi`
    (:`Authority`
      _)
    (:`Remote`
      _))
  (`self.StopBuildMode`)
  (set `self.IsDeleteMode` true)
  (`self.DeleteCycle`))

(event `Initialize OS`
  (params (Character :type "/Game/Assets/Characters/Player/ConquerorBot/Blueprints/BP_ConquerorBot Object Reference") (MaxDistanceToSpawn :type "Float (double-precision)") (InstantlySpawnBuildingGhost :type Boolean))
  (set `self.Character` Character)
  (set `self.MaxDistanceToSpawn` MaxDistanceToSpawn)
  (if InstantlySpawnBuildingGhost
    (`self.SpawnBuildingGhost`)))

(event `DestroyActor OS`
  (params (Actor :type "Actor Object Reference"))
  (`/Engine/EditorBlueprintResources/StandardMacros.IsValid` Actor
    (:`Is Valid`
      (`Actor.K2_DestroyActor` Actor))))

(event `SetBuildingGhostRotation OS`
  (params (Target :type "Actor Object Reference") (NewRotation :type "Rotator Structure"))
  (`Actor.K2_SetActorRotation` Target NewRotation false))

(event `SpawnBuilding OS`
  (params (Class :type "/Game/Assets/Building/BaseBlueprints/BP_BuildingBase Class Reference") (`Spawn Transform` :type "Transform Structure") (CollisionHandlingOverride :type "ESpawnActorCollisionHandlingMethod Enum" :default "Undefined") (`Expendable Costs` :type "Map of /Game/EnumClasses/E_Expendable Enum to Integer") (IsGhost :type Boolean) (`Ghost Color` :type "/Game/EnumClasses/E_BuildingOutlineColor Enum" :default "NewEnumerator0") (OriginalBuilding :type "/Game/Assets/Building/BaseBlueprints/BP_BuildingBase Object Reference") (IsSpawned :type Boolean) (EnvironmentalSound :type "/Game/Structs/S_AudioProperty Structure"))
  ;[0 0.9839 1] Building Cycle
  (`|SpawnActorFromClass` Class `Spawn Transform` CollisionHandlingOverride "OverrideRootScale" null `Expendable Costs` IsGhost `Ghost Color` OriginalBuilding false EnvironmentalSound 100.0 IsSpawned null))

(event `SpawnBuildingGhost OS`
  (params (`Spawn Transform` :type "Transform Structure") (CollisionHandlingOverride :type "ESpawnActorCollisionHandlingMethod Enum" :default "Undefined") (Owner :type "Actor Object Reference") (Instigator :type "Pawn Object Reference"))
  (bind _buildingghost (`self.BuildingGhost`))
  (bind _output_mesh (break `/Game/Structs/S_BD_GhostData` (`|GetArrayItem` (`self.GhostDatas`) (`self.DataID`))))
  ;[0 0.9839 1] Building Cycle
  (bind _returnvalue (`|SpawnActorFromClass` "/Game/Assets/Building/BaseBlueprints/BP_BuildingGhost.BP_BuildingGhost_C" `Spawn Transform` CollisionHandlingOverride "OverrideRootScale" Owner Instigator))
  (`/Engine/EditorBlueprintResources/StandardMacros.IsValid` _buildingghost
    (:`Is Valid`
      (`Actor.K2_DestroyActor` _buildingghost))
    (:`Is Not Valid`
      _))
  (bind _output_get (set `self.BuildingGhost` _returnvalue))
  (`/Game/Assets/Building/BaseBlueprints/BP_BuildingGhost.Initialize` _output_get _output_mesh))

(event `SetGhostLocation OS`
  (params (NewLocation :type "Vector Structure"))
  (bind _buildingghost (`self.BuildingGhost`))
  ;[0 0.9839 1] Building Cycle
  (`/Engine/EditorBlueprintResources/StandardMacros.IsValid` _buildingghost
    (:`Is Valid`
      (`Actor.K2_SetActorLocation` _buildingghost NewLocation false true))))

(event `PayResource OS`
  (params (BuildingID :type Integer))
  ;[1 1 1] Pay Resource
  (`self.PayResource MC` BuildingID))

(event `PayResource MC`
  (params (`Building ID` :type Integer))
  (bind (_output_mesh _output_actor _output_cost _output_buildingname _output_interactiontext _output_interactionwidget _output_environmentalsound) (break `/Game/Structs/S_BD_GhostData` (`|GetArrayItem` (`self.GhostDatas`) `Building ID`)))
  ;[1 1 1] Pay Resource
  (bind _ispaid (`/Game/GameMode/BP_GS_InGame.Pay Resources` (`self.GameState`) _output_cost))
  (if (and _ispaid (`self.IsOwnerClient`))
    (set `self.IsOwnerClient` false)
    (`self.SpawnBuilding OS` _output_actor (`Actor.GetTransform` (`self.BuildingGhost`)) "Undefined" _output_cost false "NewEnumerator0" null true _output_environmentalsound)))

(event `RefundResource OS`
  (params (Building :type "/Game/Assets/Building/BaseBlueprints/BP_BuildingBase Object Reference"))
  (`self.RefundResource MC` Building))

(event `RefundResource MC`
  (params (Building :type "/Game/Assets/Building/BaseBlueprints/BP_BuildingBase Object Reference"))
  (`/Game/GameMode/BP_GS_InGame.Refund Resources` (`self.GameState`) (`/Game/Assets/Building/BaseBlueprints/BP_BuildingBase.ExpendableCosts` Building))
  (`self.DestroyActor OS` Building))

(fn `BuildCycle`
  (`/Engine/EditorBlueprintResources/StandardMacros.IsValid` (`self.BuildingGhost`)
    (:`Is Valid`
      (bind (_outhit _returnvalue) (`self.GetTracedHit`))
      (if _returnvalue
        (bind (_bblockinghit _binitialoverlap _time _distance _location _impactpoint _normal _impactnormal _physmat _hitactor _hitcomponent _hitbonename _bonename _hititem _elementindex _faceindex _tracestart _traceend) (`GameplayStatics.BreakHitResult` _outhit))
        (`self.SetGhostLocation OS` _impactpoint)
        ;[1 1 0] Lagacy
        (`Actor.K2_SetActorLocation` (`self.BuildingGhost`) _impactpoint false true)
        (bind _hit (`self.CheckOverlap`))
        (if _hit
          (set `self.CanBuild` false :!label _label)
          (`/Game/Assets/Building/BaseBlueprints/BP_BuildingGhost.SetOutlineColor` (`self.BuildingGhost`) "NewEnumerator1")
          (else
            (set `self.CanBuild` true)
            (`/Game/Assets/Building/BaseBlueprints/BP_BuildingGhost.SetOutlineColor` (`self.BuildingGhost`) "NewEnumerator0")))
        (else
          (`self.SetGhostLocation OS` _traceend)
          (`Actor.K2_SetActorLocation` (`self.BuildingGhost`) _traceend false true)
          (goto _label)))
      (`self.BuildDelay`))
    (:`Is Not Valid`
      (`self.SpawnBuildingGhost`)
      (`self.BuildDelay`))))

(fn `ChangeBuildingGhost`
  (params (DataID :type Integer))
  (bind _buildingghost (`self.BuildingGhost`))
  (`/Engine/EditorBlueprintResources/StandardMacros.IsValid` _buildingghost
    (:`Is Valid`
      (`/Game/Assets/Building/BaseBlueprints/BP_BuildingGhost.ChangeMeshes` _buildingghost null))
    (:`Is Not Valid`
      (`self.SpawnBuildingGhost`))))

(fn `CheckOverlap`
  (returns (Hit :type Boolean))
  (locals (IsHit :type Boolean))
  (bind _staticmesh (`/Game/Assets/Building/BaseBlueprints/BP_BuildingGhost.StaticMesh` (`self.BuildingGhost`)))
  (bind (_origin _boxextent) (`KismetSystemLibrary.GetComponentBounds` _staticmesh))
  (bind (_outhits _returnvalue) (`KismetSystemLibrary.BoxTraceMulti` :`Start` _origin :`End` _origin :`HalfSize` (/ _boxextent 1.4) :`Orientation` (`SceneComponent.K2_GetComponentRotation` _staticmesh) :`TraceChannel` "TraceTypeQuery1" :`DrawTime` (`GameplayStatics.GetWorldDeltaSeconds`)))
  (if _returnvalue
    (set `local.IsHit` false)
    (for _array_element _outhits
      (bind _returnvalue_2 (`PrimitiveComponent.GetCollisionObjectType` (`.HitComponent` (`GameplayStatics.BreakHitResult` _array_element))))
      (if (not (or (`|EnumEquality` _returnvalue_2 "ECC_GameTraceChannel8") (`|EnumEquality` _returnvalue_2 "ECC_GameTraceChannel1")))
        (set `local.IsHit` true)
        (break)))
    (return (`local.IsHit`))
    (else
      (return false))))

(fn `DeleteBuilding`
  (bind _asbp_building_base (cast `/Game/Assets/Building/BaseBlueprints/BP_BuildingBase` (`self.Deleting Actor`)))
  (`self.RefundResource OS` _asbp_building_base))

(fn `DeleteCycle`
  (bind (_start _end) (`self.GetTraceStartEnd`))
  (bind (_outhit _returnvalue) (`KismetSystemLibrary.LineTraceSingle` _start _end "TraceTypeQuery1"))
  (if _returnvalue
    (cast `/Game/Assets/Building/BaseBlueprints/BP_BuildingBase` (`self.Deleting Actor`)
      (:`then`
        (bind (_bblockinghit _binitialoverlap _time _distance _location _impactpoint _normal _impactnormal _physmat _hitactor) (`GameplayStatics.BreakHitResult` _outhit))
        (if (not (== _hitactor (`self.Deleting Actor`)))
          (`self.DespawnDeletingBuildingOutline`)
          (bind _output_get (set `self.Deleting Actor` _hitactor :!label _label))
          (bind _asbp_building_base (cast `/Game/Assets/Building/BaseBlueprints/BP_BuildingBase` _output_get)
            (:`then`
              (`self.SpawnDeletingBuildingOutline` _asbp_building_base "NewEnumerator2"))
            (:`CastFailed`
              (set `self.Deleting Actor` null :!label _label_2)))))
      (:`CastFailed`
        (goto _label)))
    (else
      (cast `/Game/Assets/Building/BaseBlueprints/BP_BuildingBase` (`self.Deleting Actor`)
        (:`then`
          (`self.DespawnDeletingBuildingOutline`)
          (goto _label_2))
        (:`CastFailed`
          (goto _label_2)))))
  (`self.DeleteDelay`))

(fn `DespawnDeletingBuildingOutline`
  (`self.Has Athority in Dedi`
    (:`Authority`
      _)
    (:`Remote`
      _))
  (`Actor.K2_DestroyActor` (`self.DeletingGhost`)))

(fn `Initialize`
  (params (Character :type "/Game/Assets/Characters/Player/ConquerorBot/Blueprints/BP_ConquerorBot Object Reference") (MaxDistanceToSpawn :type "Float (double-precision)") (InstantlySpawnBuildingGhost :type Boolean :default true))
  (`self.Initialize OS` Character MaxDistanceToSpawn InstantlySpawnBuildingGhost))

(fn `NextBuilding`
  (bind _output_mesh (break `/Game/Structs/S_BD_GhostData` (`|GetArrayItem` (`self.GhostDatas`) (`self.DataID`))))
  (bind _returnvalue (+ (`self.DataID`) 1))
  (if (>= _returnvalue (`KismetArrayLibrary.Array_Length` (`self.GhostDatas`)))
    (set `self.DataID` 0)
    (else
      (set `self.DataID` _returnvalue)))
  (`/Game/Assets/Building/BaseBlueprints/BP_BuildingGhost.ChangeMeshes` (`self.BuildingGhost`) _output_mesh))

(fn `PrevBuilding`
  (bind _output_mesh (break `/Game/Structs/S_BD_GhostData` (`|GetArrayItem` (`self.GhostDatas`) (`self.DataID`))))
  (bind _returnvalue (- (`self.DataID`) 1))
  (if (< _returnvalue 0)
    (set `self.DataID` (- (`KismetArrayLibrary.Array_Length` (`self.GhostDatas`)) 1))
    (else
      (set `self.DataID` _returnvalue)))
  (`/Game/Assets/Building/BaseBlueprints/BP_BuildingGhost.ChangeMeshes` (`self.BuildingGhost`) _output_mesh))

(fn `RotateBuildingGhost`
  (params (Yaw :type "Float (double-precision)"))
  (`/Engine/EditorBlueprintResources/StandardMacros.IsValid` (`self.BuildingGhost`)
    (:`Is Valid`
      (`self.SetBuildingGhostRotation OS` (`self.BuildingGhost`) (`KismetMathLibrary.MakeRotator` (.roll (`Actor.K2_GetActorRotation` (`self.BuildingGhost`))) (.pitch (`Actor.K2_GetActorRotation` (`self.BuildingGhost`))) (+ Yaw (.yaw (`Actor.K2_GetActorRotation` (`self.BuildingGhost`)))))))))

(fn `SpawnBuilding`
  (set `self.IsOwnerClient` true)
  (if (`self.CanBuild`)
    (`self.PayResource OS` (`self.DataID`))))

(fn `SpawnBuildingGhost`
  (bind _character (`self.Character`))
  (bind _character_2 (`self.Character`))
  (bind (_outhit _returnvalue) (`self.GetTracedHit`))
  (if _returnvalue
    (bind (_bblockinghit _binitialoverlap _time _distance _location _impactpoint _normal _impactnormal _physmat _hitactor _hitcomponent _hitbonename _bonename _hititem _elementindex _faceindex _tracestart _traceend) (`GameplayStatics.BreakHitResult` _outhit))
    (`self.SpawnBuildingGhost OS` (`KismetMathLibrary.MakeTransform` _impactpoint) "Undefined" _character _character)
    (else
      (`self.SpawnBuildingGhost OS` (`KismetMathLibrary.MakeTransform` _traceend) "Undefined" _character_2 _character_2))))

(fn `SpawnDeletingBuildingOutline`
  (params (Building :type "/Game/Assets/Building/BaseBlueprints/BP_BuildingBase Object Reference") (OutlineColor :type "/Game/EnumClasses/E_BuildingOutlineColor Enum" :default "NewEnumerator0"))
  (bind _returnvalue (`|SpawnActorFromClass` (`GameplayStatics.GetObjectClass` Building) (`Actor.GetTransform` Building) "Undefined" "OverrideRootScale" null (`|MakeMap` "NewEnumerator0" :!type "/Game/EnumClasses/E_Expendable Enum") true "NewEnumerator2" Building false (struct) 100.0 true null))
  (set `self.DeletingGhost` _returnvalue))