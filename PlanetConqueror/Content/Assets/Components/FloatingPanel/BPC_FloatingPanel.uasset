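; Widget component that floats a resource-increase notice (image and amount) along a set direction, optionally facing the player camera.
; StartFloating runs a zero-delay loop while active, easing position with EaseOutBack and setting opacity from fade thresholds, then resets hidden at the start location.
; The fade-in formula lowers opacity from 1 to 0 before jumping to full.
; SetPanel fills the notice widget; SetPanelFloatingTimeByDefault caps duration at the default.
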(event `self.ReceiveBeginPlay`
  (bind _output_get (set `self.FadeInStartTimeRate` (`KismetMathLibrary.FClamp` (`self.FadeInStartTimeRate`))))
  (set `self.FadeOutStartTimeRate` (`KismetMathLibrary.FClamp` (`self.FadeOutStartTimeRate`) _output_get))
  (set `self.FloatingDirection` (`KismetMathLibrary.Normal` (`self.FloatingDirection`)))
  (`self.InitFloating`)
  (`self.SetCastShadow` false)
  (set `self.RealFloatingTime` (`self.DefaultFloatingTime`)))

(event `StartFloating`
  (if (`self.IsAcvated`) :!label _label
    (`|ExecutionSequence`
      (:`then_0`
        ;[1 1 1] Look at Player
        (if (`self.IsLookingAtPlayer`)
          (`self.LookAtPlayer`)))
      (:`then_1`
        (`self.FloatingCycle`)))))

(event `FloatingDelay`
  (`KismetSystemLibrary.Delay` 0.0)
  (goto _label))

(fn `FloatingCycle`
  (bind _initlocation (`self.InitLocation`))
  (bind _fadeinstarttimerate (`self.FadeInStartTimeRate`))
  (bind _fadeoutstarttimerate (`self.FadeOutStartTimeRate`))
  (bind _result (`/Game/Macros/GlobalMacros.EaseOutBack (vector)` (`self.EaseAlpha`) _initlocation (+ _initlocation (* (`self.FloatingDirection`) (`self.Distance`)))))
  (if (>= (`self.EaseAlpha`) 1.0)
    (`self.K2_SetRelativeLocation` _result)
    (`self.InitFloating`)
    (else
      (`self.K2_SetRelativeLocation` _result)
      (`|ExecutionSequence`
        (:`then_0`
          ;[1 1 1] Set Ease Alpha
          (set `self.EaseAlpha` (`KismetMathLibrary.FMin` (+ (`self.EaseAlpha`) (* (/ 1.0 (`self.RealFloatingTime`)) (`GameplayStatics.GetWorldDeltaSeconds`))) 1.0)))
        (:`then_1`
          ;[1 1 1] Fade In Process
          (`/Game/Macros/GlobalMacros.Compare In Range (float)` (`self.EaseAlpha`) (`self.FadeInStartTimeRate`) (`self.FadeOutStartTimeRate`)
            (:`Value < Min`
              (`Widget.SetRenderOpacity` (`self.GetWidget`) (/ (- _fadeinstarttimerate (`self.EaseAlpha`)) _fadeinstarttimerate) :!label _label))
            (:`Value == Min`
              (goto _label))
            (:`Value In Range`
              (`Widget.SetRenderOpacity` (`self.GetWidget`) 1.0))
            (:`Value == Max`
              ;[1 1 1] Fade Out Process
              (`/Game/Macros/GlobalMacros.Compare on Equality (float)` (`self.EaseAlpha`) 1.0 :!label _label_2
                (:`<`
                  (`Widget.SetRenderOpacity` (`self.GetWidget`) (- 1.0 (/ (- (`self.EaseAlpha`) _fadeoutstarttimerate) (- 1.0 _fadeoutstarttimerate)))))
                (:`==`
                  (`Widget.SetRenderOpacity` (`self.GetWidget`) 0.0 :!label _label_3))
                (:`>`
                  (goto _label_3))))
            (:`Value > Max`
              (goto _label_2))))
        (:`then_2`
          (`self.FloatingDelay`))))))

(fn `InitFloating`
  (set `self.EaseAlpha` 0.0)
  (`self.K2_SetRelativeLocation` (`self.InitLocation`))
  (`Widget.SetRenderOpacity` (`self.GetWidget`) 0.0))

(fn `LookAtPlayer`
  (bind _returnvalue (`GameplayStatics.GetPlayerCameraManager` 0))
  ;[1 1 1] Player의 화면을 바라보도록 위치 구하기
  (`/Engine/EditorBlueprintResources/StandardMacros.IsValid` _returnvalue
    (:`Is Valid`
      (set `self.PlayerCameraLocation` (`PlayerCameraManager.GetCameraLocation` _returnvalue))
      (`self.K2_SetWorldRotation` (`KismetMathLibrary.FindLookAtRotation` (`self.K2_GetComponentLocation`) (`self.PlayerCameraLocation`)) false true))))

(fn `SetPanel`
  (params (Image :type "Texture2D Object Reference") (Increase :type Integer))
  (bind _aswbp_increasing_resource_notice (cast `/Game/Widget/BuildingWidgets/Blueprints/WBP_IncreasingResourceNotice` (`self.GetWidget`)))
  (set `/Game/Widget/BuildingWidgets/Blueprints/WBP_IncreasingResourceNotice.ResourceImageTexture` Image _aswbp_increasing_resource_notice)
  (set `/Game/Widget/BuildingWidgets/Blueprints/WBP_IncreasingResourceNotice.IncreasingAmount` Increase _aswbp_increasing_resource_notice))

(fn `SetPanelFloatingTimeByDefault`
  (params (FloatingTime :type "Float (double-precision)"))
  (bind _defaultfloatingtime (`self.DefaultFloatingTime`))
  (if (< FloatingTime _defaultfloatingtime)
    (set `self.RealFloatingTime` FloatingTime)
    (else
      (set `self.RealFloatingTime` _defaultfloatingtime))))