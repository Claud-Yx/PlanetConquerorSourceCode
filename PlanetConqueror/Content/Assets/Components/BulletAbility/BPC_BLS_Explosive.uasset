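; Bullet ability component that makes its bullet explode when the component ends play.
; EndPlay spawns a Niagara explosion scaled by range and, only if that spawn is valid, runs a sphere trace at the bullet's location.
; Each distinct actor hit receives one HitWithCheck call through the bullet, using CacluatedDamage, whose percentage-plus-absolute formula appears unconnected.
; Initialize supplies range, damage settings and effect; the Hit override is empty.
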(event `self.ReceiveEndPlay`
  (params (EndPlayReason :type "EEndPlayReason Enum" :default "Destroyed"))
  (bind _returnvalue (`Actor.K2_GetActorLocation` (`self.BulletRef`)))
  (bind _returnvalue_2 (`NiagaraFunctionLibrary.SpawnSystemAtLocation` (`self.VFX_HitExplosion`) (`Actor.K2_GetActorLocation` (`self.BulletRef`))))
  (`/Engine/EditorBlueprintResources/StandardMacros.IsValid` _returnvalue_2
    (:`Is Valid`
      (`FXSystemComponent.SetFloatParameter` _returnvalue_2 "Overall_Scale" (* (`self.ExplosiveRange`) 0.01))
      (bind _outhits (`KismetSystemLibrary.SphereTraceMulti` _returnvalue _returnvalue (`self.ExplosiveRange`) "TraceTypeQuery6"))
      (for _array_element _outhits
        (bind (_bblockinghit _binitialoverlap _time _distance _location _impactpoint _normal _impactnormal _physmat _hitactor) (`GameplayStatics.BreakHitResult` _array_element))
        (if (not (`KismetArrayLibrary.Array_Contains` (`self.DamagedActors`) _hitactor))
          (`/Game/Assets/Bullet/Blueprints/BP_Bullet.Hit with Check` (`self.BulletRef`) _array_element (+ (* (`/Game/Assets/Bullet/Blueprints/BP_Bullet.Damage` (`self.BulletRef`)) (* (`self.ExplosivePercentageDamage`) 0.01)) (`self.ExplosiveAbsoluteDamage`)))
          (`KismetArrayLibrary.Array_Add` (`self.DamagedActors`) _hitactor))))))

(fn `Hit`
  (params (HitComponent :type "PrimitiveComponent Object Reference") (OtherActor :type "Actor Object Reference") (OtherComp :type "PrimitiveComponent Object Reference") (NormalImpulse :type "Vector Structure") (Hit :type "HitResult Structure")))

(fn `Initialize`
  (params (OriginalDamage :type "Float (double-precision)") (ExplosiveRange :type "Float (double-precision)") (ExplosiveAbsoluteDamage :type "Float (double-precision)") (ExplosivePercentageDamage :type "Float (double-precision)") (HitExplosion :type "NiagaraSystem Object Reference"))
  (`|ExecutionSequence`
    (:`then_0`
      (set `self.OriginalDamage` OriginalDamage))
    (:`then_1`
      (set `self.ExplosiveRange` ExplosiveRange))
    (:`then_2`
      (set `self.ExplosiveAbsoluteDamage` ExplosiveAbsoluteDamage))
    (:`then_3`
      (set `self.ExplosivePercentageDamage` ExplosivePercentageDamage))
    (:`then_4`
      (set `self.VFX_HitExplosion` HitExplosion))))