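; Weapon muzzle component that fires replicated BP_Bullet actors using stats passed to Initialize.
; Shoot gates on cooldown, burst and ammo, then loops bursts via Delay, spawning muzzle VFX and calling server event ShootOS.
; ShootOS spawns pellets with sound, cone spread and extra damage, rotating the muzzle toward the AimObject's line-trace target; Tick resets that rotation.
; Helpers handle reload, fire rate (BPM) and bonus damage.
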(event `self.ReceiveTick`
  (params (DeltaSeconds :type "Float (single-precision)"))
  ;[1 1 1] Event Tick
  (`self.K2_SetRelativeRotation` (struct))
  ;;[0.7274 0.9968 1] 발사 쿨다운 감소
  (if (not (<= (`self.CurShotCooldown`) 0.0))
    (set `self.CurShotCooldown` (- (`self.CurShotCooldown`) DeltaSeconds))))

(event `Shoot`
  (params (AimObject :type "SceneComponent Object Reference") (TraceStartOffset :type "Vector Structure") (TracedTargetMinDist :type "Float (double-precision)"))
  (bind (_value _returnvalue) (`BlueprintMapLibrary.Map_Find` (`.VFX_21_EDDB9C01427162EE1EA862BD6DBA1312` (break `/Game/Structs/S_BL_Data` (`self.BulletData`))) "NewEnumerator1"))
  ;[1 1 0.467] Shoot
  ;;[0.7274 0.9968 1] 발사 가능 여부 확인
  (if (`self.CanShoot`)
    ;;[1 1 1] 발사 가능하다면 점사 회수 초기화
    (set `self.CurBurstCount` (`self.BurstCount`))
    ;;[1 1 1] 점사 회수가 남았는가
    (if (> (`self.CurBurstCount`) 0) :!label _label
      (if _returnvalue
        ;;[0.7274 0.9968 1] Muzzle Flash VFX Spawning
        (bind _returnvalue_2 (`NiagaraFunctionLibrary.SpawnSystemAttached` _value self "None" (0.0 0.0 0.0) (struct) "KeepRelativeOffset" true))
        (set `self.VFX` _returnvalue_2))
      ;;[0.7274 0.9968 1] 최대 총알이 0 이거나
      ;; 현재 총알이 0 미만 이라면
      (if (or (< 0 (`self.CurAmmo`)) (== (`self.AmmoMax`) 0))
        (`self.Shoot OS` AimObject TraceStartOffset TracedTargetMinDist (`self.ExtraDamage`))
        ;;[0.7274 0.9968 1] Ammo 및 Burst Count 소모
        (if (not (== (`self.AmmoMax`) 0))
          (set `self.CurAmmo` (- (`self.CurAmmo`) 1)))
        (set `self.CurBurstCount` (- (`self.CurBurstCount`) 1))
        ;;[0.7274 0.9968 1] 점사 지연 후 다시 발사
        (`KismetSystemLibrary.Delay` (`self.BurstDelay`))
        (goto _label)
        (else
          _)))
    ;;[0.7274 0.9968 1] 발사 초기화
    (set `self.CurShotCooldown` (`self.SecondsPerBullet`))
    (set `self.CurBurstCount` -1)))

(event `Shoot OS`
  (params (AimObject :type "SceneComponent Object Reference") (TraceStartOffset :type "Vector Structure") (TracedTargetMinDist :type "Float (double-precision)") (ExtraDamage :type "Float (double-precision)"))
  (bind (_bulletdata_mesh _bulletdata_vfx _bulletdata_sfx) (break `/Game/Structs/S_BL_Data` (`self.BulletData`)))
  (bind _bulletdata (`self.BulletData`))
  (bind (_mesh _vfx _sfx _baseability _specialabilitycomponents _specialability _excepttargets) (break `/Game/Structs/S_BL_Data` _bulletdata))
  (bind (_itemappearancedata _volume _starttime _attenuation) (break `/Game/Structs/S_AudioProperty` (`BlueprintMapLibrary.Map_Find` _bulletdata_sfx "NewEnumerator1")))
  (bind _s_bl_data (make `/Game/Structs/S_BL_Data` _mesh _vfx _sfx _baseability _specialabilitycomponents _specialability _excepttargets))
  (bind _returnvalue (+ (`.Damage_8_95FA65794938F8646CAD6B9925CAF05F` (break `/Game/Structs/S_BL_Base` (`.BaseAbility_8_9AC7F1424787AED21383DDB4C16A02F5` (break `/Game/Structs/S_BL_Data` _bulletdata)))) (`self.ExtraDamage`)))
  ;[0.5298 0.5087 1] Shoot On Server
  (set `self.TraceStartOffset` TraceStartOffset)
  (set `self.TracedTargetMinDist` TracedTargetMinDist)
  (set `self.AimObject` AimObject)
  (set `self.ExtraDamage` ExtraDamage)
  ;;[0.7274 0.9968 1] 한 발 당 총알 수
  (for _ (range (+ (`self.BuckCount`) 1))
    ;;[0.7274 0.9968 1] Bullet 소환
    (bind _returnvalue_2 (`|SpawnActorFromClass` "/Game/Assets/Bullet/Blueprints/BP_Bullet.BP_Bullet_C" (`KismetMathLibrary.MakeTransform` (`self.K2_GetComponentLocation`) (`KismetMathLibrary.Conv_VectorToRotator` (`self.GetForwardVector`))) "Undefined" "OverrideRootScale" null null))
    (`/Engine/EditorBlueprintResources/StandardMacros.IsValid` (`self.AimObject`)
      (:`Is Valid`
        (`self.CalcAimmingTarget`))
      (:`Is Not Valid`
        _))
    (`Actor.SetReplicates` _returnvalue_2 true)
    (`Actor.SetReplicateMovement` _returnvalue_2 false)
    (bind _output_get (set `self.ShotDirection` (`KismetMathLibrary.RandomUnitVectorInConeInRadians` (`self.GetForwardVector`) (`self.SpreadRadians`))))
    (bind _structout (setmembers `/Game/Structs/S_BL_Base` :`StructRef` (`.BaseAbility_8_9AC7F1424787AED21383DDB4C16A02F5` (break `/Game/Structs/S_BL_Data` _s_bl_data)) :`Damage` _returnvalue))
    (bind _structout_2 (setmembers `/Game/Structs/S_BL_Data` :`StructRef` _s_bl_data :`BaseAbility` _structout))
    (set `self.CurBulletDamage` _returnvalue)
    ;;[0.7274 0.9968 1] 총알 데이터 초기화
    (`/Game/Assets/Bullet/Blueprints/BP_Bullet.Initialize OS` _returnvalue_2 (`self.Shooter`) (`self.CollisionStartDist`) _structout_2 _output_get true)
    (`GameplayStatics.SpawnSoundAtLocation` _itemappearancedata (`self.K2_GetComponentLocation`) (`self.K2_GetComponentRotation`) _volume 1.0 _starttime _attenuation null)))

(fn `CanShootExtern`
  (returns (CanShoot :type Boolean))
  (return (`self.CanShoot`)))

(fn `GetCurBPM`
  (returns (CurBPM :type "Float (double-precision)"))
  (return (`self.CurBPM`)))

(fn `GetExtraDamage`
  (returns (ExtraDamage :type "Float (double-precision)"))
  (return (`self.ExtraDamage`)))

(fn `GetOriginalBPM`
  (returns (OriginalBPM :type "Float (double-precision)"))
  (return (`self.OriginalBPM`)))

(fn `IncreaseBPM`
  (params (Value :type "Float (double-precision)") (BasedOnOriginalBPM :type Boolean))
  (if BasedOnOriginalBPM
    (`self.SetBPM` (+ Value (`self.OriginalBPM`)))
    (else
      (`self.SetBPM` (+ (`self.CurBPM`) Value)))))

(fn `IncreaseBulletExtraDamage`
  (params (Value :type "Float (double-precision)") (BasedOnOriginalDamage :type Boolean))
  (if BasedOnOriginalDamage
    (set `self.ExtraDamage` Value)
    (else
      (set `self.ExtraDamage` (+ Value (`self.ExtraDamage`))))))

(fn `Initialize`
  (params (Shooter :type "Actor Object Reference") (Data :type "/Game/Structs/S_MuzzleData Structure"))
  (bind _returnvalue (`self.K2_GetComponentLocation`))
  (bind (_bpm _ammomax _spreadadjustmenttargetdist _spreadextent) (break `/Game/Structs/S_MuzzleData` (`local.Data`)))
  (bind (_bpm_2 _ammomax_2 _spreadadjustmenttargetdist_2 _spreadextent_2 _burstcount _burstdelay _buckcount _bulletdata) (break `/Game/Structs/S_MuzzleData` (`local.Data`)))
  (bind _returnvalue_2 (+ (`self.K2_GetComponentLocation`) (* (`self.GetForwardVector`) _spreadadjustmenttargetdist)))
  ;[0 0.9839 1] Shooter Setting
  (set `self.Shooter` Shooter)
  (`|ExecutionSequence`
    (:`then_0`
      ;[0.7274 0.9968 1] Setting Stats
      (bind _output_get (set `self.OriginalBPM` _bpm_2))
      (`self.SetBPM` _output_get))
    (:`then_1`
      (bind _output_get_2 (set `self.AmmoMax` _ammomax_2))
      (set `self.CurAmmo` _output_get_2))
    (:`then_2`
      (set `self.BurstCount` _burstcount)
      (set `self.BurstDelay` _burstdelay))
    (:`then_3`
      (set `self.BuckCount` _buckcount))
    (:`then_4`
      (set `self.BulletData` _bulletdata))
    (:`then_5`
      ;;[0 0.9839 1] Default is -1
      (set `self.CurBurstCount` -1))
    (:`then_6`
      (if (== _spreadextent 0.0)
        ;[0 0.9839 1] 퍼지는 탄착군 넓이가 0이라면 각도도 0
        (set `self.SpreadRadians` 0.0)
        (else
          ;[0 0.9839 1] 퍼지는 탄착군 넓이가 0 초과일 때
          (bind _radians (`/Game/Macros/GlobalFunctions.Get Radians from Vectors` (- _returnvalue_2 _returnvalue) (- (+ _returnvalue_2 (* (`self.GetUpVector`) _spreadextent)) _returnvalue)))
          (set `self.SpreadRadians` _radians))))))

(fn `Reload`
  (set `self.CurAmmo` (`self.AmmoMax`)))

(fn `SetBPM`
  (params (BPM :type "Float (double-precision)"))
  (bind _output_get (set `self.CurBPM` BPM))
  (bind _output_get_2 (set `self.SecondsPerBullet` (/ 60.0 _output_get)))
  (set `self.CurShotCooldown` _output_get_2))