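; Harvestable mining resource (such as an oak or lignite) that takes swing damage and throws item pickups toward the player.
; Construction loads HP, mesh, hit sound and loot rules from DT_MiningResourceData by Type, then pre-rolls hit and destroy item queues.
; Hits pop queued items with Niagara and sound effects.
; At negative HP it drops the remainder, swaps to a per-type Chaos Geometry Collection shattered by a short-lived field, then destroys itself.
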(event `self.ReceiveBeginPlay`
  (`parent.ReceiveBeginPlay`)
  (`BoxComponent.SetBoxExtent` (`self.Box`) (`.BoxExtent` (`KismetSystemLibrary.GetComponentBounds` (`self.Mesh`))) true))

(event `/Game/Interfaces/BPI_SwingDamageble.TakeSwingDamage`
  (params (Damage :type "Float (double-precision)") (Hit :type "HitResult Structure") (Swinger :type "Actor Object Reference") (HitVFX :type "NiagaraSystem Object Reference"))
  (bind (_bblockinghit _binitialoverlap _time _distance _location) (`GameplayStatics.BreakHitResult` Hit))
  (bind _returnvalue (`self.K2_GetActorLocation` Swinger))
  (bind (_sfx_swinghit_itemappearancedata _sfx_swinghit_volume _sfx_swinghit_starttime _sfx_swinghit_attenuation) (break `/Game/Structs/S_AudioProperty` (`self.SFX_SwingHit`)))
  (bind _output_get (set `self.CurHP` (- (`self.CurHP`) Damage)))
  (`NiagaraFunctionLibrary.SpawnSystemAtLocation` "/Game/Import/VFX/ToonHIt/NS_ToonHit.NS_ToonHit" _location)
  (`GameplayStatics.PlaySoundAtLocation` _sfx_swinghit_itemappearancedata _location (struct) _sfx_swinghit_volume 1.0 _sfx_swinghit_starttime _sfx_swinghit_attenuation null null null)
  (if (< _output_get 0.0)
    (`/Engine/EditorBlueprintResources/StandardMacros.DoOnce` false
      (:`Completed`
        (set `self.IsDestroyed` true)
        (`self.PopItemByDestroying` _location _returnvalue)
        (`/Game/Interfaces/BPI_ChaosDestructable.SpawnChaosDestruct` "All")
        (`KismetSystemLibrary.Delay` 4.0)
        (`self.K2_DestroyActor`)))
    (else
      (`self.PopItemByHitting` 1 1 _location _returnvalue))))

(event `/Game/Interfaces/BPI_ChaosDestructable.SpawnChaosDestruct`
  (params (Part :type Name))
  (`self.SetActorEnableCollision` false)
  (`SceneComponent.SetVisibility` (`self.DefaultSceneRoot`) false true)
  (bind _geometrycollection (`self.SpawnGC`))
  (`KismetSystemLibrary.Delay` 4.0)
  (`ActorComponent.K2_DestroyComponent` _geometrycollection))

(fn `Get Force`
  (returns (ForceType :type "/Game/EnumClasses/E_ForceType Enum"))
  (return "NewEnumerator6"))

(fn `GetDataFromTable`
  (bind _returnvalue (`|GetDataTableRow` "/Game/DataTables/DT_MiningResourceData.DT_MiningResourceData" (`KismetStringLibrary.Conv_StringToName` (`|GetEnumeratorNameAsString` (`self.Type`))))
    (:`then`
      (`|ExecutionSequence`
        (:`then_0`
          (bind (_type _mesh _hp _itemdatabydestroying _itemdatabyhit _sfx) (break `/Game/Structs/S_MiningResourceData` _returnvalue))
          (set `self.HP Max` _hp))
        (:`then_1`
          (set `self.DestroyItemData` _itemdatabydestroying))
        (:`then_2`
          (set `self.HitItemData` _itemdatabyhit))
        (:`then_3`
          (`StaticMeshComponent.SetStaticMesh` (`self.Mesh`) _mesh))
        (:`then_4`
          (set `self.SFX_SwingHit` (`BlueprintMapLibrary.Map_Find` _sfx "NewEnumerator5")))))))

(fn `Init`
  (bind (_destroyitemdata_mustcreateitems _destroyitemdata_itemchances _destroyitemdata_mintypes _destroyitemdata_maxtypes) (break `/Game/Structs/S_ItemAppearanceData` (`self.DestroyItemData`)))
  (bind (_hititemdata_mustcreateitems _hititemdata_itemchances _hititemdata_mintypes _hititemdata_maxtypes) (break `/Game/Structs/S_ItemAppearanceData` (`self.HitItemData`)))
  (set `self.CurHP` (`self.HP Max`))
  (bind _selecteditems (`/Game/Macros/GlobalFunctions.GetRandomItems` _destroyitemdata_mustcreateitems _destroyitemdata_itemchances _destroyitemdata_mintypes _destroyitemdata_maxtypes))
  (set `self.DestroyItems` _selecteditems)
  (bind _selecteditems_2 (`/Game/Macros/GlobalFunctions.GetRandomItems` _hititemdata_mustcreateitems _hititemdata_itemchances _hititemdata_mintypes _hititemdata_maxtypes))
  (set `self.HitItems` _selecteditems_2))

(fn `PopItemByDestroying`
  (params (SpawnLocation :type "Vector Structure") (PlayerLocation :type "Vector Structure"))
  (`KismetArrayLibrary.Array_Append` (`self.DestroyItems`) (`self.HitItems`))
  (for (_array_element _array_index) (`self.DestroyItems`)
    (`self.SpawnItem` _array_element SpawnLocation PlayerLocation)
    (`KismetArrayLibrary.Array_Remove` (`self.DestroyItems`) _array_index)))

(fn `PopItemByHitting`
  (params (MinAmount :type Integer :default 1) (MaxAmount :type Integer :default 1) (SpawnLocation :type "Vector Structure") (PlayerLocation :type "Vector Structure"))
  (locals (PopCnt :type Integer :default 0))
  (set `local.PopCnt` (- (`KismetMathLibrary.RandomIntegerInRange` MinAmount MaxAmount) 1))
  (for _ (range (+ (`local.PopCnt`) 1))
    (bind _output (`/Game/Macros/GlobalMacros.Front` (`self.HitItems`))
      (:`Succeed`
        (`self.SpawnItem` _output SpawnLocation PlayerLocation)
        (`/Game/Macros/GlobalMacros.PopFront` (`self.HitItems`))))))

(fn `SpawnFSMasterField`
  (params (`FS Master Field Transform` :type "Transform Structure") (`Radial Magnitude` :type "Float (double-precision)") (`Directional Magnitude` :type "Float (double-precision)") (`Torque Mult` :type "Float (double-precision)"))
  (locals (FSMasterField :type "/Engine/EditorResources/FieldNodes/FS_MasterField Object Reference"))
  (bind _fsmasterfield (`local.FSMasterField`))
  (bind _returnvalue (`|SpawnActorFromClass` "/Engine/EditorResources/FieldNodes/FS_MasterField.FS_MasterField_C" (`KismetMathLibrary.MakeTransform` `FS Master Field Transform_Location` `FS Master Field Transform_Rotation` (`.BoxExtent` (`self.GetActorBounds` false true))) "AlwaysSpawn" "OverrideRootScale" null null))
  (set `local.FSMasterField` _returnvalue)
  (`|ExecutionSequence`
    (:`then_0`
      (set `/Engine/EditorResources/FieldNodes/FS_MasterField.Field Falloff Shape` "NewEnumerator0" (`local.FSMasterField`)))
    (:`then_1`
      (set `/Engine/EditorResources/FieldNodes/FS_MasterField.ActivationType` "NewEnumerator2" (`local.FSMasterField`)))
    (:`then_2`
      (`self.SetLifeSpan` (`local.FSMasterField`) 0.1))
    (:`then_3`
      (set `/Engine/EditorResources/FieldNodes/FS_MasterField.Radial Magnitude` (`local.Radial Magnitude`) (`local.FSMasterField`)))
    (:`then_4`
      (set `/Engine/EditorResources/FieldNodes/FS_MasterField.UseDirectionalVector` true _fsmasterfield)
      (set `/Engine/EditorResources/FieldNodes/FS_MasterField.DirectionalMagnitude` (`local.Directional Magnitude`) _fsmasterfield))
    (:`then_5`
      (set `/Engine/EditorResources/FieldNodes/FS_MasterField.TorqueMult` (`local.Torque Mult`) (`local.FSMasterField`)))))

(fn `SpawnGC`
  (returns (GeometryCollection :type "GeometryCollectionComponent Object Reference"))
  (bind _mesh (`self.Mesh`))
  (bind _mesh_2 (`self.Mesh`))
  (switch `/Game/EnumClasses/E_MiningResourceType` (`self.Type`)
    (:`NewEnumerator4`
      (bind _returnvalue (`AddComponent|NODE_AddGeometryCollectionComponent-0` :`RelativeTransform` (`SceneComponent.GetRelativeTransform` _mesh_2)))
      (`self.SpawnFSMasterField` (`SceneComponent.K2_GetComponentToWorld` _mesh_2) 50.0 20.0 1.3)
      (return _returnvalue))
    (:`NewEnumerator1`
      (bind _returnvalue_2 (`AddComponent|NODE_AddGeometryCollectionComponent-1` :`RelativeTransform` (`SceneComponent.GetRelativeTransform` _mesh)))
      (`self.SpawnFSMasterField` (`SceneComponent.K2_GetComponentToWorld` _mesh) 50.0 20.0 1.3)
      (return _returnvalue_2))))

(fn `SpawnItem`
  (params (Items :type "/Game/Structs/S_ItemAmount Structure") (SpawnLocation :type "Vector Structure") (PlayerLocation :type "Vector Structure"))
  (bind (_type _amount) (break `/Game/Structs/S_ItemAmount` Items))
  (bind (_returnvalue_roll _returnvalue_pitch _returnvalue_yaw) (`KismetMathLibrary.BreakRotator` (`KismetMathLibrary.FindLookAtRotation` SpawnLocation PlayerLocation)))
  (bind (_x _y _z) (`KismetMathLibrary.BreakVector3f` SpawnLocation))
  (bind _returnvalue (/ _returnvalue_yaw 10.0))
  (bind _returnvalue_2 (`|SpawnActorFromClass` "/Game/Assets/Item/Blueprints/BP_Item.BP_Item_C" (`KismetMathLibrary.MakeTransform` (`KismetMathLibrary.MakeVector` _x _y (+ _z 30.0))) "Undefined" "OverrideRootScale" null _amount (- _returnvalue 7.0) (+ _returnvalue 7.0) null))
  (`/Game/Assets/Item/Blueprints/BP_Item.Initialize` :`self` _returnvalue_2 :`Type` _type :`InstantlyThrow` true))

(fn `UserConstructionScript`
  (`parent.UserConstructionScript`)
  (`self.GetDataFromTable`)
  (`self.Init`))