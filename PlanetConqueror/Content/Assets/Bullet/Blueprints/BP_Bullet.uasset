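; Networked projectile bullet, configured from init data with mesh, VFX, stats and special ability components such as Explosive.
; The authority drives flight, enabling collision past a start distance and destroying the bullet beyond max range.
; Hits damage BPI_BulletDamageble actors outside excepted forces and trigger each ability's hook.
; Multicasts replicate setup, velocity and hit VFX, with a macro separating dedicated server, authority and remote so cosmetics skip dedicated servers.
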(event `self.ReceiveBeginPlay`
  (`self.DEBUG_Initialize`))

(event `self.ReceiveTick`
  (params (DeltaSeconds :type "Float (single-precision)"))
  (`self.Has Athority in Dedi`
    (:`Authority in Dedi`
      _)
    (:`Authority`
      _))
  (`self.Fly`))

(event `self.HitCollision.OnComponentHit`
  (params (HitComponent :type "PrimitiveComponent Object Reference") (OtherActor :type "Actor Object Reference") (OtherComp :type "PrimitiveComponent Object Reference") (NormalImpulse :type "Vector Structure") (Hit :type "HitResult Structure (by ref)"))
  (`self.Has Athority in Dedi`
    (:`Authority in Dedi`
      _)
    (:`Authority`
      _))
  (`self.Hit` HitComponent OtherActor OtherComp NormalImpulse Hit))

(event `Initialize OS`
  (params (Shooter :type "Actor Object Reference") (CollisionStartDist :type "Float (double-precision)") (InitData :type "/Game/Structs/S_BL_Data Structure") (ShotDirection :type "Vector Structure") (InstantlyShoot :type Boolean))
  (`self.Initialize` Shooter CollisionStartDist InitData ShotDirection InstantlyShoot))

(event `Shoot MC`
  (params (Velocity :type "Vector Structure"))
  (`self.Has Athority in Dedi`
    (:`Authority`
      _)
    (:`Remote`
      (set `MovementComponent.Velocity` Velocity (`self.ProjectileMovement`))))
  (`ActorComponent.Activate` (`self.VFX`) true)
  (`self.Has Athority in Dedi`
    (:`Authority`
      (`SceneComponent.K2_SetWorldRotation` (`self.VFX`) (`KismetMathLibrary.Conv_VectorToRotator` (`self.ShotDirection`)) false false))))

(event `Initialize MC`
  (params (`Max Speed` :type "Float (single-precision)") (`Projectile Gravity Scale` :type "Float (single-precision)") (BulletVFX :type "NiagaraSystem Object Reference"))
  (bind _projectilemovement (`self.ProjectileMovement`))
  (bind _returnvalue (/ (`self.RangeMax`) (`self.Speed`)))
  (`|ExecutionSequence`
    (:`then_0`
      (`self.Has Athority in Dedi`
        (:`Remote`
          (`|ExecutionSequence`
            (:`then_0`
              (bind _output_get (set `ProjectileMovementComponent.MaxSpeed` `Max Speed` _projectilemovement)))
            (:`then_1`
              (set `ProjectileMovementComponent.ProjectileGravityScale` `Projectile Gravity Scale` _projectilemovement))
            (:`then_2`
              (`NiagaraComponent.SetAsset` (`self.VFX`) BulletVFX true))
            (:`then_3`
              (`self.SetActorEnableCollision` false))))))
    (:`then_1`
      (`self.Has Athority in Dedi`
        (:`Authority`
          _)
        (:`Remote`
          _))
      ;[0 0 0] Test VFX Setting
      (`FXSystemComponent.SetFloatParameter` (`self.VFX`) "ProjectileVelocity" _output_get)
      (`FXSystemComponent.SetFloatParameter` (`self.VFX`) "LoopDuration" _returnvalue)
      (`FXSystemComponent.SetFloatParameter` (`self.VFX`) "LifeTime" _returnvalue))))

(event `SpawnHitVFX MC`
  (params (Hit :type "HitResult Structure (by ref)"))
  (bind (_bblockinghit _binitialoverlap _time _distance _location _impactpoint _normal _impactnormal) (`GameplayStatics.BreakHitResult` Hit))
  (`self.Has Athority in Dedi`
    (:`Authority`
      _)
    (:`Remote`
      _))
  ;[1 1 0.467] Output Hit VFX
  (`NiagaraFunctionLibrary.SpawnSystemAtLocation` (`self.VFX_Hit`) _impactpoint (`KismetMathLibrary.Conv_VectorToRotator` _impactnormal)))

(fn `DEBUG_DrawTrajectory`
  (params (DrawLines :type Boolean) (`DrawLines by Time` :type Boolean) (LineDuration :type "Float (double-precision)") (LineThickness :type "Float (double-precision)") (LineColor :type "LinearColor Structure") (LineDrawingInterval :type "Float (double-precision)") (DrawPoints :type Boolean) (`DrawPoints by Time` :type Boolean) (PointSize :type "Float (double-precision)") (PointDuration :type "Float (double-precision)") (PointColor :type "LinearColor Structure") (PointDrawingInterval :type "Float (double-precision)"))
  (`|ExecutionSequence`
    (:`then_0`
      (if (`local.DrawLines`)
        (if (>= (`self.DEBUG_CurLineDrawingInterval`) (`local.LineDrawingInterval`))
          (set `self.DEBUG_CurLineDrawingInterval` 0.0)
          (`KismetSystemLibrary.DrawDebugLine` (`self.DEBUG_LineStart`) (`self.K2_GetActorLocation`) (`local.LineColor`) (`/Game/Macros/GlobalMacros.ReplaceValue` (`local.LineDuration`) 0.0 30.0) (`local.LineThickness`))
          (set `self.DEBUG_LineStart` (`self.K2_GetActorLocation`))
          (else
            (set `self.DEBUG_CurLineDrawingInterval` (+ (`self.DEBUG_CurLineDrawingInterval`) (select `bool` (`local.DrawLines by Time`) :`false` (`KismetMathLibrary.Vector_Distance` (`self.K2_GetActorLocation`) (`self.DEBUG_LineStart`)) :`true` (`GameplayStatics.GetWorldDeltaSeconds`))))))))
    (:`then_1`
      (if (`local.DrawPoints`)
        (if (>= (`self.DEBUG_CurPointDrawingInterval`) (`local.PointDrawingInterval`))
          (set `self.DEBUG_CurPointDrawingInterval` 0.0)
          (set `self.DEBUG_PrevPointLocation` (`self.K2_GetActorLocation`))
          (`KismetSystemLibrary.DrawDebugPoint` (`self.K2_GetActorLocation`) (`local.PointSize`) (`local.PointColor`) (`/Game/Macros/GlobalMacros.ReplaceValue` (`local.PointDuration`) 0.0 30.0))
          (else
            (set `self.DEBUG_CurPointDrawingInterval` (+ (`self.DEBUG_CurPointDrawingInterval`) (select `bool` (`local.DrawPoints by Time`) :`false` (`KismetMathLibrary.Vector_Distance` (`self.K2_GetActorLocation`) (`self.DEBUG_PrevPointLocation`)) :`true` (`GameplayStatics.GetWorldDeltaSeconds`))))))))))

(fn `DEBUG_Initialize`
  (bind _returnvalue (`self.K2_GetActorLocation`))
  (set `self.DEBUG_LineStart` _returnvalue)
  (set `self.DEBUG_PrevPointLocation` _returnvalue))

(fn `Fly`
  (locals (Distance :type "Float (double-precision)" :default 0.0))
  (`self.Has Athority in Dedi`
    (:`Authority in Dedi`
      _)
    (:`Authority`
      _))
  (`|ExecutionSequence`
    (:`then_0`
      (if (`self.isShot`)
        ;[1 1 0.467] Set Distance from Initial Location
        (set `local.Distance` (`KismetMathLibrary.Vector_Distance` (`self.K2_GetActorLocation`) (`self.InitialLocation`)))
        (`|ExecutionSequence`
          (:`then_0`
            ;[1 1 0.467] Enable Collision
            (`/Engine/EditorBlueprintResources/StandardMacros.Gate` false :!label _label
              (:`Exit`
                (if (>= (`local.Distance`) (`self.CollisionStartDist`))
                  (`self.SetCollision` true)
                  (goto _label :!via `Close`)))))
          (:`then_1`
            ;[0.7274 0.9968 1] Destroy
            ;;[1 1 0.467] Max Range Check
            (if (> (`local.Distance`) (`self.RangeMax`))
              (`self.K2_DestroyActor`))))))
    (:`then_1`
      ;[1 1 0.467] Component Fly, 필요  부에서 IsShot 체크
      (for _array_element (`self.SpecialAbilities`)
        (`/Engine/EditorBlueprintResources/StandardMacros.IsValid` _array_element
          (:`Is Valid`
            (`/Game/Assets/Components/BulletAbility/BPC_BL_SpecialAbilityBase.Fly` _array_element)))))))

(fn `Hit`
  (params (HitComponent :type "PrimitiveComponent Object Reference") (OtherActor :type "Actor Object Reference") (OtherComp :type "PrimitiveComponent Object Reference") (NormalImpulse :type "Vector Structure") (Hit :type "HitResult Structure"))
  (locals (OtherActorIsDerived :type Boolean))
  (`|ExecutionSequence`
    (:`then_0`
      (`self.SpawnHitVFX MC` (`local.Hit`)))
    (:`then_1`
      ;[1 0 0] Other Actor와 Shooter가 같은가
      ; True: 무시
      ; False: 인터페이스 확인
      (if (not (== (`local.OtherActor`) (`self.Shooter`)))
        ;[1 1 0.467] BulletDamageble 인터페이스 여부 확인
        ; True: 제외클래스 확인
        ; False: Bullet Destroy
        (if (`KismetSystemLibrary.DoesImplementInterface` (`local.OtherActor`) "/Game/Interfaces/BPI_BulletDamageble.BPI_BulletDamageble_C")
          (bind _forcetype (message `/Game/Interfaces/BPI_Force.Get Force` (`local.OtherActor`)))
          ;[1 1 0.467] 제외 클래스 여부 확인
          ; True: Bullet Destroy
          ; False: 제외 클래스 상속 확인
          (if (not (`KismetArrayLibrary.Array_Contains` (`self.ExceptForces`) _forcetype))
            ;[0.7274 0.9968 1] Take Damage
            (message `/Game/Interfaces/BPI_BulletDamageble.TakeBulletDamage` (`local.OtherActor`) (`self.Damage`) (`local.Hit`) (`self.Shooter`) (`self.VFX_Hit`))
            ;[0.7274 0.9968 1] Special Ability Hit Setting
            (bind (_arrayindex _arrayelement) (`/Engine/EditorBlueprintResources/StandardMacros.ReverseForEachLoop` (`self.SpecialAbilities`))
              (:`LoopBody`
                (`/Engine/EditorBlueprintResources/StandardMacros.IsValid` _arrayelement
                  (:`Is Valid`
                    (`/Game/Assets/Components/BulletAbility/BPC_BL_SpecialAbilityBase.Hit` _arrayelement (`local.HitComponent`) (`local.OtherActor`) (`local.OtherComp`) (`local.NormalImpulse`) (`local.Hit`)))))
              (:`Completed`
                ;[0.2316 1 0] Destroy
                (`self.K2_DestroyActor` :!label _label)))
            (else
              (goto _label)))
          (else
            (goto _label)))))))

(fn `Hit with Check`
  (params (Hit :type "HitResult Structure") (Damage :type "Float (double-precision)"))
  (returns (Damaged :type Boolean))
  (locals (OtherActorIsDerived :type Boolean))
  ;[1 1 0.467] Other Actor와 Shooter가 같은가
  ; True: 무시
  ; False: 인터페이스 확인
  (if (not (== (`self.Shooter`) (`.HitActor` (`GameplayStatics.BreakHitResult` (`local.Hit`)))))
    ;[1 1 0.467] BulletDamageble 인터페이스 여부 확인
    ; True: 제외클래스 확인
    ; False: Bullet Destroy
    (if (`KismetSystemLibrary.DoesImplementInterface` (`.HitActor` (`GameplayStatics.BreakHitResult` (`local.Hit`))) "/Game/Interfaces/BPI_BulletDamageble.BPI_BulletDamageble_C")
      ;[1 1 0.467] 제외 클래스 여부 확인
      ; True: Bullet Destroy
      ; False: 제외 클래스 상속 확인
      (bind _forcetype (message `/Game/Interfaces/BPI_Force.Get Force` (`.HitActor` (`GameplayStatics.BreakHitResult` (`local.Hit`)))))
      (if (not (`KismetArrayLibrary.Array_Contains` (`self.ExceptForces`) _forcetype))
        ;[0.7274 0.9968 1] Take Damage
        (message `/Game/Interfaces/BPI_BulletDamageble.TakeBulletDamage` (`.HitActor` (`GameplayStatics.BreakHitResult` (`local.Hit`))) (`local.Damage`) (`local.Hit`) null (`self.VFX_Hit`))
        (return true)
        (else
          _)))
    ;[0.2316 1 0] Destroy
    (return false)))

(fn `Initialize`
  (params (Shooter :type "Actor Object Reference") (CollisionStartDist :type "Float (double-precision)") (`Init Data` :type "/Game/Structs/S_BL_Data Structure") (ShotDirection :type "Vector Structure") (InstantlyShoot :type Boolean :default true))
  (bind (_damage _rangemax _speed _gravityscale) (break `/Game/Structs/S_BL_Base` `Init Data_BaseAbility_8_9AC7F1424787AED21383DDB4C16A02F5`))
  (bind _vfx (`self.VFX`))
  (bind _projectilemovement (`self.ProjectileMovement`))
  (bind _projectilemovement_2 (`self.ProjectileMovement`))
  (bind _projectilemovement_3 (`self.ProjectileMovement`))
  (bind (_mesh _vfx_2) (break `/Game/Structs/S_BL_Data` (`local.Init Data`)))
  (bind (_mesh_2 _vfx_3 _sfx _baseability _specialabilitycomponents _specialability) (break `/Game/Structs/S_BL_Data` (`local.Init Data`)))
  (`|ExecutionSequence`
    (:`then_0`
      ;[0.7274 0.9968 1] Set Static Mesh
      (`StaticMeshComponent.SetStaticMesh` (`self.Mesh`) `Init Data_Mesh_2_A6E108124127F330D81A55A805F4BCA2`))
    (:`then_1`
      ;[0.7274 0.9968 1] Set Common VFXs
      (`|ExecutionSequence`
        (:`then_0`
          (`self.Has Athority in Dedi`
            (:`Authority in Dedi`
              _)
            (:`Authority`
              _))
          (`NiagaraComponent.SetAsset` _vfx (`BlueprintMapLibrary.Map_Find` _vfx_2 "NewEnumerator0") true)
          (`self.Has Athority in Dedi`
            (:`Authority`
              (`SceneComponent.K2_DetachFromComponent` _vfx "KeepWorld" "KeepWorld" "KeepWorld" true))))
        (:`then_1`
          (set `self.VFX_MuzzleFlash` (`BlueprintMapLibrary.Map_Find` _vfx_2 "NewEnumerator1")))
        (:`then_2`
          (set `self.VFX_Hit` (`BlueprintMapLibrary.Map_Find` _vfx_2 "NewEnumerator2")))))
    (:`then_2`
      (`self.Has Athority in Dedi`
        (:`Authority in Dedi`
          _)
        (:`Authority`
          _))
      ;[0.7274 0.9968 1] Set Base Data
      (`|ExecutionSequence`
        (:`then_0`
          (set `self.Damage` _damage))
        (:`then_1`
          (set `self.RangeMax` _rangemax))
        (:`then_2`
          (bind _output_get (set `self.Speed` _speed))
          (set `ProjectileMovementComponent.MaxSpeed` _output_get _projectilemovement_3))
        (:`then_3`
          (bind _output_get_2 (set `self.GravityScale` _gravityscale))
          (set `ProjectileMovementComponent.ProjectileGravityScale` _output_get_2 _projectilemovement_3))))
    (:`then_3`
      ;[0.7274 0.9968 1] Init Ability Components
      (for _array_element _specialabilitycomponents
        (if (`KismetSystemLibrary.IsValidClass` _array_element)
          (bind _returnvalue (`self.InitializeAbility` _array_element _specialability _vfx_3))
          (bind _type (`/Game/Assets/Components/BulletAbility/BPC_BL_SpecialAbilityBase.GetType` _returnvalue))
          (bind _casted_ability (`/Game/Macros/GlobalMacros.CastBLS` _type _returnvalue)
            (:`None`
              (`KismetArrayLibrary.Array_Add` (`self.SpecialAbilities`) _casted_ability))))))
    (:`then_4`
      ;[0.7274 0.9968 1] Set Except Targets
      (set `self.ExceptForces` `Init Data_ExceptTargets_35_F944DB67486861D158FED7B037C95F52`)
      ;[0.7274 0.9968 1] Set Shooter
      (set `self.Shooter` (`local.Shooter`))
      ;[0.7274 0.9968 1] Set Collision Starting Distance
      (set `self.CollisionStartDist` (`local.CollisionStartDist`))
      (`self.SetCollision` false))
    (:`then_5`
      (`self.Initialize MC` (`MovementComponent.GetMaxSpeed` _projectilemovement_2) (`ProjectileMovementComponent.ProjectileGravityScale` _projectilemovement_2) (`NiagaraComponent.GetAsset` (`self.VFX`))))
    (:`then_6`
      ;[0.7274 0.9968 1] Set Shot Direction and Shoot
      (set `self.ShotDirection` ShotDirection)
      (if (`local.InstantlyShoot`)
        (set `ProjectileMovementComponent.InitialSpeed` (`MovementComponent.GetMaxSpeed` _projectilemovement) _projectilemovement)
        (`self.Shoot`)))))

(fn `InitializeAbility`
  (params (SpecialAbilityComponentClass :type "/Game/Assets/Components/BulletAbility/BPC_BL_SpecialAbilityBase Class Reference") (AbilityFigures :type "Map of /Game/EnumClasses/E_BLS_AbilityFigure Enum to Float (double-precision)") (VFX :type "Map of /Game/EnumClasses/E_BL_VFX Enum to NiagaraSystem Object Reference"))
  (returns (ReturnValue :type "/Game/Assets/Components/BulletAbility/BPC_BL_SpecialAbilityBase Object Reference"))
  (locals (BLSComponent :type "/Game/Assets/Components/BulletAbility/BPC_BL_SpecialAbilityBase Object Reference"))
  (bind _abilityfigures (`local.AbilityFigures`))
  (bind _returnvalue (`|AddComponentByClass` SpecialAbilityComponentClass self))
  (bind _output_get (set `local.BLSComponent` _returnvalue))
  (bind _type (`/Game/Assets/Components/BulletAbility/BPC_BL_SpecialAbilityBase.GetType` _output_get))
  (switch `/Game/EnumClasses/E_BLS_Component` _type
    (:`NewEnumerator4`
      ;[1 1 0.467] Return NULL
      (return null))
    (:`NewEnumerator0`
      ;[1 1 0.467] Explosive Ability
      (bind _asbpc_bls_explosive (cast `/Game/Assets/Components/BulletAbility/BPC_BLS_Explosive` (`local.BLSComponent`)))
      (`/Game/Assets/Components/BulletAbility/BPC_BLS_Explosive.Initialize` _asbpc_bls_explosive (`self.Damage`) (`BlueprintMapLibrary.Map_Find` _abilityfigures "NewEnumerator0") (`BlueprintMapLibrary.Map_Find` _abilityfigures "NewEnumerator1") (`BlueprintMapLibrary.Map_Find` _abilityfigures "NewEnumerator3") (`BlueprintMapLibrary.Map_Find` (`local.VFX`) "NewEnumerator3"))
      (return _asbpc_bls_explosive))))

(fn `SetCollision`
  (params (On :type Boolean))
  (if On
    (`PrimitiveComponent.SetCollisionProfileName` (`self.HitCollision`) "Bullet" true)
    (else
      (`PrimitiveComponent.SetCollisionResponseToAllChannels` (`self.HitCollision`) "ECR_Ignore"))))

(fn `Shoot`
  (`self.Has Athority in Dedi`
    (:`Authority in Dedi`
      _)
    (:`Authority`
      _))
  ;[0.7274 0.9968 1] Set Initial Location
  (set `self.InitialLocation` (`self.K2_GetActorLocation`))
  ;[0.7274 0.9968 1] Set Velocity
  (bind _output_get (set `MovementComponent.Velocity` (* (`self.ShotDirection`) (`ProjectileMovementComponent.InitialSpeed` (`self.ProjectileMovement`))) (`self.ProjectileMovement`)))
  (`self.Shoot MC` _output_get)
  ;[1 1 1] Components
  (for _array_element (`self.SpecialAbilities`)
    (`/Engine/EditorBlueprintResources/StandardMacros.IsValid` _array_element
      (:`Is Valid`
        (`/Game/Assets/Components/BulletAbility/BPC_BL_SpecialAbilityBase.Shoot` _array_element))))
  (set `self.isShot` true))

(fn `UserConstructionScript`)