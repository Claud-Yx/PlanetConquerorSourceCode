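; Base Blueprint for extractor buildings that periodically add a set resource to the in-game GameState.
; On BeginPlay, unless it is a ghost, it looks up its expendable type in DT_Expendable to set the notice panel's image and amount.
; It then starts a looping timer at the extract period that increases the base resource and triggers the floating notice, whose float time is also derived from that period.
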(event `self.ReceiveBeginPlay`
  (`parent.ReceiveBeginPlay`)
  (if (not (`self.IsGhost`))
    (bind _asbp_gs_in_game (cast `/Game/GameMode/BP_GS_InGame` (`GameplayStatics.GetGameState`)))
    (set `self.GameState` _asbp_gs_in_game)
    (`|ExecutionSequence`
      (:`then_0`
        ;[1 1 1] Panel 이미지, 증가량 설정
        (bind _outrownames (`DataTableFunctionLibrary.GetDataTableRowNames` "/Game/DataTables/DT_Expendable.DT_Expendable"))
        (for _array_element _outrownames
          (bind _returnvalue (`|GetDataTableRow` "/Game/DataTables/DT_Expendable.DT_Expendable" _array_element)
            (:`then`
              (bind (_expendable _image) (break `/Game/Structs/S_Expendable` _returnvalue))
              (if (`|EnumEquality` (`self.ExpendableType`) _expendable)
                (`/Game/Assets/Components/FloatingPanel/BPC_FloatingPanel.SetPanel` (`self.BPC_IncreasingResourceNotice`) _image (`self.ExpendableAmount`))
                (`KismetSystemLibrary.K2_SetTimer` null "IncreaseResource" (`self.ExtractPeriod`) true)
                (break))))))
      (:`then_1`
        (`/Game/Assets/Components/FloatingPanel/BPC_FloatingPanel.SetPanelFloatingTimeByDefault` (`self.BPC_IncreasingResourceNotice`) (`self.ExtractPeriod`))))))

(fn `IncreaseResource`
  (`/Game/GameMode/BP_GS_InGame.IncreaseBaseResource` (`self.GameState`) (`self.ExpendableType`) (`self.ExpendableAmount`))
  (`/Game/Assets/Components/FloatingPanel/BPC_FloatingPanel.StartFloating` (`self.BPC_IncreasingResourceNotice`)))

(fn `UserConstructionScript`
  (`parent.UserConstructionScript`))