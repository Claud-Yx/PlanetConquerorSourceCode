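; BP_BuildingGhost is the building preview actor, showing a given mesh with a colored blueprint-style outline.
; Initialize and ChangeMeshes route through server events to a multicast that sets the same mesh on the StaticMesh and OutLine components.
; SetOutlineColor follows the same server-to-multicast route, applying a green, red or orange material to every OutLine material slot, skipped on dedicated servers.
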(event `Initizlize OS`
  (params (Mesh :type "StaticMesh Object Reference"))
  (`self.ChangeMeshes` Mesh))

(event `SetOutlineColor MC`
  (params (OutlineColor :type "/Game/EnumClasses/E_BuildingOutlineColor Enum" :default "NewEnumerator0"))
  (bind _outline (`self.OutLine`))
  (bind _returnvalue (- (`KismetArrayLibrary.Array_Length` (`MeshComponent.GetMaterials` _outline)) 1))
  (`self.Has Athority in Dedi`
    (:`Authority`
      _)
    (:`Remote`
      _))
  (bind _output_get (set `self.OutlineColor` OutlineColor))
  (switch `/Game/EnumClasses/E_BuildingOutlineColor` _output_get
    (:`NewEnumerator0`
      (`self.SetOutlineColorLoop` _returnvalue _outline "/Game/Assets/Building/CommonMaterials/M_Blueprint_Green.M_Blueprint_Green"))
    (:`NewEnumerator1`
      (`self.SetOutlineColorLoop` _returnvalue _outline "/Game/Assets/Building/CommonMaterials/M_Blueprint_Red.M_Blueprint_Red"))
    (:`NewEnumerator2`
      (`self.SetOutlineColorLoop` _returnvalue _outline "/Game/Assets/Building/CommonMaterials/M_Blueprint_Orange.M_Blueprint_Orange"))))

(event `SetOutlineColor OS`
  (params (OutlineColor :type "/Game/EnumClasses/E_BuildingOutlineColor Enum" :default "NewEnumerator0"))
  (`self.SetOutlineColor MC` OutlineColor))

(event `ChangeMeshes OS`
  (params (Mesh :type "StaticMesh Object Reference"))
  (`self.ChangeMeshes MC` Mesh))

(event `ChangeMeshes MC`
  (params (Mesh :type "StaticMesh Object Reference"))
  (`StaticMeshComponent.SetStaticMesh` (`self.StaticMesh`) Mesh)
  (`StaticMeshComponent.SetStaticMesh` (`self.OutLine`) Mesh))

(fn `ChangeMeshes`
  (params (Mesh :type "StaticMesh Object Reference"))
  (`self.ChangeMeshes OS` Mesh))

(fn `Initialize`
  (params (Mesh :type "StaticMesh Object Reference"))
  (`self.Initizlize OS` Mesh))

(fn `SetOutlineColor`
  (params (OutlineColor :type "/Game/EnumClasses/E_BuildingOutlineColor Enum" :default "NewEnumerator0"))
  (`self.SetOutlineColor OS` OutlineColor))

(fn `SetOutlineColorLoop`
  (params (LastIndex :type Integer) (OutlineMesh :type "PrimitiveComponent Object Reference") (Material :type "MaterialInterface Object Reference"))
  (for _index (range (+ LastIndex 1))
    (`PrimitiveComponent.SetMaterial` OutlineMesh _index Material))
  (return))

(fn `UserConstructionScript`)