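; Base turret building Blueprint that supplies shared setup, aiming and firing functions for turrets.
; Init applies turret data, looked up from DT_Turret by GetTurretData, to muzzles, the detection Sensor's range, pitch limits and turn speed.
; RotateBody interpolates yaw and RotateGun pitch, while Shoot delegates to a muzzle.
; Ghost copies never fire; on Tick they mirror OriginalBuilding's component transforms by matching names instead of running parent Tick.
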(event `self.ReceiveBeginPlay`
  (`KismetArrayLibrary.Array_Add` (`self.NoBoundComponents`) (`self.Sensor`))
  (`parent.ReceiveBeginPlay`))

(event `self.ReceiveTick`
  (params (DeltaSeconds :type "Float (single-precision)"))
  (if (`self.IsGhost`)
    (for _array_element (`SceneComponent.GetChildrenComponents` (`/Game/Assets/Building/BaseBlueprints/BP_BuildingBase.DefaultSceneRoot` (`self.OriginalBuilding`)) true)
      (bind _asprimitive_component (cast `PrimitiveComponent` _array_element))
      (`/Engine/EditorBlueprintResources/StandardMacros.IsValid` _asprimitive_component
        (:`Is Valid`
          (for _array_element_2 (`SceneComponent.GetChildrenComponents` (`self.DefaultSceneRoot`) true)
            (if (`KismetStringLibrary.EqualEqual_StrStr` (`self.GetComponentName` (`KismetSystemLibrary.GetDisplayName` _array_element_2)) (`self.GetComponentName` (`KismetSystemLibrary.GetDisplayName` _asprimitive_component)))
              (`SceneComponent.K2_SetWorldTransform` _array_element_2 (`SceneComponent.K2_GetComponentToWorld` _asprimitive_component) false true)
              (`SceneComponent.K2_SetRelativeTransform` _array_element_2 (`SceneComponent.GetRelativeTransform` _asprimitive_component) false true))))))
    (else
      (`parent.ReceiveTick` DeltaSeconds))))

(fn `Get Turret Data`
  (params (TurretName :type Name))
  (returns (TurretData :type "/Game/Structs/S_TurretData Structure") (Found :type Boolean) (RowName :type Name))
  (bind _returnvalue (`|GetDataTableRow` "/Game/DataTables/DT_Turret.DT_Turret" TurretName)
    (:`then`
      (return _returnvalue true TurretName))
    (:`RowNotFound`
      (return (struct) false TurretName))))

(fn `Init`
  (params (TurretData :type "/Game/Structs/S_TurretData Structure"))
  (bind (_muzzledatas _mindetectdist _maxdetectdist _minheightangle _maxheightangle _rotatelerpspeed) (break `/Game/Structs/S_TurretData` TurretData))
  (bind _sensor (`self.Sensor`))
  (`self.Has Authority in Dedi`
    (:`Authority in Dedi`
      _)
    (:`Authority`
      _)
    (:`Remote`
      _))
  (`|ExecutionSequence`
    (:`then_0`
      (set `self.Muzzles` _muzzledatas))
    (:`then_1`
      (bind _output_get (set `self.MinDetectDist` _mindetectdist))
      (set `/Game/Assets/Components/ActorSensor/BPC_ActorSensor.MinDist` _output_get _sensor))
    (:`then_2`
      (bind _output_get_2 (set `self.MaxDetectDist` _maxdetectdist))
      (`SphereComponent.SetSphereRadius` _sensor _output_get_2 true))
    (:`then_3`
      (set `self.MinHeightAngle` _minheightangle))
    (:`then_4`
      (set `self.MaxHeightAngle` _maxheightangle))
    (:`then_5`
      (set `self.RotateInterpSpeed` _rotatelerpspeed))
    (:`then_6`
      (set `/Game/Assets/Components/ActorSensor/BPC_ActorSensor.Owner` self (`self.Sensor`)))))

(fn `RotateBody`
  (params (Body :type "SceneComponent Object Reference") (RotationToTarget :type "Rotator Structure"))
  (bind (_returnvalue_roll _returnvalue_pitch _returnvalue_yaw) (`KismetMathLibrary.BreakRotator` (`KismetMathLibrary.RInterpTo` (`SceneComponent.K2_GetComponentRotation` Body) RotationToTarget (`GameplayStatics.GetWorldDeltaSeconds`) (`self.RotateInterpSpeed`))))
  (`SceneComponent.K2_SetWorldRotation` Body (`KismetMathLibrary.MakeRotator` 0.0 0.0 _returnvalue_yaw) false false))

(fn `RotateGun`
  (params (Gun :type "SceneComponent Object Reference") (RotationToTarget :type "Rotator Structure"))
  (bind (_returnvalue_roll _returnvalue_pitch) (`KismetMathLibrary.BreakRotator` (`KismetMathLibrary.RInterpTo` (`SceneComponent.K2_GetComponentRotation` Gun) RotationToTarget (`GameplayStatics.GetWorldDeltaSeconds`) (`self.RotateInterpSpeed`))))
  (`SceneComponent.K2_SetRelativeRotation` Gun (`KismetMathLibrary.MakeRotator` 0.0 _returnvalue_pitch) false false))

(fn `Shoot`
  (params (Muzzle :type "/Game/Assets/Components/Muzzle/BPC_Muzzle Object Reference") (AimObject :type "SceneComponent Object Reference"))
  (if (not (`self.IsGhost`))
    (`/Game/Assets/Components/Muzzle/BPC_Muzzle.Shoot` Muzzle AimObject (0.0 0.0 0.0) 0.0)))

(fn `UserConstructionScript`
  (`parent.UserConstructionScript`))