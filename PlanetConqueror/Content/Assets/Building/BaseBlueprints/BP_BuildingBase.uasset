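; Base actor for placeable buildings, handling damage, destruction and a colored ghost preview mode.
; Initialize randomizes skeletal animation phase, sets up the HP bar from bounds and pulls name, widget and other data from DT_Ghost by class.
; Damage briefly shows the HP bar; depletion multicasts timer-driven explosions, skipped on dedicated servers, and a Chaos destruct message, then destroys the actor after a delay.
; It also plays environmental sound and provides a Chaos field-spawning helper.
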(event `self.ReceiveBeginPlay`
  (bind (_environmentalsound_itemappearancedata _environmentalsound_volume _environmentalsound_starttime _environmentalsound_attenuation) (break `/Game/Structs/S_AudioProperty` (`self.EnvironmentalSound`)))
  (`self.Initialize`)
  (`/Engine/EditorBlueprintResources/StandardMacros.IsValid` _environmentalsound_itemappearancedata
    (:`Is Valid`
      (`KismetSystemLibrary.PrintText` (`KismetTextLibrary.Conv_StringToText` (`KismetSystemLibrary.GetDisplayName` _environmentalsound_itemappearancedata)))
      (`GameplayStatics.SpawnSoundAttached` _environmentalsound_itemappearancedata (`self.DefaultSceneRoot`) "None" (0.0 0.0 0.0) (struct) "KeepRelativeOffset" true _environmentalsound_volume 1.0 _environmentalsound_starttime _environmentalsound_attenuation null))))

(event `self.TakeBulletDamage`
  (params (Damage :type "Float (double-precision)") (Hit :type "HitResult Structure") (Shooter :type "Actor Object Reference") (HitVFX :type "NiagaraSystem Object Reference"))
  (bind (_origin _boxextent) (`self.GetActorBounds` true true))
  (bind _hpbar (`self.HPBar`))
  (bind _empty (`/Game/Assets/Components/BlockProgressBarComponent/BPC_BlockProgressBar.IncreaseValue` (`self.HPBar`) (* Damage -1.0) false))
  (`|ExecutionSequence`
    (:`then_0`
      (`/Game/Assets/Components/BlockProgressBarComponent/BPC_BlockProgressBar.ShowBPBar` (`self.HPBar`) true 0.2)
      (`KismetSystemLibrary.K2_ClearAndInvalidateTimerHandle` (`self.Fade Out Timer`)))
    (:`then_1`
      (if _empty
        (`/Engine/EditorBlueprintResources/StandardMacros.DoOnce` false
          (:`Completed`
            (`|ExecutionSequence`
              (:`then_0`
                ;[1 1 1] Destroy VFX에 필요한 변수 설정
                (`self.UnableComponentsCollision`)
                (set `self.BoundOrigin` _origin)
                (set `self.BoundRadious` (`KismetMathLibrary.FMax` (.x _boxextent) (.y _boxextent) (.z _boxextent))))
              (:`then_1`
                ;[1 1 1] HPBar 없애기
                (`SceneComponent.SetVisibility` (`self.HPBar`) true true)
                (`/Game/Assets/Components/BlockProgressBarComponent/BPC_BlockProgressBar.HideBPBar` (`self.HPBar`) true true 1.5)
                ;[1 1 1] 충돌 끄기
                (`self.SetActorEnableCollision` false))
              (:`then_2`
                (set `self.IsDestroyed` true)
                (set `/Game/Assets/Components/BlockProgressBarComponent/BPC_BlockProgressBar.BPBarLerpSpeed` 0.25 (`self.HPBar`))
                (`self.SpawnDestroyVFX MC`)
                (`KismetSystemLibrary.Delay` 4.0)
                (`self.DestroyActor OS`)))))
        (else
          ;[1 1 1] 건물이 무너지지 않았을 때
          (set `/Game/Assets/Components/BlockProgressBarComponent/BPC_BlockProgressBar.TimerFadeOutTime` 0.2 _hpbar)
          (bind _returnvalue (`KismetSystemLibrary.K2_SetTimer` _hpbar "TimerHideBPBar" 2.0))
          (set `self.Fade Out Timer` _returnvalue))))))

(event `/Game/Interfaces/BPI_SwingDamageble.TakeSwingDamage`
  (params (Damage :type "Float (double-precision)") (Hit :type "HitResult Structure") (Swinger :type "Actor Object Reference") (HitVFX :type "NiagaraSystem Object Reference"))
  (`self.TakeBulletDamage` Damage Hit Swinger HitVFX))

(event `/Game/Interfaces/BPI_ChaosDestructable.SpawnChaosDestruct`
  (params (Part :type Name))
  (`self.SetActorEnableCollision` false)
  (`SceneComponent.SetVisibility` (`self.DefaultSceneRoot`) false true))

(event `DestroyActor OS`
  (`self.K2_DestroyActor`))

(event `SpawnDestroyVFX MC`
  (`self.Has Athority in Dedi`
    (:`Authority`
      _)
    (:`Remote`
      _))
  ;[1 0 0] 이후 건물마다 달리 한다면 수정 필요
  (`self.SpawnDestroySubVFXTimer`)
  (bind _returnvalue (`KismetSystemLibrary.K2_SetTimer` null "SpawnDestroySubVFXTimer" 0.1 true))
  (set `self.DestroyVFXTimer` _returnvalue)
  (`KismetSystemLibrary.K2_SetTimer` null "SpawnDestroyVFXTimer" 0.4))

(fn `Get Force`
  (returns (ForceType :type "/Game/EnumClasses/E_ForceType Enum"))
  (return "NewEnumerator8"))

(fn `Initialize`
  (locals (CollisionEnableTmp :type "Array of ECollisionEnabled Enum"))
  (bind (_origin _boxextent) (`self.GetActorBounds` true))
  (bind (_origin_2 _boxextent_2) (`self.GetActorBounds` true))
  (bind _hpbar (`self.HPBar`))
  (bind _hpbar_2 (`self.HPBar`))
  ;[1 0.3142 0.3142] 프레임 드랍 해결하기
  (`|ExecutionSequence`
    (:`then_0`
      ;;[1 1 1] Noise 적용
      (if (not (`self.IsGhost`))
        ;;;[1 1 1] Noise값 설정(랜덤)
        (set `self.Noise` (`KismetMathLibrary.RandomFloatInRange` 0.0 1.0))
        ;;;[1 1 1] Animation에 Noise값 적용
        (for _array_element (`SceneComponent.GetChildrenComponents` (`self.DefaultSceneRoot`) true)
          (bind _asskeletal_mesh_component (cast `SkeletalMeshComponent` _array_element))
          (`SkeletalMeshComponent.SetPosition` _asskeletal_mesh_component (* (`AnimationAsset.GetPlayLength` (`.AnimToPlay` (break `SingleAnimationPlayData` (`SkeletalMeshComponent.AnimationData` _asskeletal_mesh_component)))) (`self.Noise`)) true))))
    (:`then_1`
      ;;[1 1 1] HPBar 설정
      (for _array_element_2 (`self.NoBoundComponents`)
        (`KismetArrayLibrary.Array_Add` (`local.CollisionEnableTmp`) (`PrimitiveComponent.GetCollisionEnabled` _array_element_2))
        (`PrimitiveComponent.SetCollisionEnabled` _array_element_2 "NoCollision"))
      (`SceneComponent.K2_SetRelativeLocation` (`self.HPBar`) (`KismetMathLibrary.MakeVector` 0.0 0.0 (+ (.z _boxextent_2) (.z _boxextent_2) 50.0)) false true)
      (for (_array_element_3 _array_index) (`self.NoBoundComponents`)
        (`PrimitiveComponent.SetCollisionEnabled` _array_element_3 (`|GetArrayItem` (`local.CollisionEnableTmp`) _array_index)))
      (`/Game/Assets/Components/BlockProgressBarComponent/BPC_BlockProgressBar.Reinit BPBar` (`self.HPBar`) (make `/Game/Structs/S_BlockProgressBarData` "/Game/Assets/Building/CommonMaterials/M_BD_BlockOn.M_BD_BlockOn" "/Game/Assets/Building/CommonMaterials/M_BD_BlockOff.M_BD_BlockOff" (`KismetMathLibrary.FCeil` (/ (`self.HP Max`) 5.0))))
      (if (`self.IsGhost`)
        (`self.SetActorEnableCollision` false)
        (`self.SetGhostColor`)
        (`ActorComponent.K2_DestroyComponent` _hpbar_2)
        (`ActorComponent.K2_DestroyComponent` (`self.BPC_IncreasingResourceNotice`))
        (else
          (bind _output_get (set `/Game/Assets/Components/BlockProgressBarComponent/BPC_BlockProgressBar.MaxValue` (`self.HP Max`) _hpbar))
          (`/Game/Assets/Components/BlockProgressBarComponent/BPC_BlockProgressBar.SetValue` _hpbar _output_get true)
          (`/Game/Assets/Components/BlockProgressBarComponent/BPC_BlockProgressBar.HideBPBar` _hpbar_2 false false 0.0))))
    (:`then_2`
      (if (not (`self.IsGhost`))
        (set `/Game/Assets/Components/FloatingPanel/BPC_FloatingPanel.InitLocation` (`KismetMathLibrary.MakeVector` 0.0 0.0 (+ (.z _boxextent) (.z _boxextent) 0.0)) (`self.BPC_IncreasingResourceNotice`))))
    (:`then_3`
      (if (`KismetMathLibrary.BooleanNAND` (`self.IsGhost`) (`self.IsSpawned`))
        (bind _outrownames (`DataTableFunctionLibrary.GetDataTableRowNames` "/Game/DataTables/DT_Ghost.DT_Ghost"))
        (for _array_element_4 _outrownames
          (bind _returnvalue (`|GetDataTableRow` "/Game/DataTables/DT_Ghost.DT_Ghost" _array_element_4)
            (:`then`
              (bind (_mesh _actor _cost _buildingname _interactiontext _interactionwidget _environmentalsound) (break `/Game/Structs/S_BD_GhostData` _returnvalue))
              (if (== _actor (`GameplayStatics.GetObjectClass` self))
                (set `self.BuildingName` _buildingname)
                (set `self.InteractionWidget` _interactionwidget)
                (cast `/Game/GameMode/BP_GS_InGame` (`GameplayStatics.GetGameState`))
                (set `self.ExpendableCosts` _cost)
                (set `self.EnvironmentalSound` _environmentalsound)
                (break)))))
        (else
          (bind _outrownames_2 (`DataTableFunctionLibrary.GetDataTableRowNames` "/Game/DataTables/DT_Ghost.DT_Ghost"))
          (for _array_element_5 _outrownames_2
            (bind _returnvalue_2 (`|GetDataTableRow` "/Game/DataTables/DT_Ghost.DT_Ghost" _array_element_5)
              (:`then`
                (bind (_mesh_2 _actor_2 _cost_2 _buildingname_2 _interactiontext_2 _interactionwidget_2) (break `/Game/Structs/S_BD_GhostData` _returnvalue_2))
                (if (== _actor_2 (`GameplayStatics.GetObjectClass` self))
                  (set `self.BuildingName` _buildingname_2)
                  (set `self.InteractionWidget` _interactionwidget_2)
                  (break))))))))
    (:`then_4`
      (if (and (not (`self.UseFloatingBar`)) (not (`self.IsGhost`)))
        (`ActorComponent.K2_DestroyComponent` (`self.BPC_IncreasingResourceNotice`))))))

(fn `PlaySoundTimer`
  (bind (_environmentalsound_itemappearancedata _environmentalsound_volume _environmentalsound_starttime _environmentalsound_attenuation) (break `/Game/Structs/S_AudioProperty` (`self.EnvironmentalSound`)))
  (bind _returnvalue (`GameplayStatics.SpawnSoundAttached` _environmentalsound_itemappearancedata (`self.DefaultSceneRoot`) "None" (0.0 0.0 0.0) (struct) "KeepRelativeOffset" true _environmentalsound_volume 1.0 _environmentalsound_starttime _environmentalsound_attenuation null))
  (set `self.EnvironmentalSoundComponent` _returnvalue))

(fn `SetGhostColor`
  (locals (`Outline Color` :type "MaterialInstance Object Reference") (OriginalComponents :type "Array of SceneComponent Object Reference") (index :type Integer))
  (set `local.OriginalComponents` (`SceneComponent.GetChildrenComponents` (`/Game/Assets/Building/BaseBlueprints/BP_BuildingBase.DefaultSceneRoot` (`self.OriginalBuilding`)) true))
  (switch `/Game/EnumClasses/E_BuildingOutlineColor` (`self.GhostColor`)
    (:`NewEnumerator0`
      (set `local.Outline Color` "/Game/Assets/Building/CommonMaterials/M_Blueprint_Green_Inst.M_Blueprint_Green_Inst"))
    (:`NewEnumerator1`
      (set `local.Outline Color` "/Game/Assets/Building/CommonMaterials/M_Blueprint_Red_Inst.M_Blueprint_Red_Inst"))
    (:`NewEnumerator2`
      (set `local.Outline Color` "/Game/Assets/Building/CommonMaterials/M_Blueprint_Orange_Inst.M_Blueprint_Orange_Inst")))
  (for (_array_element _array_index) (`SceneComponent.GetChildrenComponents` (`self.DefaultSceneRoot`) true)
    (set `local.index` _array_index)
    (bind _asmesh_component (cast `MeshComponent` _array_element))
    (for _index (range (`PrimitiveComponent.GetNumMaterials` _asmesh_component))
      (`PrimitiveComponent.SetMaterial` _asmesh_component _index (`local.Outline Color`)))
    (bind _asskeletal_mesh_component (cast `SkeletalMeshComponent` _asmesh_component))
    (bind _asskeletal_mesh_component_2 (cast `SkeletalMeshComponent` (`|GetArrayItem` (`local.OriginalComponents`) (`local.index`))))
    (`SkeletalMeshComponent.SetPosition` _asskeletal_mesh_component (`SkeletalMeshComponent.GetPosition` _asskeletal_mesh_component_2) true))
  (`self.SetActorScale3D` (1.025 1.025 1.025)))

(fn `SpawnDestroySubVFXTimer`
  (bind _returnvalue (`NiagaraFunctionLibrary.SpawnSystemAtLocation` "/Game/Assets/VFX/Gunner_Shooter_VFX/Effects/Bomb/NS_Bomb_Explosion_1.NS_Bomb_Explosion_1" (+ (`self.BoundOrigin`) (* (`KismetMathLibrary.RandomUnitVectorInConeInDegrees` (0.0 0.0 1.0) 135.0) (* (`self.BoundRadious`) (`KismetMathLibrary.RandomFloatInRange` 0.8 1.25))))))
  (`GameplayStatics.SpawnSoundAttached` "/Game/Assets/Sounds/SoundCue/SC_Explosion_1.SC_Explosion_1" _returnvalue "None" (0.0 0.0 0.0) (struct) "KeepRelativeOffset" false 0.6 3.0 0.0 "/Game/Assets/Sounds/SoundAttenuation/SA_Test.SA_Test" null)
  (`FXSystemComponent.SetFloatParameter` _returnvalue "Overall_Scale" (* (`KismetMathLibrary.RandomFloatInRange` 0.008 0.01) (`self.BoundRadious`)))
  (bind _result (`/Engine/EditorBlueprintResources/StandardMacros.IncrementInt` (`self.CurDestroyLoopCnt`))
    (:`  `
      (if (>= _result (`self.MaxDestroyLoopCnt`))
        (`KismetSystemLibrary.K2_ClearAndInvalidateTimerHandle` (`self.DestroyVFXTimer`))))))

(fn `SpawnDestroyVFXTimer`
  (bind _returnvalue (`NiagaraFunctionLibrary.SpawnSystemAtLocation` "/Game/Assets/VFX/Gunner_Shooter_VFX/Effects/Bomb/NS_Bomb_Explosion_1.NS_Bomb_Explosion_1" (`self.BoundOrigin`)))
  (`GameplayStatics.SpawnSoundAttached` "/Game/Assets/Sounds/SoundCue/SC_Explosion_2.SC_Explosion_2" _returnvalue "None" (0.0 0.0 0.0) (struct) "KeepRelativeOffset" false 1.0 1.0 0.0 "/Game/Assets/Sounds/SoundAttenuation/SA_Test.SA_Test" null)
  (`FXSystemComponent.SetFloatParameter` _returnvalue "Overall_Scale" (* (`self.BoundRadious`) 0.025))
  (message `/Game/Interfaces/BPI_ChaosDestructable.SpawnChaosDestruct` self "All"))

(fn `SpawnFSMasterField`
  (params (`FS Master Field Transform` :type "Transform Structure") (`Radial Magnitude` :type "Float (double-precision)") (`Directional Magnitude` :type "Float (double-precision)") (`Torque Mult` :type "Float (double-precision)"))
  (locals (FSMasterField :type "/Engine/EditorResources/FieldNodes/FS_MasterField Object Reference"))
  (bind _fsmasterfield (`local.FSMasterField`))
  (bind _returnvalue (`|SpawnActorFromClass` "/Engine/EditorResources/FieldNodes/FS_MasterField.FS_MasterField_C" (`KismetMathLibrary.MakeTransform` `FS Master Field Transform_Location` `FS Master Field Transform_Rotation` (`.BoxExtent` (`self.GetActorBounds` false true))) "AlwaysSpawn" "OverrideRootScale" null null))
  (set `local.FSMasterField` _returnvalue)
  (`|ExecutionSequence`
    (:`then_0`
      (set `/Engine/EditorResources/FieldNodes/FS_MasterField.Field Falloff Shape` "NewEnumerator0" (`local.FSMasterField`)))
    (:`then_1`
      (set `/Engine/EditorResources/FieldNodes/FS_MasterField.ActivationType` "NewEnumerator2" (`local.FSMasterField`)))
    (:`then_2`
      (`self.SetLifeSpan` (`local.FSMasterField`) 0.1))
    (:`then_3`
      (set `/Engine/EditorResources/FieldNodes/FS_MasterField.Radial Magnitude` (`local.Radial Magnitude`) (`local.FSMasterField`)))
    (:`then_4`
      (set `/Engine/EditorResources/FieldNodes/FS_MasterField.UseDirectionalVector` true _fsmasterfield)
      (set `/Engine/EditorResources/FieldNodes/FS_MasterField.DirectionalMagnitude` (`local.Directional Magnitude`) _fsmasterfield))
    (:`then_5`
      (set `/Engine/EditorResources/FieldNodes/FS_MasterField.TorqueMult` (`local.Torque Mult`) (`local.FSMasterField`)))))

(fn `UnableComponentsCollision`
  (for _array_element (`self.NoBoundComponents`)
    (`PrimitiveComponent.SetCollisionEnabled` _array_element "NoCollision")))

(fn `UserConstructionScript`)