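; BP_BD_MineralMiner is the mineral miner extractor building, a child Blueprint that mostly relies on its parent's behavior.
; It extends the parent's SpawnChaosDestruct by adding a Geometry Collection component at the static mesh's relative transform.
; It then spawns an FS master field at the mesh's world transform with radial, directional and torque forces for Chaos destruction.
; An unconnected debug print reports skeletal mesh animation position and length.
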(event `self.ReceiveBeginPlay`
  (`parent.ReceiveBeginPlay`))

(event `/Game/Interfaces/BPI_ChaosDestructable.SpawnChaosDestruct`
  (params (Part :type Name))
  (bind _staticmesh (`self.StaticMesh`))
  (`|ExecutionSequence`
    (:`then_0`
      (`parent.SpawnChaosDestruct` Part))
    (:`then_1`
      (`AddComponent|NODE_AddGeometryCollectionComponent-0` :`RelativeTransform` (`SceneComponent.GetRelativeTransform` _staticmesh))
      (`self.SpawnFSMasterField` (`SceneComponent.K2_GetComponentToWorld` _staticmesh) 40.0 10.0 2.0))))

(fn `UserConstructionScript`
  (`parent.UserConstructionScript`))