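; Blueprint for the Organic Extractor building, adding its own Chaos destruction on top of the parent class behavior.
; SpawnChaosDestruct calls the parent, then adds a geometry collection at the static mesh's relative transform and spawns an FS master field at its world transform.
; The field receives radial, directional and torque settings to drive the break-up.
; BeginPlay, overlap and Tick are disabled stubs, and construction only calls the parent.
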(event `/Game/Interfaces/BPI_ChaosDestructable.SpawnChaosDestruct`
  (params (Part :type Name))
  (bind _staticmesh (`self.StaticMesh`))
  (`|ExecutionSequence`
    (:`then_0`
      (`parent.SpawnChaosDestruct` Part))
    (:`then_1`
      (`AddComponent|NODE_AddGeometryCollectionComponent-0` :`RelativeTransform` (`SceneComponent.GetRelativeTransform` _staticmesh))
      (`self.SpawnFSMasterField` (`SceneComponent.K2_GetComponentToWorld` _staticmesh) 40.0 10.0 2.0))))

(fn `UserConstructionScript`
  (`parent.UserConstructionScript`))