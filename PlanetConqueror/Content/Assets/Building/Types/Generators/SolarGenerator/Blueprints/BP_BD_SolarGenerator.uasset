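; Solar generator building Blueprint that extends a parent building with base-resource accounting and Chaos destruction.
; On BeginPlay it applies the negated expendable cost of one resource to the game state if not flagged as spawned, and registers its skeletal mesh in NoBoundComponents.
; On destruction it adds a geometry collection at the static mesh's transform, breaks it with an FS master field, and reverses the resource change unless it is a ghost.
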(event `self.ReceiveBeginPlay`
  (`parent.ReceiveBeginPlay`)
  (if (not (`self.IsSpawned`))
    (bind _asbp_gs_in_game (cast `/Game/GameMode/BP_GS_InGame` (`GameplayStatics.GetGameState`)))
    (`/Game/GameMode/BP_GS_InGame.IncreaseBaseResource` _asbp_gs_in_game "NewEnumerator3" (* (`BlueprintMapLibrary.Map_Find` (`self.ExpendableCosts`) "NewEnumerator3") -1))
    (`KismetArrayLibrary.Array_Add` (`self.NoBoundComponents`) (`self.SkeletalMesh`))))

(event `/Game/Interfaces/BPI_ChaosDestructable.SpawnChaosDestruct`
  (params (Part :type Name))
  (bind _staticmesh (`self.StaticMesh`))
  (`|ExecutionSequence`
    (:`then_0`
      (`parent.SpawnChaosDestruct` Part))
    (:`then_1`
      (`AddComponent|NODE_AddGeometryCollectionComponent-0` :`RelativeTransform` (`SceneComponent.GetRelativeTransform` _staticmesh))
      (`self.SpawnFSMasterField` (`SceneComponent.K2_GetComponentToWorld` _staticmesh) 45.0 20.0 2.0)
      (if (not (`self.IsGhost`))
        (bind _asbp_gs_in_game (cast `/Game/GameMode/BP_GS_InGame` (`GameplayStatics.GetGameState`)))
        (`/Game/GameMode/BP_GS_InGame.IncreaseBaseResource` _asbp_gs_in_game "NewEnumerator3" (`BlueprintMapLibrary.Map_Find` (`self.ExpendableCosts`) "NewEnumerator3"))))))

(fn `UserConstructionScript`
  (`parent.UserConstructionScript`))