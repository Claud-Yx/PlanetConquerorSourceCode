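; Enemy portal structure that scales up from zero, releases a queue of enemies on a timer, and can shrink and destroy itself afterwards.
; Scaling uses zero-delay interpolation loops instead of Tick, with a gate halting growth on despawn.
; The spawn policy expands enemy amounts into an ordered or random queue.
; Each enemy receives patrol and target data, then launches upward in a random direction; manually placed portals self-start after a delay.
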(event `self.ReceiveBeginPlay`
  (bind (_returnvalue_x _returnvalue_y _returnvalue_z) (`KismetMathLibrary.BreakVector` (`self.K2_GetActorLocation`)))
  (bind _fixed_target (`self.Fixed Target`))
  (bind (_returnvalue_roll _returnvalue_pitch _returnvalue_yaw) (`KismetMathLibrary.BreakRotator` (`KismetMathLibrary.FindLookAtRotation` (`self.K2_GetActorLocation`) (`self.K2_GetActorLocation` _fixed_target))))
  (`parent.ReceiveBeginPlay`)
  (`self.SetActorScale3D` (0.0 0.0 0.0))
  (`/Engine/EditorBlueprintResources/StandardMacros.IsValid` _fixed_target
    (:`Is Valid`
      (`self.K2_SetActorRotation` (`KismetMathLibrary.MakeRotator` 0.0 0.0 _returnvalue_yaw)))
    (:`Is Not Valid`
      _))
  (`self.K2_SetActorLocation` (`KismetMathLibrary.MakeVector` _returnvalue_x _returnvalue_y (+ _returnvalue_z (`self.DistToGround`))))
  ;[1 0 0.0501] 임시
  (if (`self.IsManualSpawnedPortal`)
    (`KismetSystemLibrary.Delay` (`self.StartTimer`))
    (`self.StartSpawnPortal` 1.0)
    (`self.StartSpawnEnemyTimer`)))

(event `StartSpawnPortal`
  (params (SpawnInterp :type "Float (double-precision)" :default 1.0))
  (set `self.PortalInterpSpeed` SpawnInterp)
  (`self.SpawnPortalDelay`))

(event `SpawnPortalDelay`
  (`/Engine/EditorBlueprintResources/StandardMacros.Gate` false :!label _label
    (:`Exit`
      (`KismetSystemLibrary.Delay` 0.0)
      (`self.SpawnPortalCycle`))))

(event `StartDespawnPortal`
  (params (`Spawn Time` :type "Float (double-precision)" :default 1.0))
  (`|ExecutionSequence`
    (:`then_0`
      (goto _label :!via `Close`))
    (:`then_1`
      (set `self.PortalInterpSpeed` `Spawn Time`)
      (`self.DespawnPortalDelay`))))

(event `DespawnPortalDelay`
  (`KismetSystemLibrary.Delay` 0.0)
  (`self.DespawnPortalCycle`))

(event `SpawnEnemy OS`
  (params (Class :type "/Game/Assets/Characters/Enemy/BaseBlueprints/BP_EnemyBase Class Reference") (PatrolBase :type "Actor Object Reference") (FixedTarget :type "Actor Object Reference") (ItemAppearanceData :type "/Game/Structs/S_ItemAppearanceData Structure"))
  (bind (_returnvalue_location _returnvalue_rotation) (`KismetMathLibrary.BreakTransform` (`self.GetTransform`)))
  (bind _returnvalue (`|SpawnActorFromClass` Class (`KismetMathLibrary.MakeTransform` _returnvalue_location _returnvalue_rotation) "Undefined" "OverrideRootScale" null 50.0 PatrolBase FixedTarget ItemAppearanceData null))
  (bind _output_get (set `self.RandomImpulse` (* (`KismetMathLibrary.GetForwardVector` (`KismetMathLibrary.MakeRotator` 0.0 (`KismetMathLibrary.RandomFloatInRange` 60.0 80.0) (* (`KismetMathLibrary.RandomFloatInRange` 0.0 36.0) 10.0))) (`KismetMathLibrary.RandomFloatInRange` 1100.0 1350.0))))
  (bind (_returnvalue_roll _returnvalue_pitch _returnvalue_yaw) (`KismetMathLibrary.BreakRotator` (`KismetMathLibrary.Conv_VectorToRotator` _output_get)))
  (`self.K2_SetActorRotation` _returnvalue (`KismetMathLibrary.MakeRotator` 0.0 0.0 _returnvalue_yaw) false)
  (`CharacterMovementComponent.AddImpulse` (`Character.CharacterMovement` _returnvalue) (`self.RandomImpulse`) true))

(fn `DespawnPortalCycle`
  (`self.SetActorScale3D` (`KismetMathLibrary.VInterpTo` (`self.GetActorScale3D`) (0.0 0.0 0.0) (`GameplayStatics.GetWorldDeltaSeconds`) (`self.PortalInterpSpeed`)))
  (if (== (0.0 0.0 0.0) (`self.GetActorScale3D`) :`ErrorTolerance` 0.1)
    (`self.SetActorScale3D` (0.0 0.0 0.0))
    (set `self.IsSpawned` false)
    (set `self.IsDestroyed` true)
    (`self.K2_DestroyActor`)
    (else
      (`self.DespawnPortalDelay`))))

(fn `SpawnEnemy`
  (params (Class :type "/Game/Assets/Characters/Enemy/BaseBlueprints/BP_EnemyBase Class Reference") (PatrolBase :type "Actor Object Reference") (FixedTarget :type "Actor Object Reference") (ItemAppearanceData :type "/Game/Structs/S_ItemAppearanceData Structure"))
  (`self.SpawnEnemy OS` Class PatrolBase FixedTarget ItemAppearanceData))

(fn `SpawnEnemyTimer`
  (bind _output (`/Game/Macros/GlobalMacros.Front` (`self.OrderedSpawningEnemies`))
    (:`Succeed`
      (`self.SpawnEnemy` _output (`self.Patrol Base`) (`self.Fixed Target`) (`self.Item Appearance Data`))
      (`/Game/Macros/GlobalMacros.PopFront` (`self.OrderedSpawningEnemies`)
        (:`Succeed`
          (`/Engine/EditorBlueprintResources/StandardMacros.DecrementInt` (`self.SpawnCount`)
            (:`  `
              (if (<= (`self.SpawnCount`) 0)
                (if (`self.Despawn After Spawn Enemies`)
                  (`self.StartDespawnPortal` 1.0))
                (else
                  (`KismetSystemLibrary.K2_SetTimer` null "SpawnEnemyTimer" (`self.EnemySpawnDelay`)))))))))))

(fn `SpawnPortalCycle`
  (`self.SetActorScale3D` (`KismetMathLibrary.VInterpTo` (`self.GetActorScale3D`) (`self.OriginalScale`) (`GameplayStatics.GetWorldDeltaSeconds`) (`self.PortalInterpSpeed`)))
  (if (== (`self.OriginalScale`) (`self.GetActorScale3D`) :`ErrorTolerance` 0.1)
    (`self.SetActorScale3D` (`self.OriginalScale`))
    (set `self.IsSpawned` true)
    (else
      (`self.SpawnPortalDelay`))))

(fn `StartSpawnEnemyTimer`
  (locals (CurAmount :type Integer) (SpawningEnemiesTmp :type "Array of /Game/Structs/S_EnemySpawnAmount Structure") (CurIndex :type Integer :default 0))
  (bind _spawningenemiestmp (`local.SpawningEnemiesTmp`))
  (bind _curamount (`local.CurAmount`))
  (`|ExecutionSequence`
    (:`then_0`
      (switch `/Game/EnumClasses/Policies/E_EnemySpawnPolicy` (`self.EnemySpawnPolicy`)
        (:`NewEnumerator0`
          ;[1 1 1] In Order
          (for _array_element (`self.SpawningEnemies`)
            (set `local.CurAmount` (`.Amount_85_8619E27C4C13E5120EBDA5A280D7115B` (break `/Game/Structs/S_EnemySpawnAmount` _array_element)))
            (if (> _curamount 0) :!label _label
              (`KismetArrayLibrary.Array_Add` (`self.OrderedSpawningEnemies`) (`.TypeClass_84_C6F11D2140E11F27FAB692A22CFC41F3` (break `/Game/Structs/S_EnemySpawnAmount` _array_element)))
              (`/Engine/EditorBlueprintResources/StandardMacros.DecrementInt` _curamount
                (:`  `
                  (goto _label))))))
        (:`NewEnumerator1`
          (set `local.SpawningEnemiesTmp` (`self.SpawningEnemies`))
          (while (`KismetArrayLibrary.Array_IsNotEmpty` _spawningenemiestmp)
            (bind _output_get (set `local.CurIndex` (`.OutIndex` (`KismetArrayLibrary.Array_Random` _spawningenemiestmp))))
            (bind (_output_typeclass _output_amount) (break `/Game/Structs/S_EnemySpawnAmount` (`|GetArrayItem` (`local.SpawningEnemiesTmp`) _output_get)))
            (if (> _output_amount 0)
              (`KismetArrayLibrary.Array_Add` (`self.OrderedSpawningEnemies`) _output_typeclass)
              (`/Engine/EditorBlueprintResources/StandardMacros.DecrementInt` _output_amount)
              (else
                (`KismetArrayLibrary.Array_Remove` (`local.SpawningEnemiesTmp`) (`local.CurIndex`))))))))
    (:`then_1`
      (set `self.SpawnCount` (`KismetArrayLibrary.Array_Length` (`self.OrderedSpawningEnemies`)))
      (`KismetSystemLibrary.K2_SetTimer` null "SpawnEnemyTimer" (`self.EnemySpawnDelay`)))))

(fn `UserConstructionScript`
  (`parent.UserConstructionScript`)
  (set `self.OriginalScale` (`self.GetActorScale3D`)))