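; Dyson Panel Launcher building that fires at the BP_Dyson actor and increases its panel count by one per shot.
; Tick runs through a Delay as a roughly one-second fire loop, with the first shot offset by Noise.
; Each cycle yaws the body and pitches the gun toward the Dyson, then fires BPCMuzzle with railgun effects and a long beam.
; Destruction adds a geometry collection and spawns a master field to scatter it.
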(event `/Game/Interfaces/BPI_ChaosDestructable.SpawnChaosDestruct`
  (params (Part :type Name))
  (bind _base (`self.Base`))
  (`|ExecutionSequence`
    (:`then_0`
      (`parent.SpawnChaosDestruct` Part))
    (:`then_1`
      (`AddComponent|NODE_AddGeometryCollectionComponent-0` :`RelativeTransform` (`SceneComponent.GetRelativeTransform` _base))
      (`self.SpawnFSMasterField` (`SceneComponent.K2_GetComponentToWorld` _base) 80.0 30.0 2.0))))

(event `self.ReceiveBeginPlay`
  (`parent.ReceiveBeginPlay`)
  (`/Game/Assets/Components/Muzzle/BPC_Muzzle.Initialize` (`self.BPC_Muzzle`) self (make `/Game/Structs/S_MuzzleData` 60.0 0 0.0 0.0 1 0.0 1 (make `/Game/Structs/S_BL_Data` null (`|MakeMap` "NewEnumerator1" "/Game/Blueprints/Building/Buildables/NS_Railgun_Muzzle.NS_Railgun_Muzzle" :!type "/Game/EnumClasses/E_BL_VFX Enum" :!valuetype "NiagaraSystem Object Reference") (`|MakeMap` "NewEnumerator1" (make `/Game/Structs/S_AudioProperty` "/Game/Assets/Sounds/SoundWave/SW_Railgun_1.SW_Railgun_1" 1.0 0.2 "/Game/Assets/Sounds/SoundAttenuation/SA_Test.SA_Test") :!type "/Game/EnumClasses/E_BL_VFX Enum") (struct) _ _ (`|MakeArray` "NewEnumerator0" "NewEnumerator8" "NewEnumerator1" "NewEnumerator2" "NewEnumerator5" "NewEnumerator6" "NewEnumerator7" :!type "/Game/EnumClasses/E_ForceType Enum"))))
  (set `self.ShootDelay` (* (`self.Noise`) 1.0)))

(event `self.ReceiveTick`
  (params (DeltaSeconds :type "Float (single-precision)"))
  (bind _bpc_muzzle (`self.BPC_Muzzle`))
  (bind _gun (`self.Gun`))
  (bind _gun_2 (`self.Gun`))
  (bind _body (`self.Body`))
  (bind (_returnvalue_roll _returnvalue_pitch _returnvalue_yaw) (`KismetMathLibrary.BreakRotator` (`SceneComponent.K2_GetComponentRotation` _gun_2)))
  (bind (_returnvalue_roll_2 _returnvalue_pitch_2) (`KismetMathLibrary.BreakRotator` (`SceneComponent.K2_GetComponentRotation` _body)))
  (bind _vfx (`/Game/Assets/Components/Muzzle/BPC_Muzzle.VFX` _bpc_muzzle))
  (`KismetSystemLibrary.Delay` (`self.ShootDelay`))
  (set `self.ShootDelay` 1.0)
  (bind _returnvalue (`GameplayStatics.GetActorOfClass` "/Game/Assets/Environment/Types/DysonSphere/BP_Dyson.BP_Dyson_C"))
  (bind (_returnvalue_roll_3 _returnvalue_pitch_3 _returnvalue_yaw_2) (`KismetMathLibrary.BreakRotator` (`KismetMathLibrary.FindLookAtRotation` (`SceneComponent.K2_GetComponentLocation` (`self.Gun`)) (`self.K2_GetActorLocation` _returnvalue))))
  (`SceneComponent.K2_SetWorldRotation` _gun_2 (`KismetMathLibrary.MakeRotator` _returnvalue_roll _returnvalue_pitch_3 _returnvalue_yaw) false false)
  (`SceneComponent.K2_SetWorldRotation` _body (`KismetMathLibrary.MakeRotator` _returnvalue_roll_2 _returnvalue_pitch_2 _returnvalue_yaw_2) false false)
  (`/Game/Assets/Components/Muzzle/BPC_Muzzle.Shoot` _bpc_muzzle null (0.0 0.0 0.0) 0.0)
  (`/Game/Assets/Environment/Types/DysonSphere/BP_Dyson.IncreasePanel` _returnvalue 1)
  (`/Engine/EditorBlueprintResources/StandardMacros.IsValid` _vfx
    (:`Is Valid`
      (`FXSystemComponent.SetVectorParameter` _vfx "BeamEnd" (+ (* (`SceneComponent.GetForwardVector` _gun) 50000.0) (`SceneComponent.K2_GetComponentLocation` _gun))))))

(fn `UserConstructionScript`
  (`parent.UserConstructionScript`))