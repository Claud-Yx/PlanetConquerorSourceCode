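; Gun turret building that automatically tracks and shoots enemies, configured from the GunTurret data row.
; On authority, Tick refreshes the nearest enemy about once a second and fires when the muzzle is nearly aligned.
; Body and gun rotate separately toward a bullet-speed-based lead point, also on remote clients.
; Bullet damage adds sensor weight to the shooter, though targeting uses distance only, and destruction spawns Chaos debris.
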(event `self.ReceiveBeginPlay`
  (`parent.ReceiveBeginPlay`)
  (bind (_turretdata _found _rowname) (`self.Get Turret Data` "GunTurret"))
  (if _found
    (`self.Init` _turretdata)
    (`/Game/Assets/Components/Muzzle/BPC_Muzzle.Initialize` (`self.Muzzle`) self (`|GetArrayItem` (`self.Muzzles`)))
    (else
      ;[0.2316 1 0] Error Notify
      (`KismetSystemLibrary.PrintText` (`|FormatText` "Error: [{Class}] Invalid Row Name: {RowName} " (`KismetSystemLibrary.GetClassDisplayName` (`GameplayStatics.GetObjectClass` self)) _rowname)))))

(event `self.ReceiveTick`
  (params (DeltaSeconds :type "Float (single-precision)"))
  (bind _target (`self.Target`))
  (`parent.ReceiveTick` DeltaSeconds)
  (`self.Has Authority in Dedi`
    (:`Authority in Dedi`
      (`|ExecutionSequence` :!label _label
        (:`then_0`
          (`KismetSystemLibrary.Delay` 1.0)
          (bind (_nearestactor _detected) (`/Game/Assets/Components/ActorSensor/BPC_ActorSensor.DetectNearestActor` (`self.Sensor`) "/Game/Assets/Characters/Enemy/BaseBlueprints/BP_EnemyBase.BP_EnemyBase_C"))
          (if _detected
            (set `self.Target` _nearestactor)
            (else
              (set `self.Target` null))))
        (:`then_1`
          (`/Engine/EditorBlueprintResources/StandardMacros.IsValid` _target :!label _label_2
            (:`Is Valid`
              (bind _returnvalue (`/Game/Macros/GlobalFunctions.GetAimOffsetToExpectedTargetLocation` _target self (`.Speed_12_F3490B5D488958F851966D88C1A155D3` (break `/Game/Structs/S_BL_Base` (`.BaseAbility_8_9AC7F1424787AED21383DDB4C16A02F5` (break `/Game/Structs/S_BL_Data` (`/Game/Assets/Components/Muzzle/BPC_Muzzle.BulletData` (`self.Muzzle`))))))))
              (`self.RotateBody` (`self.Body`) (`KismetMathLibrary.FindLookAtRotation` (`self.K2_GetActorLocation`) _returnvalue))
              (bind _returnvalue_2 (`KismetMathLibrary.FindLookAtRotation` (`SceneComponent.K2_GetComponentLocation` (`self.Muzzle`)) _returnvalue))
              (`self.RotateGun` (`self.Gun`) _returnvalue_2)
              (bind _radians (`/Game/Macros/GlobalFunctions.Get Radians from Vectors` (`KismetMathLibrary.GetForwardVector` _returnvalue_2) (`SceneComponent.GetForwardVector` (`self.Muzzle`))))
              (set `self.DegreeToTarget` (`KismetMathLibrary.RadiansToDegrees` _radians)))))
        (:`then_2`
          (if (and (not (`self.IsDestroyed`)) (<= (`self.DegreeToTarget`) 8.0) (`KismetSystemLibrary.IsValid` (`self.Target`)))
            (`self.Has Authority in Dedi`
              (:`Authority in Dedi`
                _)
              (:`Authority`
                _))
            (`self.Shoot` (`self.Muzzle`))))))
    (:`Authority`
      (goto _label))
    (:`Remote`
      (goto _label_2))))

(event `/Game/Interfaces/BPI_ChaosDestructable.SpawnChaosDestruct`
  (params (Part :type Name))
  (bind _base (`self.Base`))
  (`|ExecutionSequence`
    (:`then_0`
      (`parent.SpawnChaosDestruct` Part))
    (:`then_1`
      (`AddComponent|NODE_AddGeometryCollectionComponent-0` :`RelativeTransform` (`SceneComponent.GetRelativeTransform` _base))
      (`self.SpawnFSMasterField` (`SceneComponent.K2_GetComponentToWorld` _base) 40.0 10.0 2.0))))

(event `/Game/Interfaces/BPI_BulletDamageble.TakeBulletDamage`
  (params (Damage :type "Float (double-precision)") (Hit :type "HitResult Structure") (Shooter :type "Actor Object Reference") (HitVFX :type "NiagaraSystem Object Reference"))
  (`parent.TakeBulletDamage` Damage Hit Shooter HitVFX)
  (`/Game/Assets/Components/ActorSensor/BPC_ActorSensor.GiveActorWeight` (`self.Sensor`) Shooter 1 "NewEnumerator2"))

(fn `UserConstructionScript`
  (`parent.UserConstructionScript`))