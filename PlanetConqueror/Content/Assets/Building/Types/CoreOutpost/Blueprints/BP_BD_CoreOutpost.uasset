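; Core Outpost building Blueprint that serves as a spawn site for a player's Conqueror Bot.
; SpawnConquerorBot traces along the SpawnPoint's forward vector, spawns the bot at the impact point and has the supplied controller possess it.
; SpawnChaosDestruct extends the parent's destruction by adding a Geometry Collection at the static mesh's transform and spawning a master field to drive the Chaos break-up.
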(event `self.ReceiveBeginPlay`
  (`parent.ReceiveBeginPlay`)
  (set `self.BuildingName` "Core Outpost"))

(event `/Game/Interfaces/BPI_ChaosDestructable.SpawnChaosDestruct`
  (params (Part :type Name))
  (bind _staticmesh (`self.StaticMesh`))
  (`|ExecutionSequence`
    (:`then_0`
      (`parent.SpawnChaosDestruct` Part))
    (:`then_1`
      (`AddComponent|NODE_AddGeometryCollectionComponent-0` :`RelativeTransform` (`SceneComponent.GetRelativeTransform` _staticmesh))
      (`self.SpawnFSMasterField` (`SceneComponent.K2_GetComponentToWorld` _staticmesh) 100.0 30.0 2.0))))

(fn `SpawnConquerorBot`
  (params (InGameController :type "/Game/Assets/Characters/Player/PlayerControl/BP_InGamePlayerController Object Reference"))
  (returns (ConquerorBot :type "/Game/Assets/Characters/Player/ConquerorBot/Blueprints/BP_ConquerorBot Object Reference"))
  (bind _spawnpoint (`self.SpawnPoint`))
  (bind _ingamecontroller (`local.InGameController`))
  (bind _returnvalue (`SceneComponent.K2_GetComponentLocation` _spawnpoint))
  (`/Engine/EditorBlueprintResources/StandardMacros.IsValid` InGameController
    (:`Is Valid`
      (bind _outhit (`KismetSystemLibrary.LineTraceSingle` _returnvalue (+ _returnvalue (* (`SceneComponent.GetForwardVector` _spawnpoint) 2000.0)) "TraceTypeQuery1"))
      (bind _returnvalue_2 (`|SpawnActorFromClass` "/Game/Assets/Characters/Player/ConquerorBot/Blueprints/BP_ConquerorBot.BP_ConquerorBot_C" (`KismetMathLibrary.MakeTransform` (`.ImpactPoint` (`GameplayStatics.BreakHitResult` _outhit))) "Undefined" "OverrideRootScale" _ingamecontroller _ingamecontroller null))
      (`Controller.Possess` _ingamecontroller _returnvalue_2)
      (return _returnvalue_2))))

(fn `UserConstructionScript`
  (`parent.UserConstructionScript`))