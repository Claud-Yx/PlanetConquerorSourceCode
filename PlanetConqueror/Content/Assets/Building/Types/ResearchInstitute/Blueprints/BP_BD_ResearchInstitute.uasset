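; BP_BD_ResearchInstitute is the Research Institute building, which runs one timed upgrade at a time.
; StartUpgrade stores the upgrade data and its UI panel, then Tick accumulates time and drives the panel's progress bar.
; On completion it finishes and releases the panel and calls UpgradeFinished with the upgrade data.
; When destroyed, it adds a Geometry Collection and spawns a master field for Chaos fracturing.
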(event `self.ReceiveTick`
  (params (DeltaSeconds :type "Float (single-precision)"))
  (`parent.ReceiveTick` DeltaSeconds)
  (`/Engine/EditorBlueprintResources/StandardMacros.IsValid` (`self.AssignedUpgradePanel`)
    (:`Is Valid`
      (`self.UpgradeCycle`))))

(event `/Game/Interfaces/BPI_ChaosDestructable.SpawnChaosDestruct`
  (params (Part :type Name))
  (bind _staticmesh (`self.StaticMesh`))
  (`|ExecutionSequence`
    (:`then_0`
      (`parent.SpawnChaosDestruct` Part))
    (:`then_1`
      (`AddComponent|NODE_AddGeometryCollectionComponent-0` :`RelativeTransform` (`SceneComponent.GetRelativeTransform` _staticmesh))
      (`self.SpawnFSMasterField` (`SceneComponent.K2_GetComponentToWorld` _staticmesh) 50.0 15.0 1.0))))

(fn `CompleteUpgrade`
  (`/Game/Widget/HUD/Parts/WBP_Part_UpgradePanel.CompleteUpgrade` (`self.AssignedUpgradePanel`))
  (set `self.AssignedUpgradePanel` null)
  (`self.UpgradeFinished` (`self.CurUpgradeData`)))

(fn `Start Upgrade`
  (params (CurUpgradeData :type "/Game/Structs/S_UpgradeData Structure") (AssignedUpgradePanel :type "/Game/Widget/HUD/Parts/WBP_Part_UpgradePanel Object Reference"))
  (bind _output_get (set `self.AssignedUpgradePanel` AssignedUpgradePanel))
  (bind _output_get_2 (set `self.CurUpgradeData` CurUpgradeData))
  (set `self.UpgradeTime` (`.UpgradeTime_52_C3E3F7DA4BDF44F72BB10699DC45F28B` (break `/Game/Structs/S_UpgradeData` _output_get_2)))
  (set `self.CurUpgradeTime` 0.0)
  (`/Game/Widget/HUD/Parts/WBP_Part_UpgradePanel.StartUpgrade` _output_get))

(fn `UpgradeCycle`
  (bind _output_get (set `self.CurUpgradeTime` (+ (`GameplayStatics.GetWorldDeltaSeconds`) (`self.CurUpgradeTime`))))
  (set `/Game/Widget/HUD/Parts/WBP_Part_UpgradeLoading.LoadingProgress` (/ (`self.CurUpgradeTime`) (`self.UpgradeTime`)) (`/Game/Widget/HUD/Parts/WBP_Part_UpgradePanel.UpgradeProgressBar` (`self.AssignedUpgradePanel`)))
  (if (>= _output_get (`self.UpgradeTime`))
    (`self.CompleteUpgrade`)))

(fn `UserConstructionScript`)