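; Dyson sphere actor that gets built panel by panel and fires an energy beam once complete.
; Construction places it far from the world origin and creates a dynamic material; Tick orbits it around world Z and spins the mesh.
; IncreasePanel drives the material's Appearance parameter by build progress.
; On completion, ShotEnergyBeam attaches a Niagara laser to PlanetSun, ignoring its direction input.
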(event `self.ReceiveBeginPlay`)

(event `self.ReceiveTick`
  (params (DeltaSeconds :type "Float (single-precision)"))
  (bind (_relativerotation_roll _relativerotation_pitch _relativerotation_yaw) (`KismetMathLibrary.BreakRotator` (`SceneComponent.RelativeRotation` (`self.Dyson_Shphere`))))
  (`self.K2_SetActorLocation` (`KismetMathLibrary.RotateAngleAxis` (`self.K2_GetActorLocation`) (* DeltaSeconds -1.0) (0.0 0.0 1.0)))
  (`SceneComponent.K2_SetRelativeRotation` (`self.Dyson_Shphere`) (`KismetMathLibrary.MakeRotator` _relativerotation_roll _relativerotation_pitch (+ _relativerotation_yaw (* (`GameplayStatics.GetWorldDeltaSeconds`) 5.0))) false false))

(fn `IncreasePanel`
  (params (PanelAmount :type Integer :default 1))
  (if (not (`self.IsBuiltComplete`))
    (`/Engine/EditorBlueprintResources/StandardMacros.IncrementInt` (`self.PlacedPanel`)
      (:`  `
        (`MaterialInstanceDynamic.SetScalarParameterValue` (`self.Appearance`) "Appearance" (/ (`KismetMathLibrary.Conv_IntToDouble` (`self.PlacedPanel`)) (`self.MaxRequiredPanel`)))
        (if (== (`self.PlacedPanel`) (`self.MaxRequiredPanel`))
          (set `self.IsBuiltComplete` true)
          (`self.ShotEnergyBeam` (0.0 0.0 0.0)))))))

(fn `ShotEnergyBeam`
  (params (`World Direction` :type "Vector Structure"))
  (bind _returnvalue (`NiagaraFunctionLibrary.SpawnSystemAttached` "/Game/Import/VFX/Laser/NS_Lazer.NS_Lazer" (`self.Planet_Sun`) "None" (0.0 0.0 0.0) (struct) "KeepRelativeOffset"))
  (`FXSystemComponent.SetVectorParameter` _returnvalue "Length" (0.0 50000.0 0.0))
  (message `AudioParameterControllerInterface.SetFloatParameter` _returnvalue "Scale" 500000.0))

(fn `UserConstructionScript`
  (`self.K2_SetActorLocation` (* (`KismetMathLibrary.Conv_RotatorToVector` (`KismetMathLibrary.MakeRotator` 0.0 45.0)) 100000.0) false true)
  (bind _returnvalue (`PrimitiveComponent.CreateDynamicMaterialInstance` (`self.Dyson_Shphere`) 0 "/Game/Import/Dyson_Final/MI_Dyson_Final.MI_Dyson_Final" "None"))
  (bind _output_get (set `self.Appearance` _returnvalue))
  (`MaterialInstanceDynamic.SetScalarParameterValue` _output_get "Appearance" 0.0))