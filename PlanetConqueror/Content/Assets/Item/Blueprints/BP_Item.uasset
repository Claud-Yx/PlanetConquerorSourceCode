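; BP_Item is a world item that can be thrown and pulled into a character's inventory.
; Initialize takes mesh and data from the passed struct or DT_Item, optionally launching it via ProjectileMovement with a random upward impulse.
; A dedicated server pushes location to clients every tick.
; AttractToCharacter disables collision, then a zero-delay loop accelerates it toward the character, adding it to inventory when a line trace hits them.
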(event `self.ReceiveBeginPlay`
  (`KismetSystemLibrary.Delay` 0.5)
  (`PrimitiveComponent.SetCollisionProfileName` (`self.Box`) "Item" true))

(event `SyncVelocity MC`
  (bind _projectilemovement (`self.ProjectileMovement`))
  (`self.Has Athority in Dedi`
    (:`Remote`
      (set `MovementComponent.Velocity` (0.0 0.0 0.0) _projectilemovement)
      (set `ProjectileMovementComponent.ProjectileGravityScale` 0.0 _projectilemovement))))

(event `SyncLocation`
  (params (NewLocation :type "Vector Structure"))
  (`self.Has Athority in Dedi`
    (:`Remote`
      (`self.K2_SetActorLocation` NewLocation))))

(event `self.ReceiveTick`
  (params (DeltaSeconds :type "Float (single-precision)"))
  (if (== (`MovementComponent.Velocity` (`self.ProjectileMovement`)) (0.0 0.0 0.0) :`ErrorTolerance` 1e-05)
    (`ActorComponent.Deactivate` (`self.ProjectileMovement`)))
  (`self.Has Athority in Dedi`
    (:`Authority in Dedi`
      (`self.SyncLocation` (`self.K2_GetActorLocation`)))))

(event `AttractToCharacter`
  (params (Character :type "/Game/Assets/Characters/Player/ConquerorBot/Blueprints/BP_ConquerorBot Object Reference"))
  (`|ExecutionSequence`
    (:`then_0`
      (set `self.AttractingCharacter` Character)
      (`self.AttractDelay`))
    (:`then_1`
      (`PrimitiveComponent.SetSimulatePhysics` (`self.Box`) false)
      (`PrimitiveComponent.SetCollisionEnabled` (`self.Box`) "NoCollision"))
    (:`then_2`
      (`ActorComponent.Deactivate` (`self.ProjectileMovement`)))))

(event `AttractDelay`
  (`KismetSystemLibrary.Delay` 0.0)
  (`self.AttractCycle`))

(fn `AttractCycle`
  (locals (`New Location` :type "Vector Structure"))
  (bind _attractingcharacter (`self.AttractingCharacter`))
  (bind _returnvalue (`KismetMathLibrary.GetForwardVector` (`KismetMathLibrary.FindLookAtRotation` (`self.K2_GetActorLocation`) (`self.K2_GetActorLocation` (`self.AttractingCharacter`)))))
  (`|ExecutionSequence`
    (:`then_0`
      (set `self.DistToAttractingCharacter` (`KismetMathLibrary.Vector_Distance` (`self.K2_GetActorLocation` (`self.AttractingCharacter`)) (`self.K2_GetActorLocation`))))
    (:`then_1`
      (if (and (< 0.0 (`.Z` (`KismetMathLibrary.BreakVector3f` _returnvalue))) (< (`self.CurAttractingSpeed`) 0.0))
        (set `self.AttractPopDirection` (* _returnvalue (1.0 1.0 -3.0)))
        (else
          (set `self.AttractPopDirection` _returnvalue))))
    (:`then_2`
      (set `local.New Location` (+ (`self.K2_GetActorLocation`) (* (`self.AttractPopDirection`) (`self.CurAttractingSpeed`) (`GameplayStatics.GetWorldDeltaSeconds`)))))
    (:`then_3`
      (bind _outhits (`KismetSystemLibrary.LineTraceMulti` (`self.K2_GetActorLocation`) (`local.New Location`) "TraceTypeQuery1"))
      (for _array_element _outhits
        (if (== (`.HitActor` (`GameplayStatics.BreakHitResult` _array_element)) _attractingcharacter)
          (`/Game/Assets/Components/Inventory/Blueprints/BPC_Inventory.AddItem` (`/Game/Assets/Characters/Player/ConquerorBot/Blueprints/BP_ConquerorBot.Inventory` _attractingcharacter) (`.Type_11_294AC23C412A453E27D819AF24912640` (break `/Game/Structs/S_ItemData` (`self.ItemData`))) (`self.Amount`))
          (`self.K2_DestroyActor`))))
    (:`then_4`
      (`self.K2_SetActorLocation` (`local.New Location`)))
    (:`then_5`
      (set `self.CurAttractingSpeed` (`KismetMathLibrary.FMin` (+ (`self.CurAttractingSpeed`) (* (`self.AttractingAccelSpeed`) (`GameplayStatics.GetWorldDeltaSeconds`))) (`self.MaxAttractingSpeed`)))
      (`self.AttractDelay`))))

(fn `Initialize`
  (params (UserSettingData :type "/Game/Structs/S_ItemData Structure") (Type :type "/Game/EnumClasses/E_ItemType Enum" :default "NewEnumerator0") (InstantlyThrow :type Boolean))
  (bind _staticmesh (`self.StaticMesh`))
  (set `self.Amount` 1)
  (`/Engine/EditorBlueprintResources/StandardMacros.IsValid` (`.Mesh_9_F9672CD543F02922AE310F833F140CB6` (break `/Game/Structs/S_ItemData` UserSettingData))
    (:`Is Valid`
      (set `self.ItemData` UserSettingData)
      (`|ExecutionSequence` :!label _label
        (:`then_0`
          (`StaticMeshComponent.SetStaticMesh` _staticmesh (`.Mesh_9_F9672CD543F02922AE310F833F140CB6` (break `/Game/Structs/S_ItemData` (`self.ItemData`))))
          (`SceneComponent.SetRelativeScale3D` _staticmesh (1.2 1.2 1.2))
          (`BoxComponent.SetBoxExtent` (`self.Box`) (`.BoxExtent` (`KismetSystemLibrary.GetComponentBounds` (`self.StaticMesh`))) true))
        (:`then_1`
          (if (`local.InstantlyThrow`)
            (`self.Throw`)))))
    (:`Is Not Valid`
      (bind _returnvalue (`|GetDataTableRow` "/Game/DataTables/DT_Item.DT_Item" (`KismetStringLibrary.Conv_StringToName` (`|GetEnumeratorNameAsString` Type)))
        (:`then`
          (set `self.ItemData` _returnvalue)
          (goto _label))
        (:`RowNotFound`
          (`KismetSystemLibrary.PrintText` "Error: Invalid Item Row Name" true true (struct :`R` 1.0 :`G` 0.038485 :`A` 1.0) 20.0))))))

(fn `Throw`
  (`ActorComponent.Activate` (`self.ProjectileMovement`) true)
  (set `MovementComponent.Velocity` (* (`KismetMathLibrary.GetForwardVector` (`KismetMathLibrary.MakeRotator` 0.0 (`KismetMathLibrary.RandomFloatInRange` 60.0 80.0) (* (`KismetMathLibrary.RandomFloatInRange` (`self.MinThrowYaw`) (`self.MaxThrowYaw`)) 10.0))) (`KismetMathLibrary.RandomFloatInRange` 1500.0 1650.0)) (`self.ProjectileMovement`))
  (`self.SyncVelocity MC`))

(fn `UserConstructionScript`)