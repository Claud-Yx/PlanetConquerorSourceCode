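; Base enemy Blueprint handling AI setup, health, death and item drops.
; BeginPlay ensures an AI controller, passes patrol base and fixed target to its blackboard on the server, and sizes the HP bar.
; Bullet damage drains that bar, which also serves as health; depletion triggers timer-staggered Niagara explosions, skipped on dedicated servers, then delayed destruction.
; Helpers spawn random item drops and short-lived Chaos field actors for destruction.
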(event `self.ReceiveBeginPlay`
  (bind _patrolbase (`self.PatrolBase`))
  (bind _hpbar (`self.HPBar`))
  (bind _fixedtarget (`self.FixedTarget`))
  (bind _returnvalue (`AIBlueprintHelperLibrary.GetAIController` self))
  (bind (_origin _boxextent) (`KismetSystemLibrary.GetComponentBounds` (`self.Mesh`)))
  (`|ExecutionSequence`
    (:`then_0`
      (`/Engine/EditorBlueprintResources/StandardMacros.IsValid` _returnvalue
        (:`Is Valid`
          _)
        (:`Is Not Valid`
          (`self.SpawnDefaultController` self)))
      (bind _asbp_e_enemy_controller_base (cast `/Game/Assets/Characters/Enemy/BaseBlueprints/BP_E_EnemyControllerBase` _returnvalue))
      (set `self.AIController` _asbp_e_enemy_controller_base))
    (:`then_1`
      (`self.Has Athority in Dedi`
        (:`Authority in Dedi`
          _)
        (:`Authority`
          _))
      (if (`KismetSystemLibrary.IsValid` _patrolbase)
        (`BlackboardComponent.SetValueAsObject` (`AIBlueprintHelperLibrary.GetBlackboard` (`AIBlueprintHelperLibrary.GetAIController` self)) "BB_PatrolBase" _patrolbase)))
    (:`then_2`
      ;[0.7274 0.9968 1] HP Bar 위치 지정 및 초기화
      (`SceneComponent.K2_SetRelativeLocation` (`self.HPBar`) (`KismetMathLibrary.MakeVector` 0.0 0.0 (+ (.z _boxextent) (.z _boxextent))) false true)
      (bind _output_get (set `/Game/Assets/Components/BlockProgressBarComponent/BPC_BlockProgressBar.MaxValue` (`self.HP Max`) _hpbar))
      (`/Game/Assets/Components/BlockProgressBarComponent/BPC_BlockProgressBar.SetValue` _hpbar _output_get true)
      (`/Game/Assets/Components/BlockProgressBarComponent/BPC_BlockProgressBar.HideBPBar` (`self.HPBar`) false false 0.0)
      (`self.SetReplicateMovement` true))
    (:`then_3`
      (`self.Has Athority in Dedi`
        (:`Authority in Dedi`
          _)
        (:`Authority`
          _))
      (`/Engine/EditorBlueprintResources/StandardMacros.IsValid` _fixedtarget
        (:`Is Valid`
          (`BlackboardComponent.SetValueAsObject` (`AIBlueprintHelperLibrary.GetBlackboard` (`self.AIController`)) "BB_FixedObject" _fixedtarget))))))

(event `/Game/Interfaces/BPI_BulletDamageble.TakeBulletDamage`
  (params (Damage :type "Float (double-precision)") (Hit :type "HitResult Structure") (Shooter :type "Actor Object Reference") (HitVFX :type "NiagaraSystem Object Reference"))
  (bind (_origin _boxextent) (`self.GetActorBounds` true true))
  (bind _hpbar (`self.HPBar`))
  (bind _empty (`/Game/Assets/Components/BlockProgressBarComponent/BPC_BlockProgressBar.IncreaseValue` (`self.HPBar`) (* Damage -1.0) false))
  (`|ExecutionSequence`
    (:`then_0`
      (`/Game/Assets/Components/BlockProgressBarComponent/BPC_BlockProgressBar.ShowBPBar` (`self.HPBar`) true 0.2)
      (`KismetSystemLibrary.K2_ClearAndInvalidateTimerHandle` (`self.FadeOutTimer`)))
    (:`then_1`
      (if _empty
        (`/Engine/EditorBlueprintResources/StandardMacros.DoOnce` false
          (:`Completed`
            (set `self.IsDead` true)
            (`|ExecutionSequence`
              (:`then_0`
                (set `self.BoundOrigin` _origin)
                (set `self.BoundRadious` (`KismetMathLibrary.FMax` (.x _boxextent) (.y _boxextent) (.z _boxextent))))
              (:`then_1`
                ;[1 1 1] HPBar 없애기
                (`SceneComponent.SetVisibility` (`self.HPBar`) true true)
                (`/Game/Assets/Components/BlockProgressBarComponent/BPC_BlockProgressBar.HideBPBar` (`self.HPBar`) true true 1.5)
                ;[1 1 1] 충돌 끄기
                (`self.SetActorEnableCollision` false))
              (:`then_2`
                (set `/Game/Assets/Components/BlockProgressBarComponent/BPC_BlockProgressBar.BPBarLerpSpeed` 0.25 (`self.HPBar`))
                (`self.SpawnDestroyVFX MC`)
                (`KismetSystemLibrary.Delay` 4.0)
                (`self.DestroyActorOS`)))))
        (else
          ;[1 1 1] 죽지 않았을 때
          (set `/Game/Assets/Components/BlockProgressBarComponent/BPC_BlockProgressBar.TimerFadeOutTime` 0.2 _hpbar)
          (bind _returnvalue (`KismetSystemLibrary.K2_SetTimer` _hpbar "TimerHideBPBar" 2.0))
          (set `self.FadeOutTimer` _returnvalue))))))

(event `DestroyActorOS`
  (`self.K2_DestroyActor`))

(event `/Game/Interfaces/BPI_ChaosDestructable.SpawnChaosDestruct`
  (params (Part :type Name))
  (`self.SetActorEnableCollision` false)
  (`SceneComponent.SetVisibility` (`self.CapsuleComponent`) false true))

(event `SpawnItem OS`
  (params (MustCreateItems :type "Array of /Game/Structs/S_ItemAppearanceChance Structure (by ref)") (ItemChances :type "Array of /Game/Structs/S_ItemAppearanceChance Structure (by ref)") (MinTypes :type Integer) (MaxTypes :type Integer))
  (bind (_origin _boxextent) (`self.GetActorBounds` true true))
  (bind (_returnvalue_x _returnvalue_y _returnvalue_z) (`KismetMathLibrary.BreakVector` (`self.K2_GetActorLocation`)))
  (bind _selecteditems (`/Game/Macros/GlobalFunctions.GetRandomItems` MustCreateItems ItemChances MinTypes MaxTypes))
  (for _array_element _selecteditems
    (bind _returnvalue (`|SpawnActorFromClass` "/Game/Assets/Item/Blueprints/BP_Item.BP_Item_C" (`KismetMathLibrary.MakeTransform` (`KismetMathLibrary.MakeVector` _returnvalue_x _returnvalue_y (+ _returnvalue_z (.z _boxextent) (.z _boxextent)))) "Undefined" "OverrideRootScale" null (`.Amount_76_66A14F584DA575C87A7376906BD61C6E` (break `/Game/Structs/S_ItemAmount` _array_element)) 0.0 36.0 null))
    (`/Game/Assets/Item/Blueprints/BP_Item.Initialize` :`self` _returnvalue :`Type` (break `/Game/Structs/S_ItemAmount` _array_element) :`InstantlyThrow` true)))

(event `SpawnDestroyVFX MC`
  (`self.Has Athority in Dedi`
    (:`Authority`
      _)
    (:`Remote`
      _))
  ;[1 0 0] 이후 적마다 달리 한다면 수정 필요
  (`self.SpawnDestroySubVFXTimer`)
  (bind _returnvalue (`KismetSystemLibrary.K2_SetTimer` null "SpawnDestroySubVFXTimer" 0.1 true))
  (set `self.DestroyVFXTimer` _returnvalue)
  (`KismetSystemLibrary.K2_SetTimer` null "SpawnDestroyVFXTimer" 0.25))

(event `self.ReceiveTick`
  (params (DeltaSeconds :type "Float (single-precision)"))
  (if (`self.IsDead`)
    (`self.SetActorTickEnabled` false)))

(fn `Get Force`
  (returns (ForceType :type "/Game/EnumClasses/E_ForceType Enum"))
  (return "NewEnumerator2"))

(fn `SpawnDestroySubVFXTimer`
  (bind _returnvalue (`NiagaraFunctionLibrary.SpawnSystemAtLocation` "/Game/Assets/VFX/Gunner_Shooter_VFX/Effects/Bomb/NS_Bomb_Explosion_1.NS_Bomb_Explosion_1" (+ (`self.BoundOrigin`) (* (`KismetMathLibrary.RandomUnitVectorInConeInDegrees` (0.0 0.0 1.0) 135.0) (* (`self.BoundRadious`) (`KismetMathLibrary.RandomFloatInRange` 0.8 1.25))))))
  (`FXSystemComponent.SetFloatParameter` _returnvalue "Overall_Scale" (* (`KismetMathLibrary.RandomFloatInRange` 0.0055 0.008) (`self.BoundRadious`)))
  (bind _result (`/Engine/EditorBlueprintResources/StandardMacros.IncrementInt` (`self.CurDestroyLoopCnt`))
    (:`  `
      (if (>= _result (`self.MaxDestroyLoopCnt`))
        (`KismetSystemLibrary.K2_ClearAndInvalidateTimerHandle` (`self.DestroyVFXTimer`))))))

(fn `SpawnDestroyVFXTimer`
  (bind _returnvalue (`NiagaraFunctionLibrary.SpawnSystemAtLocation` "/Game/Assets/VFX/Gunner_Shooter_VFX/Effects/Bomb/NS_Bomb_Explosion_1.NS_Bomb_Explosion_1" (`self.BoundOrigin`)))
  (`FXSystemComponent.SetFloatParameter` _returnvalue "Overall_Scale" (* (`self.BoundRadious`) 0.015))
  (message `/Game/Interfaces/BPI_ChaosDestructable.SpawnChaosDestruct` self "All"))

(fn `SpawnFSMasterField`
  (params (`FS Master Field Transform` :type "Transform Structure") (`Radial Magnitude` :type "Float (double-precision)") (`Directional Magnitude` :type "Float (double-precision)") (`Torque Mult` :type "Float (double-precision)"))
  (locals (FSMasterField :type "/Engine/EditorResources/FieldNodes/FS_MasterField Object Reference"))
  (bind _fsmasterfield (`local.FSMasterField`))
  (bind _returnvalue (`|SpawnActorFromClass` "/Engine/EditorResources/FieldNodes/FS_MasterField.FS_MasterField_C" (`KismetMathLibrary.MakeTransform` `FS Master Field Transform_Location` `FS Master Field Transform_Rotation` (`.BoxExtent` (`self.GetActorBounds` false true))) "AlwaysSpawn" "OverrideRootScale" null null))
  (set `local.FSMasterField` _returnvalue)
  (`|ExecutionSequence`
    (:`then_0`
      (set `/Engine/EditorResources/FieldNodes/FS_MasterField.Field Falloff Shape` "NewEnumerator0" (`local.FSMasterField`)))
    (:`then_1`
      (set `/Engine/EditorResources/FieldNodes/FS_MasterField.ActivationType` "NewEnumerator2" (`local.FSMasterField`)))
    (:`then_2`
      (`self.SetLifeSpan` (`local.FSMasterField`) 0.1))
    (:`then_3`
      (set `/Engine/EditorResources/FieldNodes/FS_MasterField.Radial Magnitude` (`local.Radial Magnitude`) (`local.FSMasterField`)))
    (:`then_4`
      (set `/Engine/EditorResources/FieldNodes/FS_MasterField.UseDirectionalVector` true _fsmasterfield)
      (set `/Engine/EditorResources/FieldNodes/FS_MasterField.DirectionalMagnitude` (`local.Directional Magnitude`) _fsmasterfield))
    (:`then_5`
      (set `/Engine/EditorResources/FieldNodes/FS_MasterField.TorqueMult` (`local.Torque Mult`) (`local.FSMasterField`)))))

(fn `UserConstructionScript`)