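; BP_E_TestBox is a test box enemy that shatters through Chaos destruction.
; On BeginPlay it runs the parent logic, then raises the HP bar by twice the static mesh's Z bounds extent.
; SpawnChaosDestruct disables collision, hides the capsule and its children, adds a Geometry Collection at the mesh's relative transform, and spawns an FS master field at the mesh's world transform.
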(event `self.ReceiveBeginPlay`
  (bind (_origin _boxextent) (`KismetSystemLibrary.GetComponentBounds` (`self.StaticMesh`)))
  (`parent.ReceiveBeginPlay`)
  ;[1 1 1] HP Bar 위치 지정
  (`SceneComponent.K2_SetRelativeLocation` (`self.HPBar`) (`KismetMathLibrary.MakeVector` 0.0 0.0 (+ 0.0 (.z _boxextent) (.z _boxextent))) false true))

(event `/Game/Interfaces/BPI_ChaosDestructable.SpawnChaosDestruct`
  (params (Part :type Name))
  (bind _staticmesh (`self.StaticMesh`))
  (`self.SetActorEnableCollision` false)
  (`SceneComponent.SetVisibility` (`self.CapsuleComponent`) false true)
  (`AddComponent|NODE_AddGeometryCollectionComponent-0` :`RelativeTransform` (`SceneComponent.GetRelativeTransform` _staticmesh))
  (`self.SpawnFSMasterField` (`SceneComponent.K2_GetComponentToWorld` _staticmesh)))

(fn `UserConstructionScript`)