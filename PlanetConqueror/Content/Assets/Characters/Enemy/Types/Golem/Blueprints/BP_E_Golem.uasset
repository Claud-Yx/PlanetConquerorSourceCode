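; Golem enemy Blueprint: an AI melee attacker that targets bots and buildings, shatters via Chaos destruction and drops items on death.
; BPC_ActorSensor picks targets by weight, fed by AI perception and bullet shooters, decayed on a delay.
; Authority-side Tick box-traces for attack range and writes target and attack state to the Blackboard.
; Montage notifies drive attack timing, box-trace swing damage on attackable forces, and hit VFX and sound.
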(event `Noti_AttackStart`
  (bind _returnvalue (`self.K2_GetActorRotation`))
  (bind _returnvalue_2 (`self.K2_GetActorLocation`))
  (bind _returnvalue_3 (`self.GetActorForwardVector`))
  (bind (_returnvalue_x _returnvalue_y _returnvalue_z) (`KismetMathLibrary.BreakVector` (`self.K2_GetActorLocation`)))
  (bind (_sfx_hitting_itemappearancedata _sfx_hitting_volume _sfx_hitting_starttime _sfx_hitting_attenuation) (break `/Game/Structs/S_AudioProperty` (`self.SFX_Hitting`)))
  (bind _returnvalue_4 (+ _returnvalue_2 (* _returnvalue_3 300.0)))
  (`self.Has Authority in Dedi`
    (:`Authority in Dedi`
      _)
    (:`Authority`
      _))
  (bind _outhits (`KismetSystemLibrary.BoxTraceMulti` (+ _returnvalue_2 (* _returnvalue_3 100.0)) _returnvalue_4 (70.0 80.0 80.0) _returnvalue "TraceTypeQuery1"))
  (bind _newarray (`/Game/Macros/GlobalFunctions.MakeUniqueArray(HitResult)` _outhits))
  (for _array_element _newarray
    (bind (_bblockinghit _binitialoverlap _time _distance _location _impactpoint _normal _impactnormal _physmat _hitactor) (`GameplayStatics.BreakHitResult` _array_element))
    (bind _forcetype (message `/Game/Interfaces/BPI_Force.Get Force` _hitactor))
    (if (`KismetArrayLibrary.Array_Contains` (`self.AttackableForce`) _forcetype)
      (`self.Spawn VFX MC` "/Game/Import/BlinkAndDashVFX/VFX_Niagara/NS_Blink_Fire.NS_Blink_Fire" (`KismetMathLibrary.MakeVector` (.x _returnvalue_4) (.y _returnvalue_4) _returnvalue_z) _returnvalue (0.8 0.8 0.8))
      (`self.Spawn Sound Attached MC` _sfx_hitting_itemappearancedata _sfx_hitting_volume _sfx_hitting_starttime _sfx_hitting_attenuation)
      (message `/Game/Interfaces/BPI_SwingDamageble.TakeSwingDamage` _hitactor 10.0 _array_element self null))))

(event `Noti_AttackEnd`
  (set `self.IsAttacking` false))

(event `self.ReceiveBeginPlay`
  (`parent.ReceiveBeginPlay`)
  (`|ExecutionSequence`
    (:`then_0`
      (bind _asabp_e_golem (cast `/Game/Assets/Characters/Enemy/Types/Golem/Animations/ABP_E_Golem` (`SkeletalMeshComponent.GetAnimInstance` (`self.Mesh`))))
      (bind _output_get (set `self.AnimInst` _asabp_e_golem))
      (add `/Game/Assets/Characters/Enemy/Types/Golem/Animations/ABP_E_Golem.AttackStart` _output_get (delegate `Noti_AttackStart`))
      (add `/Game/Assets/Characters/Enemy/Types/Golem/Animations/ABP_E_Golem.AttackEnd` _output_get (delegate `Noti_AttackEnd`)))))

(event `/Game/Interfaces/BPI_ChaosDestructable.SpawnChaosDestruct`
  (params (Part :type Name))
  (bind _mesh (`self.Mesh`))
  (`|ExecutionSequence`
    (:`then_0`
      (`parent.SpawnChaosDestruct` Part)
      (`AddComponent|NODE_AddGeometryCollectionComponent-0` :`RelativeTransform` (`SceneComponent.GetRelativeTransform` _mesh))
      (`self.SpawnFSMasterField` (`SceneComponent.K2_GetComponentToWorld` _mesh) 50.0 20.0 1.3))))

(event `/Game/Interfaces/BPI_Attackable.BPI_Attack`
  (params (SkillName :type Name))
  (set `self.IsAttacking` true)
  (`self.Event BPI Attack MC`))

(event `Event BPI Attack MC`
  (`/Game/Assets/Characters/Enemy/Types/Golem/Animations/ABP_E_Golem.PlayAttackMontage` (`self.AnimInst`)))

(event `Spawn VFX MC`
  (params (SystemTemplate :type "NiagaraSystem Object Reference") (Location :type "Vector Structure") (Rotation :type "Rotator Structure") (Scale :type "Vector Structure") (bAutoDestroy :type Boolean :default true) (bAutoActivate :type Boolean :default true) (PoolingMethod :type "ENCPoolMethod Enum" :default "None") (bPreCullCheck :type Boolean :default true))
  (`NiagaraFunctionLibrary.SpawnSystemAtLocation` SystemTemplate Location Rotation Scale bAutoDestroy bAutoActivate PoolingMethod bPreCullCheck))

(event `Spawn Sound Attached MC`
  (params (Sound :type "SoundBase Object Reference") (VolumeMultiplier :type "Float (single-precision)") (StartTime :type "Float (single-precision)") (AttenuationSettings :type "SoundAttenuation Object Reference"))
  (`GameplayStatics.SpawnSoundAttached` Sound (`self.CapsuleComponent`) "None" (0.0 0.0 0.0) (`KismetMathLibrary.Conv_VectorToRotator` (`self.GetActorForwardVector`)) "KeepRelativeOffset" false VolumeMultiplier 1.0 StartTime AttenuationSettings null))

(event `self.ReceiveTick`
  (params (DeltaSeconds :type "Float (single-precision)"))
  (bind _returnvalue (`self.K2_GetActorLocation`))
  (bind _returnvalue_2 (`AIBlueprintHelperLibrary.GetBlackboard` (`self.AIController`)))
  (`parent.ReceiveTick` DeltaSeconds)
  (`self.Has Authority in Dedi`
    (:`Authority in Dedi`
      _)
    (:`Authority`
      _))
  (`|ExecutionSequence`
    (:`then_0`
      (`/Engine/EditorBlueprintResources/StandardMacros.IsValid` (`self.CurTargetActor`)
        (:`Is Valid`
          (`|ExecutionSequence`
            (:`then_0`
              (bind _outhits (`KismetSystemLibrary.BoxTraceMulti` _returnvalue (+ _returnvalue (* (`self.GetActorForwardVector`) 300.0)) (70.0 80.0 80.0) (`self.K2_GetActorRotation`) "TraceTypeQuery1"))
              (bind _newarray (`/Game/Macros/GlobalFunctions.MakeUniqueArray(HitResult)` _outhits))
              (set `self.CanAttack` false)
              (for _array_element _newarray
                (bind _returnvalue_3 (== (`.HitActor` (`GameplayStatics.BreakHitResult` _array_element)) (`self.CurTargetActor`)))
                (if _returnvalue_3
                  (set `self.CanAttack` _returnvalue_3)
                  (break))))
            (:`then_1`
              (if (`GameplayStatics.ObjectIsA` (`self.CurTargetActor`) "/Game/Assets/Building/BaseBlueprints/BP_BuildingBase.BP_BuildingBase_C")
                (set `self.IsBuildingTarget` true)
                (else
                  (set `self.IsBuildingTarget` false))))
            (:`then_2`
              (`|ExecutionSequence`
                (:`then_0`
                  (`BlackboardComponent.SetValueAsBool` _returnvalue_2 "BB_CanAttack" (`self.CanAttack`)))
                (:`then_1`
                  (`BlackboardComponent.SetValueAsBool` _returnvalue_2 "BB_IsAttacking" (`self.IsAttacking`)))
                (:`then_2`
                  (`BlackboardComponent.SetValueAsBool` _returnvalue_2 "BB_IsBuildingTarget" (`self.IsBuildingTarget`)))))))))
    (:`then_1`
      (`KismetSystemLibrary.Delay` 2.0)
      (bind (_highestweightactor _detected) (`/Game/Assets/Components/ActorSensor/BPC_ActorSensor.DetectHighestWeightActor` (`self.BPC_ActorSensor`) "NewEnumerator0" "/Script/Engine.Actor"))
      (set `self.CurTargetActor` _highestweightactor)
      (`BlackboardComponent.SetValueAsObject` (`AIBlueprintHelperLibrary.GetBlackboard` (`self.AIController`)) "BB_TargetObject" (`self.CurTargetActor`)))
    (:`then_2`
      (`KismetSystemLibrary.Delay` 2.0)
      (`/Game/Assets/Components/ActorSensor/BPC_ActorSensor.GiveAllExistedActorsWeight` (`self.BPC_ActorSensor`) -1 "NewEnumerator1" true))))

(event `/Game/Interfaces/BPI_BulletDamageble.TakeBulletDamage`
  (params (Damage :type "Float (double-precision)") (Hit :type "HitResult Structure") (Shooter :type "Actor Object Reference") (HitVFX :type "NiagaraSystem Object Reference"))
  (bind (_itemappearancedata_mustcreateitems _itemappearancedata_itemchances _itemappearancedata_mintypes _itemappearancedata_maxtypes) (break `/Game/Structs/S_ItemAppearanceData` (`self.ItemAppearanceData`)))
  (bind _bpc_actorsensor (`self.BPC_ActorSensor`))
  (`parent.TakeBulletDamage` Damage Hit Shooter HitVFX)
  (`|ExecutionSequence`
    (:`then_0`
      (if (`self.IsDead`)
        (`self.SpawnItem OS` _itemappearancedata_mustcreateitems _itemappearancedata_itemchances _itemappearancedata_mintypes _itemappearancedata_maxtypes)))
    (:`then_1`
      (bind _actorweight (`/Game/Assets/Components/ActorSensor/BPC_ActorSensor.GiveActorWeight` _bpc_actorsensor Shooter 1 "NewEnumerator2"))
      (`KismetArrayLibrary.Array_AddUnique` (`/Game/Assets/Components/ActorSensor/BPC_ActorSensor.ExternActors` _bpc_actorsensor) (break `/Game/Structs/S_ActorWeight` _actorweight)))))

(event `self.AIPerception.OnTargetPerceptionUpdated`
  (params (Actor :type "Actor Object Reference") (Stimulus :type "AIStimulus Structure"))
  (bind _output (`|GetArrayItem` (`Actor.Tags` Actor)))
  (bind _externactors (`/Game/Assets/Components/ActorSensor/BPC_ActorSensor.ExternActors` (`self.BPC_ActorSensor`)))
  (`/Game/Assets/Components/ActorSensor/BPC_ActorSensor.RefreshExternActors` (`self.BPC_ActorSensor`))
  (if (and (`.bSuccessfullySensed` (break `AIStimulus` Stimulus)) (or (== _output "ConquerorBot") (== _output "Building")))
    (`KismetArrayLibrary.Array_AddUnique` _externactors Actor)
    (else
      (`KismetArrayLibrary.Array_RemoveItem` _externactors Actor)))
  (bind (_highestweightactor _detected) (`/Game/Assets/Components/ActorSensor/BPC_ActorSensor.DetectHighestWeightActor` (`self.BPC_ActorSensor`) "NewEnumerator0" "/Script/Engine.Actor"))
  (if _detected
    (set `self.CurTargetActor` _highestweightactor)
    (else
      (set `self.CurTargetActor` null)))
  (`BlackboardComponent.SetValueAsObject` (`AIBlueprintHelperLibrary.GetBlackboard` (`self.AIController`)) "BB_TargetObject" (`self.CurTargetActor`)))

(fn `UserConstructionScript`
  (`parent.UserConstructionScript`))