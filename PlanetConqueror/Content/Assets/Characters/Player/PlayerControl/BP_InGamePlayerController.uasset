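; In-game player controller that handles resource payments through the game state, which it caches on BeginPlay.
; PayResources pays on the game state locally and, if that succeeds, passes the cost through an OS-to-MC event chain (apparently server, then multicast) that calls the game state's payment again.
; A helper macro splits execution into dedicated-server authority, other authority and remote paths.
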(event `self.ReceiveBeginPlay`
  (bind _asbp_gs_in_game (cast `/Game/GameMode/BP_GS_InGame` (`GameplayStatics.GetGameState`)))
  (set `self.GameState` _asbp_gs_in_game))

(event `PayResources OS`
  (params (Cost :type "Map of /Game/EnumClasses/E_Expendable Enum to Integer"))
  (`self.PayResources MC` Cost))

(event `PayResources MC`
  (params (Cost :type "Map of /Game/EnumClasses/E_Expendable Enum to Integer"))
  (`/Game/GameMode/BP_GS_InGame.Pay Resources` (`self.GameState`) Cost))

(fn `PayResources`
  (params (Cost :type "Map of /Game/EnumClasses/E_Expendable Enum to Integer"))
  (returns (IsPaid :type Boolean) (Remains :type "Map of /Game/EnumClasses/E_Expendable Enum to Integer"))
  (bind (_ispaid _remains) (`/Game/GameMode/BP_GS_InGame.Pay Resources` (`self.GameState`) Cost))
  (if _ispaid
    (`self.PayResources OS` Cost))
  (return _ispaid _remains))

(fn `UserConstructionScript`)