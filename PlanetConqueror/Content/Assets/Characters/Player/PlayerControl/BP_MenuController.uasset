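; BP_MenuController is a menu player controller meant to switch between title and lobby HUD widgets.
; OnConnect opens the given IP address as a level, and CreateWidget replaces the current widget and shows the mouse cursor.
; BeginPlay, SwitchTitle and SwitchLobby are empty, so BackToTitle has no effect.
; The level-name switch, widget creation and binding, and lobby player registration are all disconnected and never run.
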(event `self.ReceiveBeginPlay`)

(event `SwitchTitle`)

(event `OnConnect`
  (params (`IP Address` :type Name))
  (`GameplayStatics.OpenLevel` `IP Address`))

(event `SwitchLobby`)

(event `Back To Title`
  (`self.SwitchTitle`))

(fn `Create Widget`
  (params (Class :type "UserWidget Class Reference"))
  (bind _curwidget (`self.CurWidget`))
  (`/Engine/EditorBlueprintResources/StandardMacros.IsValid` _curwidget
    (:`Is Valid`
      (`Widget.RemoveFromParent` _curwidget))
    (:`Is Not Valid`
      _))
  (bind _returnvalue (`|CreateWidget` Class self))
  (set `self.CurWidget` _returnvalue)
  (`UserWidget.AddToViewport` _returnvalue 0)
  (set `self.bShowMouseCursor` true))

(fn `UserConstructionScript`)