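; BP_FixedTPP is a ConquerorBot player pawn with a third-person spring-arm camera setup and look controls.
; On BeginPlay it sets the spring arm's location, rotation and length from its variables, then adds the attack-mode Enhanced Input mapping context, falling back to player 0's controller if none is set.
; The IA_Look action feeds its X and Y values into controller yaw and pitch.
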(event `self.ReceiveBeginPlay`
  (bind _returnvalue (pcsubsystem `EnhancedInputLocalPlayerSubsystem` (`self.PlayerController`)))
  (`SceneComponent.K2_SetRelativeLocation` (`self.SpringArm`) (`self.SpringArmLocation`) false false)
  (`SceneComponent.K2_SetRelativeRotation` (`self.SpringArm`) (`self.SpringArmRotation`) false false)
  (set `SpringArmComponent.TargetArmLength` (`self.SpringArmLength`) (`self.SpringArm`))
  (`/Engine/EditorBlueprintResources/StandardMacros.IsValid` (`self.PlayerController`)
    (:`Is Valid`
      _)
    (:`Is Not Valid`
      (set `self.PlayerController` (`GameplayStatics.GetPlayerController` 0))))
  (`/Engine/EditorBlueprintResources/StandardMacros.IsValid` _returnvalue
    (:`Is Valid`
      (`EnhancedInputSubsystemInterface.AddMappingContext` _returnvalue "/Game/Assets/Characters/Player/PlayerControl/Input/Contexts/InGame/IMC_CB_AttackMode.IMC_CB_AttackMode" 0 (struct)))))

(event `EnhancedInput|/Game/Assets/Characters/Player/PlayerControl/Input/Actions/IA_Look`
  (params (ActionValue :type "Vector2D Structure") (ElapsedSeconds :type "Float (double-precision)") (TriggeredSeconds :type "Float (double-precision)") (InputAction :type "InputAction Object Reference" :default "/Game/Assets/Characters/Player/PlayerControl/Input/Actions/IA_Look.IA_Look"))
  (:`Triggered`
    (`self.AddControllerYawInput` ActionValue_X)
    (`self.AddControllerPitchInput` ActionValue_Y)))

(fn `UserConstructionScript`)