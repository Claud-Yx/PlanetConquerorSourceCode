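; BP_WaveManager spawns enemy portals in a sequence of timed waves.
; After an initial delay, the SetCurrentWave macro loads the next entry from the Waves array and a timer schedules WaveTimer after that wave's delay.
; WaveTimer spawns a BP_ST_EnemyPortal at each target point, passing along its FixedTarget, then schedules the next wave until the array is exhausted.
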(event `self.ReceiveBeginPlay`
  (set `self.CurWaveIdx` 0)
  (`KismetSystemLibrary.Delay` (`self.InitDelay`))
  (`self.SetCurrentWave`
    (:`Next  `
      (`KismetSystemLibrary.K2_SetTimer` null "WaveTimer" (`.WaveDelay_75_8619E27C4C13E5120EBDA5A280D7115B` (break `/Game/Structs/S_WaveData` (`self.CurWave`)))))))

(fn `UserConstructionScript`)

(fn `WaveTimer`
  (for _array_element (`.Portals_78_3DBE996A46D8DA7BE9A70085A24715E0` (break `/Game/Structs/S_WaveData` (`self.CurWave`)))
    (bind (_spawningenemyclass _fixedtarget _patrolbase _spawndelay _despawnafterspawnenemies _targetpoint) (break `/Game/Structs/S_PortalData` _array_element))
    (`|SpawnActorFromClass` :`Class` "/Game/Assets/Building/Types/Structures/Portal/Blueprints/BP_ST_EnemyPortal.BP_ST_EnemyPortal_C" :`SpawnTransform` (`KismetMathLibrary.MakeTransform` (`self.K2_GetActorLocation` _targetpoint)) :`CollisionHandlingOverride` "Undefined" :`TransformScaleMethod` "OverrideRootScale" :`Fixed Target` _fixedtarget :`Instigator` null))
  (`self.SetCurrentWave`
    (:`Next  `
      (`KismetSystemLibrary.K2_SetTimer` null "WaveTimer" (`.WaveDelay_75_8619E27C4C13E5120EBDA5A280D7115B` (break `/Game/Structs/S_WaveData` (`self.CurWave`)))))))