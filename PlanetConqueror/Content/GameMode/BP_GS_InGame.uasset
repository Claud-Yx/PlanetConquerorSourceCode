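; BP_GS_InGame is the in-game Game State, holding the base resource pool and a Dyson progress value that rises steadily on Tick.
; Functions read and increase resources in an enum-keyed map, printing debug text for unknown types.
; PayResources stages remainders in a temporary map and commits only when every cost is affordable, while RefundResources adds costs back.
; A macro separates dedicated-server authority from other authority and remote execution.
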(event `self.ReceiveTick`
  (params (DeltaSeconds :type "Float (single-precision)"))
  (set `self.DysonProgress` (+ (/ (* DeltaSeconds 0.01) 180.0) (`self.DysonProgress`))))

(fn `GetBaseResource`
  (params (BaseResource :type "/Game/EnumClasses/E_Expendable Enum" :default "NewEnumerator0"))
  (returns (Value :type Integer))
  (bind (_value _returnvalue) (`BlueprintMapLibrary.Map_Find` (`self.BaseResources`) BaseResource))
  (if _returnvalue
    (return _value)
    (else
      ;[0 0 0] DEBUG
      (`KismetSystemLibrary.PrintText` (`|FormatText` "[GetBaseResource] Unvalid Resource Type: {T}" (`|GetEnumeratorNameAsString` BaseResource)) true true (struct :`R` 1.0 :`A` 1.0) 4.0))))

(fn `IncreaseBaseResource`
  (params (BaseResource :type "/Game/EnumClasses/E_Expendable Enum" :default "NewEnumerator0") (OffsetValue :type Integer))
  (bind (_value _returnvalue) (`BlueprintMapLibrary.Map_Find` (`self.BaseResources`) BaseResource))
  (if _returnvalue
    (`BlueprintMapLibrary.Map_Add` (`self.BaseResources`) BaseResource (+ OffsetValue _value))
    (else
      ;[0 0 0] DEBUG
      (`KismetSystemLibrary.PrintText` (`|FormatText` "[IncreaseBaseResource] Unvalid Resource Type: {T}" (`|GetEnumeratorNameAsString` BaseResource)) true true (struct :`R` 1.0 :`A` 1.0) 4.0))))

(fn `Pay Resources`
  (params (Cost :type "Map of /Game/EnumClasses/E_Expendable Enum to Integer"))
  (returns (IsPaid :type Boolean) (Remains :type "Map of /Game/EnumClasses/E_Expendable Enum to Integer"))
  (locals (TempResource :type "Map of /Game/EnumClasses/E_Expendable Enum to Object Object Reference"))
  (bind _baseresources (`self.BaseResources`))
  (bind _tempresource (`local.TempResource`))
  (bind _keys (`BlueprintMapLibrary.Map_Keys` Cost))
  (for _array_element _keys
    (bind _returnvalue (- (`BlueprintMapLibrary.Map_Find` (`self.BaseResources`) _array_element) (`BlueprintMapLibrary.Map_Find` (`local.Cost`) _array_element)))
    (if (< _returnvalue 0)
      (return false)
      (else
        (`BlueprintMapLibrary.Map_Add` (`local.TempResource`) _array_element _returnvalue))))
  (bind _keys_2 (`BlueprintMapLibrary.Map_Keys` _tempresource))
  (for _array_element_2 _keys_2
    (`BlueprintMapLibrary.Map_Add` _baseresources _array_element_2 (`BlueprintMapLibrary.Map_Find` _tempresource _array_element_2)))
  (return true _baseresources))

(fn `Refund Resources`
  (params (Cost :type "Map of /Game/EnumClasses/E_Expendable Enum to Integer"))
  (returns (Remains :type "Map of /Game/EnumClasses/E_Expendable Enum to Integer"))
  (bind _keys (`BlueprintMapLibrary.Map_Keys` Cost))
  (for _array_element _keys
    (`BlueprintMapLibrary.Map_Add` (`self.BaseResources`) _array_element (+ (`BlueprintMapLibrary.Map_Find` (`self.BaseResources`) _array_element) (`BlueprintMapLibrary.Map_Find` (`local.Cost`) _array_element))))
  (return (`self.BaseResources`)))

(fn `UserConstructionScript`)