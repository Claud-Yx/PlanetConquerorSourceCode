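; Lobby game state that spawns a LobbyManager on the authority at BeginPlay and tracks players in a four-slot array.
; PushPlayerOS relays through PushPlayerMC to fill the first free slot, printing a message when the lobby is full.
; PopPlayerOS clears the leaving player's slot directly, with no matching MC relay.
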(event `self.ReceiveBeginPlay`
  (`/Engine/EditorBlueprintResources/ActorMacros.Switch Has Authority`
    (:`Authority`
      (bind _returnvalue (`|SpawnActorFromClass` "/Game/Maps/LobbyManager.LobbyManager_C" (`KismetMathLibrary.MakeTransform` (0.0 0.0 0.0)) "Undefined" "OverrideRootScale" null null))
      (set `self.LobbyManager` _returnvalue))))

(event `PushPlayer MC`
  (params (NewPlayer :type "/Game/Assets/Characters/Player/PlayerControl/BP_MenuController Object Reference"))
  (`self.PushPlayer` NewPlayer))

(event `PushPlayer OS`
  (params (NewPlayer :type "/Game/Assets/Characters/Player/PlayerControl/BP_MenuController Object Reference"))
  (`self.PushPlayer MC` NewPlayer))

(event `PopPlayer OS`
  (params (Player :type "/Game/Assets/Characters/Player/PlayerControl/BP_MenuController Object Reference"))
  (`self.PopPlayer` Player))

(fn `PopPlayer`
  (params (Player :type "/Game/Assets/Characters/Player/PlayerControl/BP_MenuController Object Reference"))
  (for (_array_element _array_index) (`self.Players`)
    (if (== _array_element Player)
      (`KismetArrayLibrary.Array_Set` (`self.Players`) _array_index))))

(fn `PushPlayer`
  (params (NewPlayer :type "/Game/Assets/Characters/Player/PlayerControl/BP_MenuController Object Reference"))
  (for _index (range 4)
    (`/Engine/EditorBlueprintResources/StandardMacros.IsValid` (`|GetArrayItem` (`self.Players`) _index)
      (:`Is Not Valid`
        (`KismetArrayLibrary.Array_Set` (`self.Players`) _index NewPlayer)
        (return))))
  (`KismetSystemLibrary.PrintText` "Lobby has been full."))

(fn `UserConstructionScript`)