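; In-game player state for the Conqueror bot player, managing upgrade data and respawning.
; BeginPlay polls until the bot exists, caches it and its controller, and, except on dedicated servers, loads damage, fire-rate and HP upgrades from DataTables.
; Finished Institute upgrades pass through UpgradePlayerOS and UpgradePlayerOC to boost both muzzles or max HP.
; Respawn starts a timer that replaces the pawn with a new bot spawned at the core outpost.
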(event `self.ReceiveBeginPlay`
  (`|ExecutionSequence`
    (:`then_0`
      (bind _asbp_conqueror_bot (cast `/Game/Assets/Characters/Player/ConquerorBot/Blueprints/BP_ConquerorBot` (`GameplayStatics.GetPlayerCharacter` 0) :!label _label)
        (:`then`
          (bind _output_get (set `self.Player` _asbp_conqueror_bot))
          (`self.SetOwner` _output_get)
          (bind _asbp_in_game_player_controller (cast `/Game/Assets/Characters/Player/PlayerControl/BP_InGamePlayerController` (`Pawn.GetController` (`self.Player`))))
          (set `self.PlayerController` _asbp_in_game_player_controller))
        (:`CastFailed`
          (`KismetSystemLibrary.Delay` 0.0)
          (goto _label))))
    (:`then_1`
      (`self.Has Authority in Dedi`
        (:`Authority`
          _)
        (:`Remote`
          _))
      (`self.InitUpgradeDatas` "/Game/DataTables/Upgrade/DT_CU_BulletExtraDamage.DT_CU_BulletExtraDamage" (`self.BulletDamageUpgrades`) (`self.U_CM_CurBulletExtraDamageData`) :!label _label_2)
      (`self.InitUpgradeDatas` "/Game/DataTables/Upgrade/DT_CU_BPM.DT_CU_BPM" (`self.BPM_Upgrades`) (`self.U_CM_CurBPM_Data`))
      (`self.InitUpgradeDatas` "/Game/DataTables/Upgrade/DT_CU_HP.DT_CU_HP" (`self.HP_Upgrades`) (`self.U_CM_CurHP_Data`)))))

(event `InitUpgradeDatas OS`
  (`self.InitUpgradeDatas MC`))

(event `InitUpgradeDatas MC`
  (goto _label_2))

(event `SetInstitute`
  (params (Institute :type "/Game/Assets/Building/Types/ResearchInstitute/Blueprints/BP_BD_ResearchInstitute Object Reference"))
  (add `/Game/Assets/Building/Types/ResearchInstitute/Blueprints/BP_BD_ResearchInstitute.UpgradeFinished` Institute (delegate `UpgradeFinished`)))

(event `UpgradeFinished`
  (params (UpgradeData :type "/Game/Structs/S_UpgradeData Structure"))
  (`self.Has Authority in Dedi`
    (:`Authority`
      _)
    (:`Remote`
      _))
  (`self.UpgradePlayer OS` UpgradeData))

(event `UpgradePlayer OS`
  (params (UpgradeData :type "/Game/Structs/S_UpgradeData Structure"))
  (`self.UpgradePlayer OC` UpgradeData))

(event `UpgradePlayer OC`
  (params (UpgradeData :type "/Game/Structs/S_UpgradeData Structure"))
  (`self.UpgradePlayer` UpgradeData))

(fn `InitUpgradeDatas`
  (params (`Data Table` :type "DataTable Object Reference") (Array :type "Array of /Game/Structs/S_UpgradeData Structure") (`Cur Data` :type "/Game/Structs/S_UpgradeData Structure (by ref)"))
  (bind _outrownames (`DataTableFunctionLibrary.GetDataTableRowNames` `Data Table`))
  (for _array_element _outrownames
    (bind _returnvalue (`|GetDataTableRow` `Data Table` _array_element)
      (:`then`
        (`KismetArrayLibrary.Array_Add` Array _returnvalue))))
  (`|VariableSetRef` `Cur Data` (`|GetArrayItem` Array)))

(fn `Respawn`
  (set `self.HUD` (`/Game/Assets/Characters/Player/ConquerorBot/Blueprints/BP_ConquerorBot.HUD` (`self.Player`)))
  (`KismetSystemLibrary.K2_SetTimer` null "RespawnTimer" (`self.RespawnTime`)))

(fn `RespawnTimer`
  (bind _returnvalue (`GameplayStatics.GetActorOfClass` "/Game/Assets/Building/Types/CoreOutpost/Blueprints/BP_BD_CoreOutpost.BP_BD_CoreOutpost_C"))
  (`/Engine/EditorBlueprintResources/StandardMacros.IsValid` _returnvalue
    (:`Is Valid`
      (`Widget.RemoveFromParent` (`self.HUD`))
      (`self.K2_DestroyActor` (`Controller.K2_GetPawn` (`self.PlayerController`)))
      (bind _conquerorbot (`/Game/Assets/Building/Types/CoreOutpost/Blueprints/BP_BD_CoreOutpost.SpawnConquerorBot` _returnvalue (`self.PlayerController`)))
      (bind _output_get (set `self.Player` _conquerorbot))
      (`self.SetOwner` _output_get))))

(fn `UpgradePlayer`
  (params (UpgradeData :type "/Game/Structs/S_UpgradeData Structure"))
  (bind _player (`self.Player`))
  (bind _player_2 (`self.Player`))
  (bind _rightmuzzle (`/Game/Assets/Characters/Player/ConquerorBot/Blueprints/BP_ConquerorBot.RightMuzzle` _player_2))
  (bind _leftmuzzle (`/Game/Assets/Characters/Player/ConquerorBot/Blueprints/BP_ConquerorBot.LeftMuzzle` _player))
  (bind _rightmuzzle_2 (`/Game/Assets/Characters/Player/ConquerorBot/Blueprints/BP_ConquerorBot.RightMuzzle` _player))
  (bind _leftmuzzle_2 (`/Game/Assets/Characters/Player/ConquerorBot/Blueprints/BP_ConquerorBot.LeftMuzzle` _player_2))
  (bind _output (`|GetArrayItem` (`.Parameters_63_6816A3134B95D0FCEFA3B798B0A79A10` (break `/Game/Structs/S_UpgradeData` (`local.UpgradeData`)))))
  (bind _output_2 (`|GetArrayItem` (`.Parameters_63_6816A3134B95D0FCEFA3B798B0A79A10` (break `/Game/Structs/S_UpgradeData` (`local.UpgradeData`)))))
  (switch `/Game/EnumClasses/E_UpgradeType` (`.UpgradeType_59_AD1C5996408CFFED7DFFED9108910A65` (break `/Game/Structs/S_UpgradeData` UpgradeData))
    (:`NewEnumerator0`
      (`/Game/Assets/Components/Muzzle/BPC_Muzzle.IncreaseBulletExtraDamage` _leftmuzzle (* (`.Damage_8_95FA65794938F8646CAD6B9925CAF05F` (break `/Game/Structs/S_BL_Base` (`.BaseAbility_8_9AC7F1424787AED21383DDB4C16A02F5` (break `/Game/Structs/S_BL_Data` (`/Game/Assets/Components/Muzzle/BPC_Muzzle.BulletData` _leftmuzzle))))) _output 0.01) true)
      (`/Game/Assets/Components/Muzzle/BPC_Muzzle.IncreaseBulletExtraDamage` _rightmuzzle_2 (* (`.Damage_8_95FA65794938F8646CAD6B9925CAF05F` (break `/Game/Structs/S_BL_Base` (`.BaseAbility_8_9AC7F1424787AED21383DDB4C16A02F5` (break `/Game/Structs/S_BL_Data` (`/Game/Assets/Components/Muzzle/BPC_Muzzle.BulletData` _rightmuzzle_2))))) _output 0.01) true))
    (:`NewEnumerator1`
      ;[1 1 1] BPM Upgrade
      (`/Game/Assets/Components/Muzzle/BPC_Muzzle.IncreaseBPM` _leftmuzzle_2 (* (`/Game/Assets/Components/Muzzle/BPC_Muzzle.GetOriginalBPM` _leftmuzzle_2) 0.01 _output_2) true)
      (`/Game/Assets/Components/Muzzle/BPC_Muzzle.IncreaseBPM` _rightmuzzle (* (`/Game/Assets/Components/Muzzle/BPC_Muzzle.GetOriginalBPM` _rightmuzzle) 0.01 _output_2) true))
    (:`NewEnumerator2`
      ;[1 1 1] HP Upgrade
      (`/Game/Assets/Characters/Player/ConquerorBot/Blueprints/BP_ConquerorBot.IncreaseMaxHP` (`self.Player`) (`|GetArrayItem` (`.Parameters_63_6816A3134B95D0FCEFA3B798B0A79A10` (break `/Game/Structs/S_UpgradeData` (`local.UpgradeData`)))) true))))

(fn `UserConstructionScript`)